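; Character actor that displays a VRM avatar, animated in both editor preview and play.
; A source VRoid mesh plays the animation, and VrmAnimInstanceCopy retargets its pose onto the VRM mesh with spring-bone and morph settings.
; Init, also run from the construction script, wires the anim-control and pose-rig components and configures MToon outline and shadow actors.
; It also runs randomized morph-target blinking, forwards look-at control, and can move the model onto a spawned BP_ModelAttach.
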(event EventBeginPlay
  (Utilities|FlowControl|Sequence
    (:then_1
      (Variables|Default|SetbBeginCalled true))
    (:then_2
      (CallFunction|Init))
    (:then_3
      (CallFunction|BeginBlink))
    (:then_4
      (Default|SetFrameLimit (Variables|Default|GetBP_VrmAnimControlComponent) (Variables|Animation|GetbEnableFrameLimit) (Variables|Animation|GetFrameLimit%20%28frames/sec%29)))))

(event Collision|EventActorBeginOverlap
  (params (OtherActor :type Actor%20Object%20Reference)))

(event EventTick
  (params (DeltaSeconds :type Float%20%28single-precision%29)))

(event Custom|init
  (bind _bp_vrmanimcontrolcomponent (Variables|Default|GetBP_VrmAnimControlComponent))
  (bind _childactor (Variables|Default|GetChildActor))
  (bind _retargetsrcanimation (Variables|Default|GetRetargetSrcAnimation))
  (bind _skeletalmeshcomponent_src (Variables|Default|GetSkeletalMeshComponent_Src))
  (bind _animsequence (Utilities|Struct|BreakVRMRetargetSrcAnimSequence _retargetsrcanimation))
  (bind _childactor_2 (Variables|/Script/Engine.ChildActorComponent|GetChildActor _childactor))
  (bind _asmtoon_attach_actor (Utilities|Casting|CastToMToonAttachActor _childactor_2))
  (Utilities|FlowControl|Sequence
    (:then_0
      (Variables|Develop|GetSkeletalMeshComponent_Dst
        (:then)
        (:else
          (Variables|Develop|SetSkeletalMeshComponent_Dst (Variables|Default|GetSkeletalMeshDst)))))
    (:then_1
      (Utilities|FlowControl|Sequence
        (:then_0
          ;[1 1 1] AnimSequence
          (bind _skeletalmeshcomponent_src_2 (Variables|Default|GetSkeletalMeshComponent_Src)
            (:then
              (bind _asabp_vroid_simple (Utilities|Casting|CastToABP_VRoidSimple (Components|SkeletalMesh|GetAnimInstance _skeletalmeshcomponent_src_2)))
              (if (== (.skeleton (Class|VrmBPFunctionLibrary|VRMGetAnimationAssetData _animsequence)) (Variables|/Script/Engine.SkeletalMesh|GetSkeleton (Variables|/Script/Engine.SkinnedMeshComponent|GetSkeletalMesh _skeletalmeshcomponent_src_2)))
                (Default|SetCustomAnimSequence _asabp_vroid_simple _animsequence)
                (Variables|/VRM4U/Util/BaseCharacter/Mesh/ABP_VRoidSimple.ABP_VRoidSimple_C|SetTargetVrmModelActor _asabp_vroid_simple self)
                (else
                  (Utilities|Struct|SetmembersinVRMRetargetSrcAnimSequence _retargetsrcanimation))))
            (:else)))
        (:then_1
          (bind _skeletalmeshcomponent_dst (Variables|Develop|GetSkeletalMeshComponent_Dst)
            (:then
              (bind _vrmassetlist (Variables|Default|GetVrmAssetList)
                (:then
                  (Class|SkinnedMeshComponent|SetSkeletalMesh _skeletalmeshcomponent_dst (Variables|/Script/VRM4U.VrmAssetListObject|GetSkeletalMesh _vrmassetlist) true)
                  (bind _skeletalmeshcomponent_dst_2 (Variables|Develop|GetSkeletalMeshComponent_Dst)
                    (:then
                      (bind _asvrm_anim_instance_copy (Utilities|Casting|CastToVrmAnimInstanceCopy (Components|SkeletalMesh|GetAnimInstance _skeletalmeshcomponent_dst_2)))
                      (Utilities|FlowControl|Sequence
                        (:then_0
                          (if (or (Variables|Default|GetbBeginCalled) (.bPlay (Class|VrmBPFunctionLibrary|VRMGetPlayMode)))
                            (Utilities|FlowControl|Sequence :!label _label
                              (:then_0
                                (Variables|/Script/VRM4U.VrmAnimInstanceCopy|SetbCopyStop _asvrm_anim_instance_copy false))
                              (:then_1
                                (Class|VrmAnimInstanceCopy|SetSkeletalMeshCopyData _asvrm_anim_instance_copy (Variables|Default|GetVrmAssetList) (Variables|Default|GetSkeletalMeshComponent_Src) 0 "/VRM4U/Util/BaseCharacter/Mesh/VRoidSimple_VrmAssetList.VRoidSimple_VrmAssetList")
                                (Class|VrmAnimInstanceCopy|SetSkeletalMeshCopyDataforCustomSpring _asvrm_anim_instance_copy (Variables|Animation|GetCustomSpringParam))))
                            (else
                              (Utilities|IsValid (Utilities|Struct|BreakVRMRetargetSrcAnimSequence (Variables|Default|GetRetargetSrcAnimation))
                                (:Is%20Valid
                                  (if (Variables|Default|GetbIgnoreAnimPreviewPose)
                                    _
                                    (else
                                      (goto _label))))
                                (:Is%20Not%20Valid
                                  _))
                              ;[1 1 1] use ref pose
                              (Variables|/Script/VRM4U.VrmAnimInstanceCopy|SetbCopyStop _asvrm_anim_instance_copy true))))
                        (:then_1
                          ;[1 1 1] morph
                          (Utilities|FlowControl|Sequence
                            (:then_1
                              (Utilities|Array|Clear (Variables|/Script/VRM4U.VrmAnimInstanceCopy|GetInitialMorphName _asvrm_anim_instance_copy))
                              (Utilities|Array|Clear (Variables|/Script/VRM4U.VrmAnimInstanceCopy|GetInitialMorphValue _asvrm_anim_instance_copy)))
                            (:then_2
                              (for _array_element (Variables|Default|GetMorphDirect)
                                (Utilities|Array|Add (Variables|/Script/VRM4U.VrmAnimInstanceCopy|GetInitialMorphName _asvrm_anim_instance_copy) (Utilities|String|StringToName (.MorphName (Utilities|Struct|BreakVRMMorphWeight _array_element))))
                                (Utilities|Array|Add (Variables|/Script/VRM4U.VrmAnimInstanceCopy|GetInitialMorphValue _asvrm_anim_instance_copy) (.Weight (Utilities|Struct|BreakVRMMorphWeight _array_element)))))))
                        (:then_2
                          (Default|SetVrmSpringBoneParam (Variables|Default|GetBP_VrmAnimControlComponent) (Variables|Animation|GetVRMSpringBoneParam)))))
                    (:else)))
                (:else)))
            (:else)))
        (:then_3
          (if (Variables|Default|GetbBeginCalled)
            (EventDispatchers|UnbindEventfromOnAnimInitialized _skeletalmeshcomponent_src (delegate Custom|CustomEvent_0))
            (else
              (EventDispatchers|AssignOnAnimInitialized _skeletalmeshcomponent_src (delegate Custom|CustomEvent_0)))))
        (:then_4
          (if (not (Variables|Develop|GetbSkipAttachActorInit))
            ;[1 1 1] AttachActor
            (Utilities|FlowControl|Sequence
              (:then_0
                (Variables|/VRM4U/Util/Actor/MToonAttachActor.MToonAttachActor_C|SetTargetByActor _asmtoon_attach_actor self))
              (:then_1
                (Variables|Default|Settmp_mtoonattach _asmtoon_attach_actor))
              (:then_2
                (bind _attachmodeactor (Variables|Develop|GetAttachModeActor)
                  (:then
                    (Variables|Default|Settmp_mtoonattach (.AsMToon%20Attach%20Actor (Utilities|Casting|CastToMToonAttachActor (Variables|/Script/Engine.ChildActorComponent|GetChildActor (Variables|/VRM4U/Util/BaseCharacter/Misc/BP_ModelAttach.BP_ModelAttach_C|GetChildActor _attachmodeactor)))))
                    (Variables|/VRM4U/Util/Actor/MToonAttachActor.MToonAttachActor_C|SetTargetByActor _asmtoon_attach_actor 0)
                    (Default|ReInit _asmtoon_attach_actor false))
                  (:else)))
              (:then_3
                (Variables|/VRM4U/Util/Actor/MToonAttachActor.MToonAttachActor_C|SetbCreateCastShadowDummyModel (Variables|Default|Gettmp_mtoonattach) (Variables|Default|GetbCreateCastShadowDummyModel))
                (Variables|/VRM4U/Util/Actor/MToonAttachActor.MToonAttachActor_C|SetbCreateOutlineModel (Variables|Default|Gettmp_mtoonattach) (Variables|Default|GetbCreateOutlineModel))
                (Variables|/VRM4U/Util/Actor/MToonAttachActor.MToonAttachActor_C|SetShadowmapDistance (Variables|Default|Gettmp_mtoonattach) (Variables|Default|GetShadowmapDistance))
                (Variables|/VRM4U/Util/Actor/MToonAttachActor.MToonAttachActor_C|SetbDisableCustomShadowMap (Variables|Default|Gettmp_mtoonattach) (Variables|Default|GetbDisableCustomShadowMap))
                (Variables|/VRM4U/Util/Actor/MToonAttachActor.MToonAttachActor_C|SetbCreateAOShadowModel (Variables|Default|Gettmp_mtoonattach) (Variables|Default|GetbAOShadowModel))
                (Variables|/VRM4U/Util/Actor/MToonAttachActor.MToonAttachActor_C|SetAOSkeletalMesh (Variables|Default|Gettmp_mtoonattach) (Variables|Default|GetAOShadowModel))
                (Variables|/VRM4U/Util/Actor/MToonAttachActor.MToonAttachActor_C|SetbDebugShadowCube (Variables|Default|Gettmp_mtoonattach) (Variables|Develop|GetbDebugDrawCube))
                (Variables|/VRM4U/Util/Actor/MToonAttachActor.MToonAttachActor_C|SetShadowMapSize (Variables|Default|Gettmp_mtoonattach) (Variables|Default|GetShadowMapSize))
                (Variables|/VRM4U/Util/Actor/MToonAttachActor.MToonAttachActor_C|SetShadowOrthSize (Variables|Default|Gettmp_mtoonattach) (Variables|Default|GetShadowCameraViewSize)))
              (:then_4
                (Default|ReInit (Variables|Default|Gettmp_mtoonattach) false)))))))
    (:then_2
      (Variables|Default|SetPreview%28Auto%29 (Variables|/Script/Engine.SkinnedMeshComponent|GetSkeletalMesh (Variables|Develop|GetSkeletalMeshComponent_Dst))))
    (:then_3
      (Utilities|FlowControl|Sequence
        (:then_0
          (Default|SetSkeleton _bp_vrmanimcontrolcomponent (Variables|Default|GetSkeletalMeshComponent_Src) (Variables|Develop|GetSkeletalMeshComponent_Dst) (Variables|Default|GetVrmAssetList))
          (EventDispatchers|BindEventtoOnForceBlink _bp_vrmanimcontrolcomponent (EventDispatchers|CreateEvent :!event Custom|ForceBlink)))
        (:then_1
          (Default|SetMasterActor (Variables|Default|GetBP_VrmPoseRigComponent) self))
        (:then_2
          (bind _attachmodeactor_2 (Variables|Develop|GetAttachModeActor)
            (:then
              (Default|UpdatePose _attachmodeactor_2))
            (:else)))))))

(event Custom|CustomEvent_0
  (if (not (or (Variables|Default|GetbBeginCalled) (.bPlay (Class|VrmBPFunctionLibrary|VRMGetPlayMode))))
    (Class|VrmBPFunctionLibrary|VRMInitAnim (Variables|Develop|GetSkeletalMeshComponent_Dst))
    (bind _attachmodeactor (Variables|Develop|GetAttachModeActor)
      (:then
        (Default|UpdatePose _attachmodeactor))
      (:else))))

(event Custom|ReInitMToonAttachActor
  (bind _childactor (Variables|Default|GetChildActor))
  (bind _childactor_2 (Variables|/Script/Engine.ChildActorComponent|GetChildActor _childactor))
  (bind _asmtoon_attach_actor (Utilities|Casting|CastToMToonAttachActor _childactor_2))
  (if (not (Variables|Develop|GetbSkipAttachActorInit))
    ;[1 1 1] AttachActor
    (Utilities|FlowControl|Sequence
      (:then_0
        (Variables|/VRM4U/Util/Actor/MToonAttachActor.MToonAttachActor_C|SetTargetByActor _asmtoon_attach_actor self))
      (:then_1
        (Variables|Default|Settmp_mtoonattach _asmtoon_attach_actor))
      (:then_2
        (bind _attachmodeactor (Variables|Develop|GetAttachModeActor)
          (:then
            (Variables|Default|Settmp_mtoonattach (.AsMToon%20Attach%20Actor (Utilities|Casting|CastToMToonAttachActor (Variables|/Script/Engine.ChildActorComponent|GetChildActor (Variables|/VRM4U/Util/BaseCharacter/Misc/BP_ModelAttach.BP_ModelAttach_C|GetChildActor _attachmodeactor)))))
            (Variables|/VRM4U/Util/Actor/MToonAttachActor.MToonAttachActor_C|SetTargetByActor _asmtoon_attach_actor 0)
            (Default|ReInit _asmtoon_attach_actor false))
          (:else)))
      (:then_3
        (Variables|/VRM4U/Util/Actor/MToonAttachActor.MToonAttachActor_C|SetbCreateCastShadowDummyModel (Variables|Default|Gettmp_mtoonattach) (Variables|Default|GetbCreateCastShadowDummyModel))
        (Variables|/VRM4U/Util/Actor/MToonAttachActor.MToonAttachActor_C|SetbCreateOutlineModel (Variables|Default|Gettmp_mtoonattach) (Variables|Default|GetbCreateOutlineModel))
        (Variables|/VRM4U/Util/Actor/MToonAttachActor.MToonAttachActor_C|SetShadowmapDistance (Variables|Default|Gettmp_mtoonattach) (Variables|Default|GetShadowmapDistance))
        (Variables|/VRM4U/Util/Actor/MToonAttachActor.MToonAttachActor_C|SetbDisableCustomShadowMap (Variables|Default|Gettmp_mtoonattach) (Variables|Default|GetbDisableCustomShadowMap))
        (Variables|/VRM4U/Util/Actor/MToonAttachActor.MToonAttachActor_C|SetbCreateAOShadowModel (Variables|Default|Gettmp_mtoonattach) (Variables|Default|GetbAOShadowModel))
        (Variables|/VRM4U/Util/Actor/MToonAttachActor.MToonAttachActor_C|SetAOSkeletalMesh (Variables|Default|Gettmp_mtoonattach) (Variables|Default|GetAOShadowModel))
        (Variables|/VRM4U/Util/Actor/MToonAttachActor.MToonAttachActor_C|SetbDebugShadowCube (Variables|Default|Gettmp_mtoonattach) (Variables|Develop|GetbDebugDrawCube))
        (Variables|/VRM4U/Util/Actor/MToonAttachActor.MToonAttachActor_C|SetShadowMapSize (Variables|Default|Gettmp_mtoonattach) (Variables|Default|GetShadowMapSize))
        (Variables|/VRM4U/Util/Actor/MToonAttachActor.MToonAttachActor_C|SetShadowOrthSize (Variables|Default|Gettmp_mtoonattach) (Variables|Default|GetShadowCameraViewSize)))
      (:then_4
        (Default|ReInit (Variables|Default|Gettmp_mtoonattach) false)))))

(event Custom|BeginBlink
  (bind _skeletalmeshcomponent_src (Variables|Default|GetSkeletalMeshComponent_Src))
  ;[1 1 1] Blink
  (Utilities|FlowControl|DoOnce false
    (:Completed
      (Variables|Default|GetVrmAssetList
        (:then
          (Utilities|FlowControl|Sequence :!label _label
            (:then_2
              (Utilities|FlowControl|Sequence
                (:then_0
                  (goto _label_2 Reset))
                (:then_1
                  (Utilities|FlowControl|RetriggerableDelay (Math|Random|RandomFloatinRange 1.0 6.0))
                  (Utilities|FlowControl|DoOnce false :!label _label_2
                    (:Completed
                      (if (Variables|Animation|GetbEnableBlink)
                        (bind _newtrack_0 (Timeline|Timeline_0 PlayFromStart)
                          (:Update
                            (if (not (Variables|/VRM4U/Util/BaseCharacter/Misc/BP_VrmAnimControlComponent.BP_VrmAnimControlComponent_C|GetAnimStopFrame (Variables|Default|GetBP_VrmAnimControlComponent)))
                              (bind _array_element (Utilities|Array|ForEachLoopwithBreak (Variables|/Script/VRM4U.VrmMetaObject|GetBlendShapeGroup (Variables|/Script/VRM4U.VrmAssetListObject|GetVrmMetaObject (Variables|Default|GetVRMAssetList))) :!label _label_3)
                                (:LoopBody
                                  (if (Utilities|Enum|Equal(Enum) (.name (Utilities|Struct|BreakVrmBlendShapeGroup _array_element)) "Blink")
                                    (Utilities|FlowControl|Sequence
                                      (:then_0
                                        (bind _array_element_2 (Utilities|Array|ForEachLoopwithBreak (.BlendShape (Utilities|Struct|BreakVrmBlendShapeGroup _array_element)))
                                          (:LoopBody
                                            (Components|SkeletalMesh|SetMorphTarget (Variables|Develop|GetSkeletalMeshComponent_Dst) (Utilities|String|StringToName (.morphTargetName (Utilities|Struct|BreakVrmBlendShape _array_element_2))) _newtrack_0 true))))
                                      (:then_1
                                        (if (Rendering|IsVisible _skeletalmeshcomponent_src)
                                          (Components|SkeletalMesh|SetMorphTarget _skeletalmeshcomponent_src "Face.M_F00_000_Fcl_EYE_Close" _newtrack_0 true)))
                                      (:then_2
                                        (goto _label_3 Break))))))))
                          (:Finished
                            (Utilities|FlowControl|Sequence
                              (:then_0
                                (goto _label))
                              (:then_1
                                (Class|SkeletalMeshComponent|ClearMorphTargets (Variables|Develop|GetSkeletalMeshComponent_Dst))))))))))))))
        (:else)))))

(event Custom|SetLookAtTarget
  (params (TargetLocation :type Vector))
  (Default|SetLookatTarget (Variables|Default|GetBP_VrmAnimControlComponent) TargetLocation))

(event Custom|ForceBlink
  (bind _skeletalmeshcomponent_src (Variables|Default|GetSkeletalMeshComponent_Src))
  ;[1 1 1] Blink
  (Utilities|FlowControl|DoOnce false :!label _label
    (:Completed
      (if (Variables|Animation|GetbEnableBlink)
        (bind _newtrack_0 (Timeline|Timeline_0 PlayFromStart)
          (:Update
            (if (not (Variables|/VRM4U/Util/BaseCharacter/Misc/BP_VrmAnimControlComponent.BP_VrmAnimControlComponent_C|GetAnimStopFrame (Variables|Default|GetBP_VrmAnimControlComponent)))
              (bind _array_element (Utilities|Array|ForEachLoopwithBreak (Variables|/Script/VRM4U.VrmMetaObject|GetBlendShapeGroup (Variables|/Script/VRM4U.VrmAssetListObject|GetVrmMetaObject (Variables|Default|GetVRMAssetList))) :!label _label_2)
                (:LoopBody
                  (if (Utilities|Enum|Equal(Enum) (.name (Utilities|Struct|BreakVrmBlendShapeGroup _array_element)) "Blink")
                    (Utilities|FlowControl|Sequence
                      (:then_0
                        (bind _array_element_2 (Utilities|Array|ForEachLoopwithBreak (.BlendShape (Utilities|Struct|BreakVrmBlendShapeGroup _array_element)))
                          (:LoopBody
                            (Components|SkeletalMesh|SetMorphTarget (Variables|Develop|GetSkeletalMeshComponent_Dst) (Utilities|String|StringToName (.morphTargetName (Utilities|Struct|BreakVrmBlendShape _array_element_2))) _newtrack_0 true))))
                      (:then_1
                        (if (Rendering|IsVisible _skeletalmeshcomponent_src)
                          (Components|SkeletalMesh|SetMorphTarget _skeletalmeshcomponent_src "Face.M_F00_000_Fcl_EYE_Close" _newtrack_0 true)))
                      (:then_2
                        (goto _label_2 Break))))))))
          (:Finished
            (Utilities|FlowControl|Sequence
              (:then_0
                (Utilities|FlowControl|Sequence
                  (:then_2
                    (Utilities|FlowControl|Sequence
                      (:then_0
                        (goto _label Reset))
                      (:then_1
                        (Utilities|FlowControl|RetriggerableDelay (Math|Random|RandomFloatinRange 1.0 6.0))
                        (goto _label))))))
              (:then_1
                (Class|SkeletalMeshComponent|ClearMorphTargets (Variables|Develop|GetSkeletalMeshComponent_Dst))))))))))

(event Custom|SetLookAtForce
  (params (LookAtForce :type Float%20%28single-precision%29))
  (Default|SetLookatForce (Variables|Default|GetBP_VrmAnimControlComponent) LookAtForce))

(event Custom|SetLookAtType
  (params (Eye :type Boolean) (Head :type Boolean))
  (Default|SetLookatType (Variables|Default|GetBP_VrmAnimControlComponent) Eye Head))

(event Custom|SetBlinkEnable
  (params (bEnable :type Boolean))
  (bind _skeletalmeshcomponent_src (Variables|Default|GetSkeletalMeshComponent_Src))
  ;[1 1 1] Blink
  (if (Math|Boolean|NotEqual(Boolean) bEnable (Variables|Animation|GetbEnableBlink))
    (Variables|Animation|SetbEnableBlink bEnable)
    (if (Variables|Animation|GetbEnableBlink) :!label _label
      (bind _newtrack_0 (Timeline|Timeline_0 PlayFromStart)
        (:Update
          (if (not (Variables|/VRM4U/Util/BaseCharacter/Misc/BP_VrmAnimControlComponent.BP_VrmAnimControlComponent_C|GetAnimStopFrame (Variables|Default|GetBP_VrmAnimControlComponent)))
            (bind _array_element (Utilities|Array|ForEachLoopwithBreak (Variables|/Script/VRM4U.VrmMetaObject|GetBlendShapeGroup (Variables|/Script/VRM4U.VrmAssetListObject|GetVrmMetaObject (Variables|Default|GetVRMAssetList))) :!label _label_2)
              (:LoopBody
                (if (Utilities|Enum|Equal(Enum) (.name (Utilities|Struct|BreakVrmBlendShapeGroup _array_element)) "Blink")
                  (Utilities|FlowControl|Sequence
                    (:then_0
                      (bind _array_element_2 (Utilities|Array|ForEachLoopwithBreak (.BlendShape (Utilities|Struct|BreakVrmBlendShapeGroup _array_element)))
                        (:LoopBody
                          (Components|SkeletalMesh|SetMorphTarget (Variables|Develop|GetSkeletalMeshComponent_Dst) (Utilities|String|StringToName (.morphTargetName (Utilities|Struct|BreakVrmBlendShape _array_element_2))) _newtrack_0 true))))
                    (:then_1
                      (if (Rendering|IsVisible _skeletalmeshcomponent_src)
                        (Components|SkeletalMesh|SetMorphTarget _skeletalmeshcomponent_src "Face.M_F00_000_Fcl_EYE_Close" _newtrack_0 true)))
                    (:then_2
                      (goto _label_2 Break))))))))
        (:Finished
          (Utilities|FlowControl|Sequence
            (:then_0
              (Utilities|FlowControl|Sequence
                (:then_2
                  (Utilities|FlowControl|Sequence
                    (:then_0
                      (goto _label_3 Reset))
                    (:then_1
                      (Utilities|FlowControl|RetriggerableDelay (Math|Random|RandomFloatinRange 1.0 6.0))
                      (Utilities|FlowControl|DoOnce false :!label _label_3
                        (:Completed
                          (goto _label))))))))
            (:then_1
              (Class|SkeletalMeshComponent|ClearMorphTargets (Variables|Develop|GetSkeletalMeshComponent_Dst)))))))))

(event Custom|ToAttachMode
  (Utilities|FlowControl|Sequence
    (:then_0
      (Variables|Develop|GetAttachModeActor
        (:then)
        (:else
          (Utilities|FlowControl|Sequence
            (:then_0
              (for _array_element (Actor|GetAttachedActors self)
                (bind _asbp_model_attach (Utilities|Casting|CastToBP_ModelAttach _array_element))
                (Actor|DestroyActor _asbp_model_attach)))))))
    (:then_1
      (Utilities|FlowControl|Sequence
        (:then_1
          (Utilities|FlowControl|Sequence
            (:then_0
              (Variables|Develop|GetAttachModeActor
                (:then)
                (:else
                  (bind _returnvalue (Game|SpawnActorfromClass "/VRM4U/Util/BaseCharacter/Misc/BP_ModelAttach.BP_ModelAttach_C" (Math|Transform|MakeTransform "0, 0, 0") "Undefined" 0 self 0))
                  (Variables|Develop|SetAttachModeActor _returnvalue))))
            (:then_1
              (Transformation|AttachComponentToComponent (Variables|Develop|GetAttachModeActor) (Variables|Default|GetSkeletalMeshComponent_Src) "None" "SnapToTarget" "SnapToTarget" "SnapToTarget" true)
              (Variables|Develop|SetSkeletalMeshComponent_Dst (Variables|/Script/Engine.SkeletalMeshActor|GetSkeletalMeshComponent (Variables|Develop|GetAttachModeActor)))
              (CallFunction|Init))))
        (:then_2
          (Default|UpdatePose (Variables|Develop|GetAttachModeActor)))))))

(event Custom|ToNormalMode
  (Utilities|FlowControl|Sequence
    (:then_0
      (Variables|Develop|SetAttachModeActor 0)
      (Variables|Develop|GetAttachModeActor
        (:then)
        (:else
          (Utilities|FlowControl|Sequence
            (:then_0
              (for _array_element (Actor|GetAttachedActors self)
                (bind _asbp_model_attach (Utilities|Casting|CastToBP_ModelAttach _array_element))
                (Actor|DestroyActor _asbp_model_attach)))))))))

(fn ConstructionScript
  (bind _returnvalue (Transformation|GetActorTransform))
  (bind _childactor (Variables|Default|GetChildActor))
  (bind _childactor_2 (Variables|/Script/Engine.ChildActorComponent|GetChildActor _childactor))
  (bind _asmtoon_attach_actor (Utilities|Casting|CastToMToonAttachActor _childactor_2))
  (Utilities|FlowControl|Sequence
    (:then_0
      (Variables|Develop|SetbSkipAttachActorInit (not (== (Variables|Develop|GetCheckForChangeTrans) _returnvalue)))
      (Variables|Develop|SetCheckForChangeTrans _returnvalue))
    (:then_1
      (Variables|Develop|GetSkeletalMeshComponent_Dst
        (:then)
        (:else
          (Variables|Develop|SetSkeletalMeshComponent_Dst (Variables|Default|GetSkeletalMeshDst)))))
    (:then_2
      (Utilities|FlowControl|Sequence
        (:then_0
          (Variables|/Script/Engine.SkeletalMeshComponent|SetGlobalAnimRateScale (Variables|Default|GetSkeletalMeshComponent_Src) (Math|Float|Max(Float) (Variables|Default|GetGlobalAnimRateScale) 0.0)))
        (:then_1
          (Variables|Default|GetVrmAssetList
            (:then
              (Utilities|FlowControl|Sequence
                (:then_0
                  (Variables|Default|SetPreview%28Auto%29 0))
                (:then_1
                  (CallFunction|Init))))
            (:else
              (Utilities|FlowControl|Sequence
                (:then_1
                  (Variables|Default|SetPreview%28Auto%29 0)
                  (Class|SkinnedMeshComponent|SetSkeletalMesh (Variables|Default|GetSkeletalMeshComponent_Src) 0 true)
                  (Variables|/VRM4U/Util/Actor/MToonAttachActor.MToonAttachActor_C|SetTargetByActor _asmtoon_attach_actor 0)
                  (Variables|/VRM4U/Util/Actor/MToonAttachActor.MToonAttachActor_C|SetVRMAssetList _asmtoon_attach_actor 0)
                  (Default|ReInit _asmtoon_attach_actor false))))))
        (:then_2
          (Variables|Default|SetRefreshDummy false))))
    (:then_3
      (bind _attachmodeactor (Variables|Develop|GetAttachModeActor)
        (:then
          (Transformation|SetActorTransform _attachmodeactor (Transformation|GetActorTransform)))
        (:else)))))