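; Base Blueprint for VRM avatar characters, handling animation retargeting, MToon rendering, blinking, look-at and ragdoll.
; Init, run at construction and BeginPlay, applies the VRM asset's mesh and materials, then copies the pose from a VRoidSimple source mesh through VrmAnimInstanceCopy.
; It also configures the MToon child actor's outline and shadows, and the anim control component for spring bones and look-at.
; A timeline drives Blink blend-shape morphs at random intervals or on demand.
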(event Custom|SetLookAtTarget
  (params (TargetLocation :type Vector))
  ;[1 1 1] LookAt
  (Default|SetLookatTarget (Variables|Default|GetBP_VrmAnimControlComponent) TargetLocation))

(event Custom|ForceBlink
  ;[1 1 1] Blink
  (Utilities|FlowControl|DoOnce false :!label _label
    (:Completed
      (if (Variables|Animation|GetbEnableBlink)
        (bind _newtrack_0 (Timeline|Timeline_0 PlayFromStart)
          (:Update
            (if (not (Variables|/VRM4U/Util/BaseCharacter/Misc/BP_VrmAnimControlComponent.BP_VrmAnimControlComponent_C|GetAnimStopFrame (Variables|Default|GetBP_VrmAnimControlComponent)))
              (bind _array_element (Utilities|Array|ForEachLoopwithBreak (Variables|/Script/VRM4U.VrmMetaObject|GetBlendShapeGroup (Variables|/Script/VRM4U.VrmAssetListObject|GetVrmMetaObject (Variables|Default|GetVRMAssetList))) :!label _label_2)
                (:LoopBody
                  (if (Utilities|Enum|Equal(Enum) (.name (Utilities|Struct|BreakVrmBlendShapeGroup _array_element)) "Blink")
                    (Utilities|FlowControl|Sequence
                      (:then_0
                        (bind _array_element_2 (Utilities|Array|ForEachLoopwithBreak (.BlendShape (Utilities|Struct|BreakVrmBlendShapeGroup _array_element)))
                          (:LoopBody
                            (Components|SkeletalMesh|SetMorphTarget (Variables|Character|GetMesh) (Utilities|String|StringToName (.morphTargetName (Utilities|Struct|BreakVrmBlendShape _array_element_2))) _newtrack_0 true))))
                      (:then_1
                        (if (Rendering|IsVisible (Variables|Character|GetMesh))
                          _))
                      (:then_2
                        (goto _label_2 Break))))))))
          (:Finished
            (Utilities|FlowControl|Sequence
              (:then_0
                (Utilities|FlowControl|Sequence
                  (:then_2
                    (Utilities|FlowControl|Sequence
                      (:then_0
                        (goto _label Reset))
                      (:then_1
                        (Utilities|FlowControl|RetriggerableDelay (Math|Random|RandomFloatinRange 1.0 6.0))
                        (goto _label))))))
              (:then_1
                (Class|SkeletalMeshComponent|ClearMorphTargets (Variables|Character|GetMesh))))))))))

(event Custom|ToRagdoll
  (bind _mesh (Variables|Character|GetMesh))
  (Collision|SetCollisionEnabled _mesh "QueryAndPhysics")
  (Collision|SetCollisionResponsetoAllChannels _mesh "ECR_Ignore")
  (Class|SkeletalMeshComponent|SetAllBodiesSimulatePhysics _mesh true)
  (Utilities|FlowControl|Sequence
    (:then_0
      (for _array_element (Utilities|Array|MakeArray "ECC_WorldStatic" "ECC_WorldDynamic")
        (Collision|SetCollisionResponsetoChannel _mesh _array_element "ECR_Block")))))

(event Custom|SetLookAtType
  (params (Eye :type Boolean) (Head :type Boolean))
  ;[1 1 1] LookAt
  (Default|SetLookatType (Variables|Default|GetBP_VrmAnimControlComponent) Eye Head))

(event Custom|SetBlinkEnable
  (params (bEnable :type Boolean))
  ;[1 1 1] Blink
  (if (Math|Boolean|NotEqual(Boolean) bEnable (Variables|Animation|GetbEnableBlink))
    (Variables|Animation|SetbEnableBlink bEnable)
    (if (Variables|Animation|GetbEnableBlink) :!label _label
      (bind _newtrack_0 (Timeline|Timeline_0 PlayFromStart)
        (:Update
          (if (not (Variables|/VRM4U/Util/BaseCharacter/Misc/BP_VrmAnimControlComponent.BP_VrmAnimControlComponent_C|GetAnimStopFrame (Variables|Default|GetBP_VrmAnimControlComponent)))
            (bind _array_element (Utilities|Array|ForEachLoopwithBreak (Variables|/Script/VRM4U.VrmMetaObject|GetBlendShapeGroup (Variables|/Script/VRM4U.VrmAssetListObject|GetVrmMetaObject (Variables|Default|GetVRMAssetList))) :!label _label_2)
              (:LoopBody
                (if (Utilities|Enum|Equal(Enum) (.name (Utilities|Struct|BreakVrmBlendShapeGroup _array_element)) "Blink")
                  (Utilities|FlowControl|Sequence
                    (:then_0
                      (bind _array_element_2 (Utilities|Array|ForEachLoopwithBreak (.BlendShape (Utilities|Struct|BreakVrmBlendShapeGroup _array_element)))
                        (:LoopBody
                          (Components|SkeletalMesh|SetMorphTarget (Variables|Character|GetMesh) (Utilities|String|StringToName (.morphTargetName (Utilities|Struct|BreakVrmBlendShape _array_element_2))) _newtrack_0 true))))
                    (:then_1
                      (if (Rendering|IsVisible (Variables|Character|GetMesh))
                        _))
                    (:then_2
                      (goto _label_2 Break))))))))
        (:Finished
          (Utilities|FlowControl|Sequence
            (:then_0
              (Utilities|FlowControl|Sequence
                (:then_2
                  (Utilities|FlowControl|Sequence
                    (:then_0
                      (goto _label_3 Reset))
                    (:then_1
                      (Utilities|FlowControl|RetriggerableDelay (Math|Random|RandomFloatinRange 1.0 6.0))
                      (Utilities|FlowControl|DoOnce false :!label _label_3
                        (:Completed
                          (goto _label))))))))
            (:then_1
              (Class|SkeletalMeshComponent|ClearMorphTargets (Variables|Character|GetMesh)))))))))

(event Custom|SetCustomAnim
  (bind _retargetsrcanimation (Variables|Default|GetRetargetSrcAnimation))
  (bind _mesh (Variables|Character|GetMesh))
  (bind _animsequence (Utilities|Struct|BreakVRMRetargetSrcAnimSequence _retargetsrcanimation))
  (bind _returnvalue (Components|SkeletalMesh|GetAnimInstance _mesh))
  (bind (_asabp_vroid_simple _bsuccess) (Utilities|Casting|CastToABP_VRoidSimple _returnvalue))
  (Utilities|IsValid _animsequence
    (:Is%20Valid
      (if _bsuccess
        (Default|SetCustomAnimSequence _asabp_vroid_simple _animsequence)
        (Development|PrintString "Hello")))))

(event EventBeginPlay
  (Utilities|FlowControl|Sequence
    (:then_0
      (Variables|Default|SetbBeginCalled true))
    (:then_1
      (CallFunction|Init))
    (:then_5
      (Default|SetFrameLimit (Variables|Default|GetBP_VrmAnimControlComponent) (Variables|Animation|GetbEnableFrameLimit) (Variables|Animation|GetFrameLimit%20%28frames/sec%29)))))

(event Collision|EventActorBeginOverlap
  (params (OtherActor :type Actor%20Object%20Reference)))

(event EventTick
  (params (DeltaSeconds :type Float%20%28single-precision%29))
  (Utilities|FlowControl|Sequence
    (:then_1
      (if (not (Variables|Default|GetMorphTargetOverride))
        ;[1 1 1] Blink
        (Utilities|FlowControl|DoOnce false
          (:Completed
            (bind _vrmassetlist (Variables|Default|GetVRMAssetList)
              (:then
                (Variables|/Script/VRM4U.VrmAssetListObject|GetVrmMetaObject _vrmassetlist
                  (:then
                    (Utilities|FlowControl|Sequence :!label _label
                      (:then_2
                        (Utilities|FlowControl|Sequence
                          (:then_0
                            (goto _label_2 Reset))
                          (:then_1
                            (Utilities|FlowControl|RetriggerableDelay (Math|Random|RandomFloatinRange 1.0 6.0))
                            (Utilities|FlowControl|DoOnce false :!label _label_2
                              (:Completed
                                (if (Variables|Animation|GetbEnableBlink)
                                  (bind _newtrack_0 (Timeline|Timeline_0 PlayFromStart)
                                    (:Update
                                      (if (not (Variables|/VRM4U/Util/BaseCharacter/Misc/BP_VrmAnimControlComponent.BP_VrmAnimControlComponent_C|GetAnimStopFrame (Variables|Default|GetBP_VrmAnimControlComponent)))
                                        (bind _array_element (Utilities|Array|ForEachLoopwithBreak (Variables|/Script/VRM4U.VrmMetaObject|GetBlendShapeGroup (Variables|/Script/VRM4U.VrmAssetListObject|GetVrmMetaObject (Variables|Default|GetVRMAssetList))) :!label _label_3)
                                          (:LoopBody
                                            (if (Utilities|Enum|Equal(Enum) (.name (Utilities|Struct|BreakVrmBlendShapeGroup _array_element)) "Blink")
                                              (Utilities|FlowControl|Sequence
                                                (:then_0
                                                  (bind _array_element_2 (Utilities|Array|ForEachLoopwithBreak (.BlendShape (Utilities|Struct|BreakVrmBlendShapeGroup _array_element)))
                                                    (:LoopBody
                                                      (Components|SkeletalMesh|SetMorphTarget (Variables|Character|GetMesh) (Utilities|String|StringToName (.morphTargetName (Utilities|Struct|BreakVrmBlendShape _array_element_2))) _newtrack_0 true))))
                                                (:then_1
                                                  (if (Rendering|IsVisible (Variables|Character|GetMesh))
                                                    _))
                                                (:then_2
                                                  (goto _label_3 Break))))))))
                                    (:Finished
                                      (Utilities|FlowControl|Sequence
                                        (:then_0
                                          (goto _label))
                                        (:then_1
                                          (Class|SkeletalMeshComponent|ClearMorphTargets (Variables|Character|GetMesh))))))))))))))
                  (:else)))
              (:else))))))))

(event Custom|init
  (bind _bp_vrmanimcontrolcomponent (Variables|Default|GetBP_VrmAnimControlComponent))
  (bind _mesh (Variables|Character|GetMesh))
  (bind _childactor (Variables|Default|GetChildActor))
  (bind _retargetsrcanimation (Variables|Default|GetRetargetSrcAnimation))
  (bind _skeletalmesh_retargetsrc (Variables|Default|GetSkeletalMesh_retargetSrc))
  (bind _animsequence (Utilities|Struct|BreakVRMRetargetSrcAnimSequence _retargetsrcanimation))
  (bind _returnvalue (Components|SkeletalMesh|GetAnimInstance _mesh))
  (bind _childactor_2 (Variables|/Script/Engine.ChildActorComponent|GetChildActor _childactor))
  (bind _asvrm_anim_instance_copy (Utilities|Casting|CastToVrmAnimInstanceCopy _returnvalue))
  (bind _asmtoon_attach_actor (Utilities|Casting|CastToMToonAttachActor _childactor_2))
  (Utilities|FlowControl|Sequence
    (:then_0
      (bind _asabp_vroid_simple (Utilities|Casting|CastToABP_VRoidSimple (Components|SkeletalMesh|GetAnimInstance _skeletalmesh_retargetsrc)))
      (if (== (.skeleton (Class|VrmBPFunctionLibrary|VRMGetAnimationAssetData _animsequence)) (Variables|/Script/Engine.SkeletalMesh|GetSkeleton (Variables|/Script/Engine.SkinnedMeshComponent|GetSkeletalMesh _skeletalmesh_retargetsrc)))
        (Default|SetCustomAnimSequence _asabp_vroid_simple _animsequence)
        (else
          (Utilities|Struct|SetmembersinVRMRetargetSrcAnimSequence _retargetsrcanimation))))
    (:then_1
      (Variables|/Script/Engine.SkeletalMeshComponent|SetGlobalAnimRateScale (Variables|Default|GetSkeletalMesh_retargetSrc) (Math|Float|Max(Float) (Variables|/Script/Engine.SkeletalMeshComponent|GetGlobalAnimRateScale (Variables|Character|GetMesh)) 0.0)))
    (:then_3
      (bind _vrmassetlist (Variables|Default|GetVRMAssetList)
        (:then
          (bind _skeletalmesh (Variables|/Script/VRM4U.VrmAssetListObject|GetSkeletalMesh _vrmassetlist)
            (:then
              (Utilities|FlowControl|Sequence
                (:then_0
                  (Class|SkinnedMeshComponent|SetSkeletalMesh _mesh _skeletalmesh true)
                  (Components|SkeletalMesh|SetAnimInstanceClass _mesh "/Script/VRM4U.VrmAnimInstanceCopy")
                  (Utilities|FlowControl|Sequence
                    (:then_0
                      (if (or (Variables|Default|GetbBeginCalled) (.bPlay (Class|VrmBPFunctionLibrary|VRMGetPlayMode)))
                        (Class|VrmAnimInstanceCopy|SetSkeletalMeshCopyData _asvrm_anim_instance_copy (Variables|Default|GetVRMAssetList) (Variables|Default|GetSkeletalMesh_retargetSrc) 0 "/VRM4U/Util/BaseCharacter/Mesh/VRoidSimple_VrmAssetList.VRoidSimple_VrmAssetList")
                        (Class|VrmAnimInstanceCopy|SetSkeletalMeshCopyDataforCustomSpring _asvrm_anim_instance_copy (Variables|Animation|GetCustomSpringParam))))
                    (:then_1
                      (Default|SetVrmSpringBoneParam (Variables|Default|GetBP_VrmAnimControlComponent) (Variables|Animation|GetVRMSpringBoneParam)))))
                (:then_1
                  (for (_array_element _array_index) (Variables|/Script/Engine.SkeletalMesh|GetMaterials _skeletalmesh)
                    (Rendering|Material|SetMaterial _mesh _array_index (.MaterialInterface (Utilities|Struct|BreakSkeletalMaterial _array_element)))))))
            (:else)))
        (:else)))
    (:then_4
      (Utilities|FlowControl|Sequence
        (:then_0
          (Variables|/VRM4U/Util/Actor/MToonAttachActor.MToonAttachActor_C|SetTargetByActor _asmtoon_attach_actor self))
        (:then_1
          (Variables|/VRM4U/Util/Actor/MToonAttachActor.MToonAttachActor_C|SetbCreateCastShadowDummyModel _asmtoon_attach_actor (Variables|Default|GetbCreateCastShadowDummyModel))
          (Variables|/VRM4U/Util/Actor/MToonAttachActor.MToonAttachActor_C|SetbCreateOutlineModel _asmtoon_attach_actor (Variables|Default|GetbCreateOutlineModel))
          (Variables|/VRM4U/Util/Actor/MToonAttachActor.MToonAttachActor_C|SetShadowmapDistance _asmtoon_attach_actor (Variables|Default|GetShadowmapDistance))
          (Variables|/VRM4U/Util/Actor/MToonAttachActor.MToonAttachActor_C|SetbDisableCustomShadowMap _asmtoon_attach_actor (Variables|Default|GetbDisableCustomShadowMap))
          (Variables|/VRM4U/Util/Actor/MToonAttachActor.MToonAttachActor_C|SetbCreateAOShadowModel _asmtoon_attach_actor (Variables|Default|GetbAOShadowModel))
          (Variables|/VRM4U/Util/Actor/MToonAttachActor.MToonAttachActor_C|SetAOSkeletalMesh _asmtoon_attach_actor (Variables|Default|GetAOShadowModel)))
        (:then_2
          (Default|ReInit _asmtoon_attach_actor false))))
    (:then_5
      (Default|SetSkeleton _bp_vrmanimcontrolcomponent (Variables|Default|GetSkeletalMesh_retargetSrc) (Variables|Character|GetMesh) (Variables|Default|GetVrmAssetList))
      (EventDispatchers|BindEventtoOnForceBlink _bp_vrmanimcontrolcomponent (EventDispatchers|CreateEvent :!event Custom|ForceBlink)))))

(fn ConstructionScript
  (Utilities|FlowControl|Sequence
    (:then_0
      (Variables|Animation|Setnotice "!!To change 'AnimationMode'. Select 'SkeletalMesh_simple' component"))
    (:then_2
      (CallFunction|Init))))

(fn CalcMainBone
  (params (TransformSpace :type ERelativeTransformSpace%20Enum :default "RTS_World"))
  (bind _vrmassetlist (Variables|Default|GetVRMAssetList))
  (bind _mesh (Variables|Character|GetMesh))
  (bind _vrmmetaobject (Variables|/Script/VRM4U.VrmAssetListObject|GetVrmMetaObject _vrmassetlist))
  (bind _humanoidbonetable (Variables|/Script/VRM4U.VrmMetaObject|GethumanoidBoneTable _vrmmetaobject))
  (return (Transformation|GetSocketTransform _mesh (Utilities|String|StringToName (.Value (Utilities|Map|Find _humanoidbonetable "head"))) TransformSpace) (Transformation|GetSocketTransform _mesh (Utilities|String|StringToName (.Value (Utilities|Map|Find _humanoidbonetable "hips"))) TransformSpace)))

(fn GetEyeRot
  (params (Location :type Vector) (Right :type Float%20%28single-precision%29) (Left :type Float%20%28single-precision%29) (Up :type Float%20%28single-precision%29) (Down :type Float%20%28single-precision%29))
  (bind (_x _y _z) (Math|Vector|BreakVector Location))
  (bind _returnvalue (Math|Float|Absolute(Float) _y))
  (bind _returnvalue_2 (Class|KismetMathLibrary|DegAtan2 _x _returnvalue))
  (bind _returnvalue_3 (Class|KismetMathLibrary|DegAtan2 _z _returnvalue))
  (bind _returnvalue_4 (Math|Float|ClampAngle _returnvalue_2 -9e+01 9e+01))
  (bind _returnvalue_5 (Math|Float|ClampAngle _returnvalue_3 -9e+01 9e+01))
  (return (Math|Rotator|MakeRotator (* _returnvalue_5 (/ 1.0 9e+01) (select (>= _returnvalue_5 0.0) Down Up) -1.0) 0.0 (* _returnvalue_4 (/ 1.0 9e+01) (select (>= _returnvalue_4 0.0) Left Right) -1.0))))