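; Base character Blueprint that displays a VRM avatar over a VRoidSimple-animated body mesh, with facial behaviour and ragdoll.
; SetVrmData spawns an MToon actor, attaches it to Mesh and uses VrmAnimInstanceCopy to copy the body's pose onto the avatar.
; A timeline drives randomly timed blink morphs, also forced by quick gaze changes.
; SetLookAtTarget computes per-eye angles, feeding both the AnimBP's bone look-at and VRM Look blendshapes.
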(event Custom|SetVrmData
  (params (VRMAssetList :type Vrm%20Asset%20List%20Object%20Object%20Reference))
  ;[1 1 1] VRM Set
  (Utilities|FlowControl|Sequence
    (:then_0
      (Variables|Default|SetVRMAssetList VRMAssetList))
    (:then_1
      (Utilities|FlowControl|Sequence
        (:then_0
          (bind _returnvalue (Game|SpawnActorfromClass (Variables|Default|GetMToonClass) (Transformation|GetActorTransform) "Undefined" 0 (Variables|Default|GetVRMAssetList) self 0))
          (bind _output_get (Variables|Default|SetMToonActor _returnvalue))
          (Utilities|FlowControl|Sequence
            (:then_0
              (Utilities|FlowControl|Delay 0.2)
              (Default|ChangeBaseCharacterActor _output_get self))
            (:then_1
              (Components|SkeletalMesh|SetAnimInstanceClass (Variables|/VRM4U/Util/BaseCharacter/Misc/MToonActor_old.MToonActor_old_C|GetSkeletalMesh (Variables|Default|GetMToonActor)) "/Script/VRM4U.VrmAnimInstanceCopy")
              (CallFunction|CalcMainBone "RTS_Component")
              (Class|Actor|AddActorWorldRotation (Variables|Default|GetMToonActor) "0,-90.000000, 0")
              (Transformation|AddRelativeLocation (Variables|/VRM4U/Util/BaseCharacter/Misc/MToonActor_old.MToonActor_old_C|GetSkeletalMesh (Variables|Default|GetMToonActor)) (Math|Vector|MakeVector 0.0 0.0 0.0) false true)
              (Transformation|AttachComponentToComponent (Variables|Default|GetMToonActor) (Variables|Character|GetMesh) "None" "SnapToTarget" "SnapToTarget" "SnapToTarget" true)
              (Collision|SetCollisionEnabled (Variables|/VRM4U/Util/BaseCharacter/Misc/MToonActor_old.MToonActor_old_C|GetSkeletalMesh (Variables|Default|GetMToonActor)) "NoCollision"))))
        (:then_1
          (bind _asvrm_anim_instance_copy (Utilities|Casting|CastToVrmAnimInstanceCopy (Components|SkeletalMesh|GetAnimInstance (Variables|/VRM4U/Util/BaseCharacter/Misc/MToonActor_old.MToonActor_old_C|GetSkeletalMesh (Variables|Default|GetMToonActor)))))
          (Class|VrmAnimInstanceCopy|SetSkeletalMeshCopyData _asvrm_anim_instance_copy (Variables|Default|GetVRMAssetList) (Variables|Character|GetMesh) "/VRM4U/Util/BaseCharacter/Mesh/VRoidSimple_VrmAssetList.VRoidSimple_VrmAssetList"))
        (:then_3
          (Variables|/VRM4U/Util/BaseCharacter/Misc/MToonActor_old.MToonActor_old_C|SetShadowmapDistance (Variables|Default|GetMToonActor) 1e+03))))
    (:then_4
      (Collision|SetCollisionEnabled (Variables|/VRM4U/Util/BaseCharacter/Misc/MToonActor_old.MToonActor_old_C|GetSkeletalMesh (Variables|Default|GetMToonActor)) "QueryAndPhysics")
      (Collision|SetCollisionResponsetoAllChannels (Variables|/VRM4U/Util/BaseCharacter/Misc/MToonActor_old.MToonActor_old_C|GetSkeletalMesh (Variables|Default|GetMToonActor)) "ECR_Ignore"))))

(event Custom|SetLookAtTarget
  (params (TargetLocation :type Vector))
  (bind _mesh (Variables|Character|GetMesh))
  (bind _mesh_2 (Variables|Character|GetMesh))
  (bind _mtoonactor (Variables|Default|GetMToonActor))
  (bind _mtoonactor_2 (Variables|Default|GetMToonActor))
  (bind _returnvalue (Transformation|GetSocketLocation _mesh "head"))
  (bind _skeletalmesh (Variables|/VRM4U/Util/BaseCharacter/Misc/MToonActor_old.MToonActor_old_C|GetSkeletalMesh _mtoonactor))
  (bind _skeletalmesh_2 (Variables|/VRM4U/Util/BaseCharacter/Misc/MToonActor_old.MToonActor_old_C|GetSkeletalMesh _mtoonactor_2))
  (bind _returnvalue_2 (- TargetLocation _returnvalue))
  (bind _returnvalue_3 (Math|Vector|Normalize _returnvalue_2))
  ;[1 1 1] LookAt
  (Utilities|FlowControl|Sequence
    (:then_0
      (Utilities|FlowControl|Sequence
        (:then_0
          (Variables|Default|SetEyeRight (CallFunction|GetEyeRot (Math|Transform|InverseTransformLocation (Transformation|GetSocketTransform _mesh_2 "J_Adj_R_FaceEyeSet" "RTS_World") TargetLocation) 12.0 8.0 1e+01 1e+01))
          (Variables|Default|SetEyeLeft (CallFunction|GetEyeRot (Math|Transform|InverseTransformLocation (Transformation|GetSocketTransform _mesh_2 "J_Adj_L_FaceEyeSet" "RTS_World") TargetLocation) 8.0 12.0 1e+01 1e+01)))))
    (:then_1
      ;[1 1 1] bone
      (Default|SetTargetLocationOrg (Variables|Default|GetAnimBP) TargetLocation (Variables|Default|GetEyeRight) (Variables|Default|GetEyeLeft) false))
    (:then_3
      ;[1 1 1] blendshape
      (bind _array_element (Utilities|Array|ForEachLoopwithBreak (Variables|/Script/VRM4U.VrmMetaObject|GetBlendShapeGroup (Variables|/Script/VRM4U.VrmAssetListObject|GetVrmMetaObject (Variables|Default|GetVRMAssetList))))
        (:LoopBody
          (switch string (.name (Utilities|Struct|BreakVrmBlendShapeGroup _array_element))
            (:LookLeft
              (for _array_element_2 (.BlendShape (Utilities|Struct|BreakVrmBlendShapeGroup _array_element))
                (Components|SkeletalMesh|SetMorphTarget _skeletalmesh_2 (Utilities|String|StringToName (.morphTargetName (Utilities|Struct|BreakVrmBlendShape _array_element_2))) (/ (Math|Float|Clamp(Float) (.Z (Math|Vector|BreakVector (Math|Vector|Lerp(Vector) (Math|Vector|MakeVector (.Roll (Math|Rotator|BreakRotator (Variables|Default|GetEyeRight))) (.Pitch (Math|Rotator|BreakRotator (Variables|Default|GetEyeRight))) (.Yaw (Math|Rotator|BreakRotator (Variables|Default|GetEyeRight)))) (Math|Vector|MakeVector (.Roll (Math|Rotator|BreakRotator (Variables|Default|GetEyeLeft))) (.Pitch (Math|Rotator|BreakRotator (Variables|Default|GetEyeLeft))) (.Yaw (Math|Rotator|BreakRotator (Variables|Default|GetEyeLeft)))) 0.5))) -5.0 0.0) -5.0) true)))
            (:LookRight
              (for _array_element_3 (.BlendShape (Utilities|Struct|BreakVrmBlendShapeGroup _array_element))
                (Components|SkeletalMesh|SetMorphTarget _skeletalmesh_2 (Utilities|String|StringToName (.morphTargetName (Utilities|Struct|BreakVrmBlendShape _array_element_3))) (/ (Math|Float|Clamp(Float) 0.0 5.0 (.Z (Math|Vector|BreakVector (Math|Vector|Lerp(Vector) (Math|Vector|MakeVector (.Roll (Math|Rotator|BreakRotator (Variables|Default|GetEyeRight))) (.Pitch (Math|Rotator|BreakRotator (Variables|Default|GetEyeRight))) (.Yaw (Math|Rotator|BreakRotator (Variables|Default|GetEyeRight)))) (Math|Vector|MakeVector (.Roll (Math|Rotator|BreakRotator (Variables|Default|GetEyeLeft))) (.Pitch (Math|Rotator|BreakRotator (Variables|Default|GetEyeLeft))) (.Yaw (Math|Rotator|BreakRotator (Variables|Default|GetEyeLeft)))) 0.5)))) 5.0) true)))
            (:LookUp
              (for _array_element_4 (.BlendShape (Utilities|Struct|BreakVrmBlendShapeGroup _array_element))
                (Components|SkeletalMesh|SetMorphTarget _skeletalmesh (Utilities|String|StringToName (.morphTargetName (Utilities|Struct|BreakVrmBlendShape _array_element_4))) (/ (Math|Float|Clamp(Float) (.X (Math|Vector|BreakVector (Math|Vector|Lerp(Vector) (Math|Vector|MakeVector (.Roll (Math|Rotator|BreakRotator (Variables|Default|GetEyeRight))) (.Pitch (Math|Rotator|BreakRotator (Variables|Default|GetEyeRight))) (.Yaw (Math|Rotator|BreakRotator (Variables|Default|GetEyeRight)))) (Math|Vector|MakeVector (.Roll (Math|Rotator|BreakRotator (Variables|Default|GetEyeLeft))) (.Pitch (Math|Rotator|BreakRotator (Variables|Default|GetEyeLeft))) (.Yaw (Math|Rotator|BreakRotator (Variables|Default|GetEyeLeft)))) 0.5))) -5.0 0.0) -5.0) true)))
            (:LookDown
              (for _array_element_5 (.BlendShape (Utilities|Struct|BreakVrmBlendShapeGroup _array_element))
                (Components|SkeletalMesh|SetMorphTarget _skeletalmesh (Utilities|String|StringToName (.morphTargetName (Utilities|Struct|BreakVrmBlendShape _array_element_5))) (/ (Math|Float|Clamp(Float) (.X (Math|Vector|BreakVector (Math|Vector|Lerp(Vector) (Math|Vector|MakeVector (.Roll (Math|Rotator|BreakRotator (Variables|Default|GetEyeRight))) (.Pitch (Math|Rotator|BreakRotator (Variables|Default|GetEyeRight))) (.Yaw (Math|Rotator|BreakRotator (Variables|Default|GetEyeRight)))) (Math|Vector|MakeVector (.Roll (Math|Rotator|BreakRotator (Variables|Default|GetEyeLeft))) (.Pitch (Math|Rotator|BreakRotator (Variables|Default|GetEyeLeft))) (.Yaw (Math|Rotator|BreakRotator (Variables|Default|GetEyeLeft)))) 0.5))) 0.0 5.0) 5.0) true)))))))
    (:then_4
      (Math|Float|CompareFloat (Math|Float|Absolute(Float) (Math|Vector|DotProduct _returnvalue_3 (Variables|Default|GetLatestLookAtDir))) 0.998
        (:<
          (CallFunction|ForceBlink))))
    (:then_5
      (Variables|Default|SetLatestLookAtDir _returnvalue_3))))

(event Custom|ForceBlink
  (bind _mesh (Variables|Character|GetMesh))
  ;[1 1 1] Blink
  (Utilities|FlowControl|DoOnce false :!label _label
    (:Completed
      (bind _newtrack_0 (Timeline|Timeline_0 PlayFromStart)
        (:Update
          (bind _array_element (Utilities|Array|ForEachLoopwithBreak (Variables|/Script/VRM4U.VrmMetaObject|GetBlendShapeGroup (Variables|/Script/VRM4U.VrmAssetListObject|GetVrmMetaObject (Variables|Default|GetVRMAssetList))) :!label _label_2)
            (:LoopBody
              (if (Utilities|Enum|Equal(Enum) (.name (Utilities|Struct|BreakVrmBlendShapeGroup _array_element)) "Blink")
                (Utilities|FlowControl|Sequence
                  (:then_0
                    (bind _array_element_2 (Utilities|Array|ForEachLoopwithBreak (.BlendShape (Utilities|Struct|BreakVrmBlendShapeGroup _array_element)))
                      (:LoopBody
                        (Components|SkeletalMesh|SetMorphTarget (Variables|/VRM4U/Util/BaseCharacter/Misc/MToonActor_old.MToonActor_old_C|GetSkeletalMesh (Variables|Default|GetMToonActor)) (Utilities|String|StringToName (.morphTargetName (Utilities|Struct|BreakVrmBlendShape _array_element_2))) _newtrack_0 true))))
                  (:then_1
                    (if (Rendering|IsVisible _mesh)
                      (Components|SkeletalMesh|SetMorphTarget _mesh "Face.M_F00_000_Fcl_EYE_Close" _newtrack_0 true)))
                  (:then_2
                    (goto _label_2 Break)))))))
        (:Finished
          (Utilities|FlowControl|Sequence
            (:then_0
              (Utilities|FlowControl|Sequence
                (:then_2
                  (Utilities|FlowControl|Sequence
                    (:then_0
                      (goto _label Reset))
                    (:then_1
                      (Utilities|FlowControl|RetriggerableDelay (Math|Random|RandomFloatinRange 1.0 6.0))
                      (goto _label))))))
            (:then_1
              (Class|SkeletalMeshComponent|ClearMorphTargets (Variables|/VRM4U/Util/BaseCharacter/Misc/MToonActor_old.MToonActor_old_C|GetSkeletalMesh (Variables|Default|GetMToonActor))))))))))

(event Custom|ToRagdoll
  (bind _mesh (Variables|Character|GetMesh))
  (Collision|SetCollisionEnabled _mesh "QueryAndPhysics")
  (Collision|SetCollisionResponsetoAllChannels _mesh "ECR_Ignore")
  (Class|SkeletalMeshComponent|SetAllBodiesSimulatePhysics _mesh true)
  (Utilities|FlowControl|Sequence
    (:then_0
      (for _array_element (Utilities|Array|MakeArray "ECC_WorldStatic" "ECC_WorldDynamic")
        (Collision|SetCollisionResponsetoChannel _mesh _array_element "ECR_Block")))))

(event EventBeginPlay
  (Utilities|FlowControl|Sequence
    (:then_2
      (Development|SetHiddeninGame (Variables|Default|GetPreviewMesh) true false))
    (:then_3
      (Variables|Default|SetAnimBP (.AsABP%20VRoid%20Simple (Utilities|Casting|CastToABP_VRoidSimple (Components|SkeletalMesh|GetAnimInstance (Variables|Character|GetMesh))))))
    (:then_4
      (bind _vrmassetlist (Variables|Default|GetVRMAssetList)
        (:then
          (CallFunction|SetVrmData _vrmassetlist))
        (:else)))))

(event Collision|EventActorBeginOverlap
  (params (OtherActor :type Actor%20Object%20Reference)))

(event EventTick
  (params (DeltaSeconds :type Float%20%28single-precision%29))
  (bind _mesh (Variables|Character|GetMesh))
  (Utilities|FlowControl|Sequence
    (:then_4
      ;[1 1 1] Blink
      (Utilities|FlowControl|DoOnce false
        (:Completed
          (Utilities|FlowControl|Sequence :!label _label
            (:then_2
              (Utilities|FlowControl|Sequence
                (:then_0
                  (goto _label_2 Reset))
                (:then_1
                  (Utilities|FlowControl|RetriggerableDelay (Math|Random|RandomFloatinRange 1.0 6.0))
                  (Utilities|FlowControl|DoOnce false :!label _label_2
                    (:Completed
                      (bind _newtrack_0 (Timeline|Timeline_0 PlayFromStart)
                        (:Update
                          (bind _array_element (Utilities|Array|ForEachLoopwithBreak (Variables|/Script/VRM4U.VrmMetaObject|GetBlendShapeGroup (Variables|/Script/VRM4U.VrmAssetListObject|GetVrmMetaObject (Variables|Default|GetVRMAssetList))) :!label _label_3)
                            (:LoopBody
                              (if (Utilities|Enum|Equal(Enum) (.name (Utilities|Struct|BreakVrmBlendShapeGroup _array_element)) "Blink")
                                (Utilities|FlowControl|Sequence
                                  (:then_0
                                    (bind _array_element_2 (Utilities|Array|ForEachLoopwithBreak (.BlendShape (Utilities|Struct|BreakVrmBlendShapeGroup _array_element)))
                                      (:LoopBody
                                        (Components|SkeletalMesh|SetMorphTarget (Variables|/VRM4U/Util/BaseCharacter/Misc/MToonActor_old.MToonActor_old_C|GetSkeletalMesh (Variables|Default|GetMToonActor)) (Utilities|String|StringToName (.morphTargetName (Utilities|Struct|BreakVrmBlendShape _array_element_2))) _newtrack_0 true))))
                                  (:then_1
                                    (if (Rendering|IsVisible _mesh)
                                      (Components|SkeletalMesh|SetMorphTarget _mesh "Face.M_F00_000_Fcl_EYE_Close" _newtrack_0 true)))
                                  (:then_2
                                    (goto _label_3 Break)))))))
                        (:Finished
                          (Utilities|FlowControl|Sequence
                            (:then_0
                              (goto _label))
                            (:then_1
                              (Class|SkeletalMeshComponent|ClearMorphTargets (Variables|/VRM4U/Util/BaseCharacter/Misc/MToonActor_old.MToonActor_old_C|GetSkeletalMesh (Variables|Default|GetMToonActor))))))))))))))))))

(fn ConstructionScript
  (bind _vrmassetlist (Variables|Default|GetVRMAssetList)
    (:then
      (Class|SkinnedMeshComponent|SetSkeletalMesh (Variables|Default|GetPreviewMesh) (Variables|/Script/VRM4U.VrmAssetListObject|GetSkeletalMesh _vrmassetlist) true))
    (:else)))

(fn CalcMainBone
  (params (TransformSpace :type ERelativeTransformSpace%20Enum :default "RTS_World"))
  (bind _mtoonactor (Variables|Default|GetMToonActor))
  (bind _skeletalmesh (Variables|/VRM4U/Util/BaseCharacter/Misc/MToonActor_old.MToonActor_old_C|GetSkeletalMesh _mtoonactor))
  (bind _vrmmeta (Variables|/VRM4U/Util/BaseCharacter/Misc/MToonActor_old.MToonActor_old_C|GetVRMMeta _mtoonactor))
  (bind _humanoidbonetable (Variables|/Script/VRM4U.VrmMetaObject|GethumanoidBoneTable _vrmmeta))
  (return (Transformation|GetSocketTransform _skeletalmesh (Utilities|String|StringToName (.Value (Utilities|Map|Find _humanoidbonetable "head"))) TransformSpace) (Transformation|GetSocketTransform _skeletalmesh (Utilities|String|StringToName (.Value (Utilities|Map|Find _humanoidbonetable "hips"))) TransformSpace)))

(fn GetEyeRot
  (params (Location :type Vector) (Right :type Float%20%28single-precision%29) (Left :type Float%20%28single-precision%29) (Up :type Float%20%28single-precision%29) (Down :type Float%20%28single-precision%29))
  (bind (_x _y _z) (Math|Vector|BreakVector Location))
  (bind _returnvalue (Math|Float|Absolute(Float) _y))
  (bind _returnvalue_2 (Class|KismetMathLibrary|DegAtan2 _x _returnvalue))
  (bind _returnvalue_3 (Class|KismetMathLibrary|DegAtan2 _z _returnvalue))
  (bind _returnvalue_4 (Math|Float|ClampAngle _returnvalue_2 -9e+01 9e+01))
  (bind _returnvalue_5 (Math|Float|ClampAngle _returnvalue_3 -9e+01 9e+01))
  (return (Math|Rotator|MakeRotator (* _returnvalue_5 (/ 1.0 9e+01) (select (>= _returnvalue_5 0.0) Down Up) -1.0) 0.0 (* _returnvalue_4 (/ 1.0 9e+01) (select (>= _returnvalue_4 0.0) Left Right) -1.0))))