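; BP_ModelAttach is a utility actor for a VRM character model that links an MToon attach actor to itself.
; Construction enables shadow casting, calls Init and clears RefreshDummy, which appears to serve as a refresh toggle.
; Init targets the child MToonAttachActor at this actor, then snaps to a valid VRMParent's transform and reinitializes its MToon attach actor.
; UpdatePose toggles skeletal mesh visibility twice, apparently to force a pose refresh.
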(event Custom|UpdatePose
  (bind _skeletalmeshcomponent (Variables|SkeletalMeshActor|GetSkeletalMeshComponent))
  (Rendering|ToggleVisibility _skeletalmeshcomponent false)
  (Rendering|ToggleVisibility _skeletalmeshcomponent false))

(event Custom|init
  (Utilities|FlowControl|Sequence
    (:then_0
      (Variables|/VRM4U/Util/Actor/MToonAttachActor.MToonAttachActor_C|SetTargetByActor (.AsMToon%20Attach%20Actor (Utilities|Casting|CastToMToonAttachActor (Variables|/Script/Engine.ChildActorComponent|GetChildActor (Variables|Default|GetChildActor)))) self))
    (:then_1
      (bind _vrmparent (Variables|Default|GetVRMParent)
        (:then
          (Utilities|FlowControl|Sequence
            (:then_0
              (Transformation|SetActorTransform self (Transformation|GetActorTransform _vrmparent)))
            (:then_1
              (Default|ReInitMToonAttachActor _vrmparent))))
        (:else)))))

(event EventBeginPlay)

(event Collision|EventActorBeginOverlap
  (params (OtherActor :type Actor%20Object%20Reference)))

(event EventTick
  (params (DeltaSeconds :type Float%20%28single-precision%29)))

(fn ConstructionScript
  (Utilities|FlowControl|Sequence
    (:then_0
      (Rendering|SetCastShadow (Variables|SkeletalMeshActor|GetSkeletalMeshComponent) true))
    (:then_1
      (CallFunction|Init))
    (:then_2
      (Variables|Default|SetRefreshDummy false))))