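; Component that poses a VRM character by feeding stored limb, head and humanoid bone transforms into the ABP_VRoidSimple instance on the master actor's source mesh.
; Tick copies the transforms each frame, but BeginPlay disables ticking if the rig actor is missing or ignored.
; UpdatePose also pushes them and sets adjust, head and all-bone modes, handling anim-init binding for updates before BeginPlay.
; ResetPose sets limb and head transforms to identity.
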(event Custom|UpdatePose
  (params (AdjustMode :type Float%20%28single-precision%29) (isHeadTrans :type Boolean) (IsHeadRot :type Boolean) (isAllBone :type Boolean))
  (bind _master (Variables|Default|Getmaster))
  (bind _skeletalmeshcomponent_src (Variables|/VRM4U/Util/BaseCharacter/BP_VrmModelActor.BP_VrmModelActor_C|GetSkeletalMeshComponent_Src _master))
  (Utilities|FlowControl|Sequence
    (:then_0
      (bind _asabp_vroid_simple (Utilities|Casting|CastToABP_VRoidSimple (Components|SkeletalMesh|GetAnimInstance (Variables|/VRM4U/Util/BaseCharacter/BP_VrmModelActor.BP_VrmModelActor_C|GetSkeletalMeshComponent_Src (Variables|Default|Getmaster)))))
      (Utilities|FlowControl|Sequence
        (:then_3
          (Variables|/VRM4U/Util/BaseCharacter/Mesh/ABP_VRoidSimple.ABP_VRoidSimple_C|Setadj_LeftHand _asabp_vroid_simple (Variables|Default|GetT_LeftHand))
          (Variables|/VRM4U/Util/BaseCharacter/Mesh/ABP_VRoidSimple.ABP_VRoidSimple_C|Setadj_LeftLowerArm _asabp_vroid_simple (Variables|Default|GetT_LeftLower))
          (Variables|/VRM4U/Util/BaseCharacter/Mesh/ABP_VRoidSimple.ABP_VRoidSimple_C|Setadj_RightHand _asabp_vroid_simple (Variables|Default|GetT_RightHand))
          (Variables|/VRM4U/Util/BaseCharacter/Mesh/ABP_VRoidSimple.ABP_VRoidSimple_C|Setadj_RightLowerArm _asabp_vroid_simple (Variables|Default|GetT_RightLower))
          (Variables|/VRM4U/Util/BaseCharacter/Mesh/ABP_VRoidSimple.ABP_VRoidSimple_C|Setadj_LeftFoot _asabp_vroid_simple (Variables|Default|GetT_LeftFoot))
          (Variables|/VRM4U/Util/BaseCharacter/Mesh/ABP_VRoidSimple.ABP_VRoidSimple_C|Setadj_LeftLeg _asabp_vroid_simple (Variables|Default|GetT_LeftLeg))
          (Variables|/VRM4U/Util/BaseCharacter/Mesh/ABP_VRoidSimple.ABP_VRoidSimple_C|Setadj_RightFoot _asabp_vroid_simple (Variables|Default|GetT_RightFoot))
          (Variables|/VRM4U/Util/BaseCharacter/Mesh/ABP_VRoidSimple.ABP_VRoidSimple_C|Setadj_RightLeg _asabp_vroid_simple (Variables|Default|GetT_RightLeg))
          (Variables|/VRM4U/Util/BaseCharacter/Mesh/ABP_VRoidSimple.ABP_VRoidSimple_C|Sethead_relative _asabp_vroid_simple (Variables|Default|GetT_Head))
          (Variables|/VRM4U/Util/BaseCharacter/Mesh/ABP_VRoidSimple.ABP_VRoidSimple_C|Sethead_rot _asabp_vroid_simple (Variables|Default|GetR_Head)))
        (:then_4
          (Variables|/VRM4U/Util/BaseCharacter/Mesh/ABP_VRoidSimple.ABP_VRoidSimple_C|SetVRMHumanoidBone _asabp_vroid_simple (Variables|Default|GetVRMBoneTransform)))))
    (:then_1
      (if (Variables|Default|GetbBeginCalled)
        (EventDispatchers|UnbindEventfromOnAnimInitialized _skeletalmeshcomponent_src (delegate Custom|CustomEvent))
        (else
          (EventDispatchers|AssignOnAnimInitialized _skeletalmeshcomponent_src (delegate Custom|CustomEvent)))))
    (:then_3
      (bind _asabp_vroid_simple_2 (Utilities|Casting|CastToABP_VRoidSimple (Components|SkeletalMesh|GetAnimInstance (Variables|/VRM4U/Util/BaseCharacter/BP_VrmModelActor.BP_VrmModelActor_C|GetSkeletalMeshComponent_Src (Variables|Default|Getmaster)))))
      (Utilities|FlowControl|Sequence
        (:then_1
          (Variables|/VRM4U/Util/BaseCharacter/Mesh/ABP_VRoidSimple.ABP_VRoidSimple_C|SetAdjustMode _asabp_vroid_simple_2 (select (or (> (Math|Vector|VectorLength (.Location (Math|Transform|BreakTransform (Variables|Default|GetT_LeftHand)))) 0.1) isAllBone) AdjustMode 0.0)))
        (:then_2
          (Variables|/VRM4U/Util/BaseCharacter/Mesh/ABP_VRoidSimple.ABP_VRoidSimple_C|SetTargetVrmModelActor _asabp_vroid_simple_2 (Variables|Default|Getmaster)))
        (:then_3
          (Variables|/VRM4U/Util/BaseCharacter/Mesh/ABP_VRoidSimple.ABP_VRoidSimple_C|SetIsHeadRot _asabp_vroid_simple_2 IsHeadRot)
          (Variables|/VRM4U/Util/BaseCharacter/Mesh/ABP_VRoidSimple.ABP_VRoidSimple_C|SetIsHeadTrans _asabp_vroid_simple_2 isHeadTrans))
        (:then_5
          (Variables|/VRM4U/Util/BaseCharacter/Mesh/ABP_VRoidSimple.ABP_VRoidSimple_C|SetHumanoidAllBoneRate _asabp_vroid_simple_2 (select isAllBone 1.0 0.0)))))))

(event Custom|CustomEvent
  (if (not (Variables|Default|GetbBeginCalled))
    (Class|VrmBPFunctionLibrary|VRMInitAnim (Variables|/VRM4U/Util/BaseCharacter/BP_VrmModelActor.BP_VrmModelActor_C|GetSkeletalMeshComponent_Dst (Variables|Default|Getmaster)))))

(event Custom|SetMasterActor
  (params (Master :type BP%20Vrm%20Model%20Actor%20Object%20Reference))
  (Variables|Default|Setmaster Master))

(event Custom|SetRigActor
  (params (RigRoot :type Character%20Pose%20Rig%20Object%20Reference))
  (Variables|Default|SetRigActor RigRoot))

(event Custom|ResetPose
  (Utilities|FlowControl|Sequence
    (:then_0
      (bind _output_get (Variables|Default|SetT_LeftHand (Math|Transform|MakeTransform "0, 0, 0")))
      (bind _output_get_2 (Variables|Default|SetT_LeftLower _output_get))
      (bind _output_get_3 (Variables|Default|SetT_RightHand _output_get_2))
      (bind _output_get_4 (Variables|Default|SetT_RightLower _output_get_3))
      (bind _output_get_5 (Variables|Default|SetT_LeftFoot _output_get_4))
      (bind _output_get_6 (Variables|Default|SetT_LeftLeg _output_get_5))
      (bind _output_get_7 (Variables|Default|SetT_RightFoot _output_get_6))
      (bind _output_get_8 (Variables|Default|SetT_RightLeg _output_get_7))
      (Variables|Default|SetT_Head _output_get_8))))

(event EventTick
  (params (DeltaSeconds :type Float%20%28single-precision%29))
  (|CallParentFunction DeltaSeconds)
  (bind _asabp_vroid_simple (Utilities|Casting|CastToABP_VRoidSimple (Components|SkeletalMesh|GetAnimInstance (Variables|/VRM4U/Util/BaseCharacter/BP_VrmModelActor.BP_VrmModelActor_C|GetSkeletalMeshComponent_Src (Variables|Default|Getmaster)))))
  (Utilities|FlowControl|Sequence
    (:then_3
      (Variables|/VRM4U/Util/BaseCharacter/Mesh/ABP_VRoidSimple.ABP_VRoidSimple_C|Setadj_LeftHand _asabp_vroid_simple (Variables|Default|GetT_LeftHand))
      (Variables|/VRM4U/Util/BaseCharacter/Mesh/ABP_VRoidSimple.ABP_VRoidSimple_C|Setadj_LeftLowerArm _asabp_vroid_simple (Variables|Default|GetT_LeftLower))
      (Variables|/VRM4U/Util/BaseCharacter/Mesh/ABP_VRoidSimple.ABP_VRoidSimple_C|Setadj_RightHand _asabp_vroid_simple (Variables|Default|GetT_RightHand))
      (Variables|/VRM4U/Util/BaseCharacter/Mesh/ABP_VRoidSimple.ABP_VRoidSimple_C|Setadj_RightLowerArm _asabp_vroid_simple (Variables|Default|GetT_RightLower))
      (Variables|/VRM4U/Util/BaseCharacter/Mesh/ABP_VRoidSimple.ABP_VRoidSimple_C|Setadj_LeftFoot _asabp_vroid_simple (Variables|Default|GetT_LeftFoot))
      (Variables|/VRM4U/Util/BaseCharacter/Mesh/ABP_VRoidSimple.ABP_VRoidSimple_C|Setadj_LeftLeg _asabp_vroid_simple (Variables|Default|GetT_LeftLeg))
      (Variables|/VRM4U/Util/BaseCharacter/Mesh/ABP_VRoidSimple.ABP_VRoidSimple_C|Setadj_RightFoot _asabp_vroid_simple (Variables|Default|GetT_RightFoot))
      (Variables|/VRM4U/Util/BaseCharacter/Mesh/ABP_VRoidSimple.ABP_VRoidSimple_C|Setadj_RightLeg _asabp_vroid_simple (Variables|Default|GetT_RightLeg))
      (Variables|/VRM4U/Util/BaseCharacter/Mesh/ABP_VRoidSimple.ABP_VRoidSimple_C|Sethead_relative _asabp_vroid_simple (Variables|Default|GetT_Head))
      (Variables|/VRM4U/Util/BaseCharacter/Mesh/ABP_VRoidSimple.ABP_VRoidSimple_C|Sethead_rot _asabp_vroid_simple (Variables|Default|GetR_Head)))
    (:then_4
      (Variables|/VRM4U/Util/BaseCharacter/Mesh/ABP_VRoidSimple.ABP_VRoidSimple_C|SetVRMHumanoidBone _asabp_vroid_simple (Variables|Default|GetVRMBoneTransform)))))

(event EventBeginPlay
  (bind _rigactor (Variables|Default|GetRigActor)
    (:then
      (if (Variables|/VRM4U/Util/Actor/CharacterPoseRig.CharacterPoseRig_C|GetbIgnore _rigactor)
        (Components|Tick|SetComponentTickEnabled false :!label _label)
        (else
          (Variables|Default|SetbBeginCalled true)
          (CallFunction|UpdatePose 1.0 false false false))))
    (:else
      (goto _label))))