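; Helper actor that adds a cast shadow to a target VRM character, using either planes or a duplicate mesh.
; Init runs from construction and BeginPlay, resolving the target through BPVrmUtilComponent, removing the unused shadow components and snap-attaching to the target mesh.
; In mesh mode, VrmPoseableMesh copies the skeletal mesh and follows its pose via master pose.
; Its dynamic M_CastShadow material, created only outside BeginPlay, receives color, alpha and light-distance settings.
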(event Custom|init
  (bind _bp_vrmutilcomponent (Variables|Default|GetBP_VrmUtilComponent))
  (bind _vrmposeablemesh (Variables|Default|GetVrmPoseableMesh))
  (Utilities|FlowControl|Sequence
    (:then_0
      (Variables|Default|SetPreview%28Auto%29 0))
    (:then_1
      (Variables|Default|GetTargetActor
        (:then
          (Utilities|FlowControl|Sequence
            (:then_0
              (Default|SetActor (Variables|Default|GetBP_VrmUtilComponent) (Variables|Default|GetTargetActor)))
            (:then_1
              (if (Variables|Default|GetShadowTexture)
                (Components|DestroyComponent (Variables|Default|GetVrmPoseableMesh))
                (else
                  (Utilities|FlowControl|Sequence
                    (:then_0
                      (Components|DestroyComponent (Variables|Default|GetPlane1)))
                    (:then_1
                      ;[1 1 1] same model
                      (Utilities|FlowControl|Sequence
                        (:then_0
                          (bind _vrmassetlist (Variables|/VRM4U/Util/Actor/Misc/sub/BP_VrmUtilComponent.BP_VrmUtilComponent_C|GetVrmAssetList _bp_vrmutilcomponent)
                            (:then
                              (Class|SkinnedMeshComponent|SetSkeletalMesh _vrmposeablemesh (Variables|/Script/VRM4U.VrmAssetListObject|GetSkeletalMesh _vrmassetlist) true))
                            (:else
                              (Class|SkinnedMeshComponent|SetSkeletalMesh _vrmposeablemesh (Variables|/Script/Engine.SkinnedMeshComponent|GetSkeletalMesh (Variables|/VRM4U/Util/Actor/Misc/sub/BP_VrmUtilComponent.BP_VrmUtilComponent_C|GetTargetMeshComponent _bp_vrmutilcomponent)) true))))
                        (:then_1
                          (if (not (Variables|Default|GetcallFromBegin))
                            (bind _returnvalue (Rendering|Material|CreateDynamicMaterialInstance "/VRM4U/Util/BaseCharacter/Misc/M_CastShadow.M_CastShadow" "None" :!class /Script/Engine.KismetMaterialLibrary))
                            (Variables|Default|SetShadowMat _returnvalue)
                            ;[1 1 1] material init
                            (for (_array_element _array_index) (Variables|/Script/Engine.SkeletalMesh|GetMaterials (Variables|/Script/Engine.SkinnedMeshComponent|GetSkeletalMesh (Variables|Default|GetVrmPoseableMesh)))
                              (Rendering|Material|SetMaterial (Variables|Default|GetVrmPoseableMesh) _array_index _returnvalue))))))))))
            (:then_3
              (bind _vrmposeablemesh_2 (Variables|Default|GetVrmPoseableMesh)
                (:then
                  (Class|SkinnedMeshComponent|SetMasterPoseComponent _vrmposeablemesh_2 (Variables|/VRM4U/Util/Actor/Misc/sub/BP_VrmUtilComponent.BP_VrmUtilComponent_C|GetTargetMeshComponent (Variables|Default|GetBP_VrmUtilComponent)) true))
                (:else)))))
        (:else
          (bind _vrmposeablemesh_3 (Variables|Default|GetVrmPoseableMesh)
            (:then
              (Components|DestroyComponent _vrmposeablemesh_3))
            (:else)))))
    (:then_2
      (bind _targetmeshcomponent (Variables|/VRM4U/Util/Actor/Misc/sub/BP_VrmUtilComponent.BP_VrmUtilComponent_C|GetTargetMeshComponent (Variables|Default|GetBP_VrmUtilComponent))
        (:then
          (Variables|Default|SetPreview%28Auto%29 (Variables|/Script/Engine.SkinnedMeshComponent|GetSkeletalMesh _targetmeshcomponent))
          (Transformation|AttachComponentToComponent self _targetmeshcomponent "None" "SnapToTarget" "SnapToTarget" "SnapToTarget" true))
        (:else)))
    (:then_3
      (bind _shadowmat (Variables|Default|GetShadowMat)
        (:then
          (Rendering|Material|SetVectorParameterValue _shadowmat "ShadowColor" (Variables|Default|GetShadowColor) :!class /Script/Engine.MaterialInstanceDynamic)
          (Rendering|Material|SetScalarParameterValue _shadowmat "AlphaOffset" (Variables|Default|GetAlphaOffset) :!class /Script/Engine.MaterialInstanceDynamic)
          (Rendering|Material|SetScalarParameterValue _shadowmat "AlphaFade" (Variables|Default|GetAlphaFade) :!class /Script/Engine.MaterialInstanceDynamic)
          (Rendering|Material|SetScalarParameterValue _shadowmat "LightDistance" (Variables|Default|GetLightDistance) :!class /Script/Engine.MaterialInstanceDynamic))
        (:else)))))

(event EventBeginPlay
  (bind _bp_vrmutilcomponent (Variables|Default|GetBP_VrmUtilComponent))
  (bind _vrmposeablemesh (Variables|Default|GetVrmPoseableMesh))
  (Variables|Default|SetcallFromBegin true)
  (Utilities|FlowControl|Sequence
    (:then_0
      (Variables|Default|SetPreview%28Auto%29 0))
    (:then_1
      (Variables|Default|GetTargetActor
        (:then
          (Utilities|FlowControl|Sequence
            (:then_0
              (Default|SetActor (Variables|Default|GetBP_VrmUtilComponent) (Variables|Default|GetTargetActor)))
            (:then_1
              (if (Variables|Default|GetShadowTexture)
                (Components|DestroyComponent (Variables|Default|GetVrmPoseableMesh))
                (else
                  (Utilities|FlowControl|Sequence
                    (:then_0
                      (Components|DestroyComponent (Variables|Default|GetPlane1)))
                    (:then_1
                      ;[1 1 1] same model
                      (Utilities|FlowControl|Sequence
                        (:then_0
                          (bind _vrmassetlist (Variables|/VRM4U/Util/Actor/Misc/sub/BP_VrmUtilComponent.BP_VrmUtilComponent_C|GetVrmAssetList _bp_vrmutilcomponent)
                            (:then
                              (Class|SkinnedMeshComponent|SetSkeletalMesh _vrmposeablemesh (Variables|/Script/VRM4U.VrmAssetListObject|GetSkeletalMesh _vrmassetlist) true))
                            (:else
                              (Class|SkinnedMeshComponent|SetSkeletalMesh _vrmposeablemesh (Variables|/Script/Engine.SkinnedMeshComponent|GetSkeletalMesh (Variables|/VRM4U/Util/Actor/Misc/sub/BP_VrmUtilComponent.BP_VrmUtilComponent_C|GetTargetMeshComponent _bp_vrmutilcomponent)) true))))
                        (:then_1
                          (if (not (Variables|Default|GetcallFromBegin))
                            (bind _returnvalue (Rendering|Material|CreateDynamicMaterialInstance "/VRM4U/Util/BaseCharacter/Misc/M_CastShadow.M_CastShadow" "None" :!class /Script/Engine.KismetMaterialLibrary))
                            (Variables|Default|SetShadowMat _returnvalue)
                            ;[1 1 1] material init
                            (for (_array_element _array_index) (Variables|/Script/Engine.SkeletalMesh|GetMaterials (Variables|/Script/Engine.SkinnedMeshComponent|GetSkeletalMesh (Variables|Default|GetVrmPoseableMesh)))
                              (Rendering|Material|SetMaterial (Variables|Default|GetVrmPoseableMesh) _array_index _returnvalue))))))))))
            (:then_3
              (bind _vrmposeablemesh_2 (Variables|Default|GetVrmPoseableMesh)
                (:then
                  (Class|SkinnedMeshComponent|SetMasterPoseComponent _vrmposeablemesh_2 (Variables|/VRM4U/Util/Actor/Misc/sub/BP_VrmUtilComponent.BP_VrmUtilComponent_C|GetTargetMeshComponent (Variables|Default|GetBP_VrmUtilComponent)) true))
                (:else)))))
        (:else
          (bind _vrmposeablemesh_3 (Variables|Default|GetVrmPoseableMesh)
            (:then
              (Components|DestroyComponent _vrmposeablemesh_3))
            (:else)))))
    (:then_2
      (bind _targetmeshcomponent (Variables|/VRM4U/Util/Actor/Misc/sub/BP_VrmUtilComponent.BP_VrmUtilComponent_C|GetTargetMeshComponent (Variables|Default|GetBP_VrmUtilComponent))
        (:then
          (Variables|Default|SetPreview%28Auto%29 (Variables|/Script/Engine.SkinnedMeshComponent|GetSkeletalMesh _targetmeshcomponent))
          (Transformation|AttachComponentToComponent self _targetmeshcomponent "None" "SnapToTarget" "SnapToTarget" "SnapToTarget" true))
        (:else)))
    (:then_3
      (bind _shadowmat (Variables|Default|GetShadowMat)
        (:then
          (Rendering|Material|SetVectorParameterValue _shadowmat "ShadowColor" (Variables|Default|GetShadowColor) :!class /Script/Engine.MaterialInstanceDynamic)
          (Rendering|Material|SetScalarParameterValue _shadowmat "AlphaOffset" (Variables|Default|GetAlphaOffset) :!class /Script/Engine.MaterialInstanceDynamic)
          (Rendering|Material|SetScalarParameterValue _shadowmat "AlphaFade" (Variables|Default|GetAlphaFade) :!class /Script/Engine.MaterialInstanceDynamic)
          (Rendering|Material|SetScalarParameterValue _shadowmat "LightDistance" (Variables|Default|GetLightDistance) :!class /Script/Engine.MaterialInstanceDynamic))
        (:else)))))

(event Collision|EventActorBeginOverlap
  (params (OtherActor :type Actor%20Object%20Reference)))

(event EventTick
  (params (DeltaSeconds :type Float%20%28single-precision%29)))

(fn ConstructionScript
  (Utilities|FlowControl|Sequence
    (:then_0
      (CallFunction|Init))))