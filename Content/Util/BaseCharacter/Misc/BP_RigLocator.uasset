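; BP_RigLocator is a cube handle actor for one humanoid bone, used to pose a VRM character rig in the editor.
; Its construction script pushes edits to RootRig, locks rotation-only handles to the rotate gizmo on selection, and index-tags finger materials.
; GetBoneTransform applies the cube's change from its initial pose to the source bone pose.
; Locators attach hierarchically, storing initial relative transforms that ResetInitPos restores recursively, keeping current rotation and scale.
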(event Custom|CustomEvent_0
  (Default|UpdateBone (Variables|Default|GetRootRig) self))

(event Custom|SetParentActor
  (params (ParentActor :type Actor%20Object%20Reference))
  (bind _output_get (Variables|Default|SetParentActor ParentActor))
  (Transformation|AttachActorToActor _output_get "None" "KeepWorld" "KeepWorld" "KeepRelative" true)
  (Variables|Default|SetInitPose_relative (Transformation|GetRelativeTransform (Variables|Default|GetCube)))
  (Variables|Default|Setinitialized true))

(event Custom|ResetInitPos
  (bind _cube (Variables|Default|GetCube))
  (bind _returnvalue (Transformation|GetRelativeTransform _cube))
  (bind (_location _rotation _scale) (Math|Transform|BreakTransform _returnvalue))
  (if (Variables|Default|Getinitialized)
    (Transformation|SetActorRelativeTransform (Math|Transform|MakeTransform (.Location (Math|Transform|BreakTransform (Variables|Default|GetInitPose_relative))) _rotation _scale) false false)
    (for _array_element (Actor|GetAttachedActors self)
      (bind _asbp_rig_locator (Utilities|Casting|CastToBP_RigLocator _array_element))
      (CallFunction|ResetInitPos _asbp_rig_locator)
      (if (Variables|Default|GetbRotationOnly)
        (Class|VrmBPFunctionLibrary|VRMSetWidgetMode "WM_Rotate")))))

(event Custom|SetNearClip
  (params (NearClip :type Float%20%28single-precision%29))
  (Rendering|Material|SetScalarParameterValue (Variables|Default|Getmaterial) "NearClip" NearClip :!class /Script/Engine.MaterialInstanceDynamic))

(event Custom|OnSelectionChangeEvent
  (params (NewParam :type Boolean))
  (Class|VrmBPFunctionLibrary|VRMSetWidgetMode "WM_Rotate"))

(event EventBeginPlay)

(event Collision|EventActorBeginOverlap
  (params (OtherActor :type Actor%20Object%20Reference)))

(event EventTick
  (params (DeltaSeconds :type Float%20%28single-precision%29)))

(fn ConstructionScript
  (bind _humanoidboneno (Variables|Default|GetHumanoidBoneNo))
  (bind _brotationonly (Variables|Default|GetbRotationOnly))
  (bind _vrmeditorevent (Variables|Default|GetVrmEditorEvent))
  (bind _returnvalue (- _humanoidboneno 24))
  (Utilities|FlowControl|Sequence
    (:then_0
      (if _brotationonly
        (EventDispatchers|BindEventtoOnSelectionChange _vrmeditorevent (EventDispatchers|CreateEvent :!event Custom|OnSelectionChangeEvent))
        (else
          (EventDispatchers|UnbindallEventsfromOnSelectionChange _vrmeditorevent))))
    (:then_1
      (Class|VrmEditorEventComponent|SetSelectCheck _vrmeditorevent _brotationonly))
    (:then_2
      (CallFunction|CustomEvent0)
      (if (and (>= _returnvalue 0) (!= _humanoidboneno 54))
        (bind _returnvalue_2 (Rendering|Material|CreateDynamicMaterialInstance (Variables|Default|GetCube) 0 0 "None" :!class /Script/Engine.PrimitiveComponent))
        (bind _output_get (Variables|Default|Setmaterial _returnvalue_2))
        (Rendering|Material|SetScalarParameterValue _returnvalue_2 "Index" (+ (Math|Conversions|ToFloat(Integer) (+ (Math|Integer|%(Integer) (/ _returnvalue 3) 5) 1)) (/ (Math|Conversions|ToFloat(Integer) (+ (Math|Integer|%(Integer) _returnvalue 3) 1)) 1e+01)) :!class /Script/Engine.MaterialInstanceDynamic)))))

(fn GetBoneTransform
  (bind _cube (Variables|Default|GetCube))
  (bind _initpose (Variables|Default|GetInitPose))
  (bind _initpose_tosrc (Variables|Default|GetInitPose_toSrc))
  (bind _returnvalue (Transformation|GetWorldTransform _cube))
  (bind (_location _rotation) (Math|Transform|BreakTransform _initpose_tosrc))
  (bind _returnvalue_2 (Math|Transform|InvertTransform _initpose))
  (bind (_location_2 _rotation_2) (Math|Transform|BreakTransform _returnvalue_2))
  (bind (_location_3 _rotation_3) (Math|Transform|BreakTransform _returnvalue))
  (return (Math|Transform|MakeTransform (+ (- (.Location (Math|Transform|BreakTransform (Variables|Default|GetInitPose_toSrc))) (.Location (Math|Transform|BreakTransform (Variables|Default|GetInitPose)))) _location_3) (.Rotation (Math|Transform|BreakTransform (Math|Transform|ComposeTransforms (Math|Transform|ComposeTransforms (Math|Transform|MakeTransform _location _rotation) (Math|Transform|MakeTransform _location_2 _rotation_2)) (Math|Transform|MakeTransform _location_3 _rotation_3)))))))