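; Actor that mirrors a target actor's pose, on the same model or on an override VRM model.
; Init, run from construction and BeginPlay, drives an override through VrmAnimInstanceCopy and BPVrmAnimControlComponent, otherwise a poseable mesh via master pose.
; It also reinitializes attached MToon actors.
; Optional frame limiting uses an audio-time-quantized Delay loop to copy pose and morphs at reduced rate, with camera attachment between steps.
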(event Custom|init
  (params (dummy :type Boolean))
  (bind _vrmposeablemesh (Variables|Default|GetVrmPoseableMesh))
  (bind _vrmposeablemesh_2 (Variables|Default|GetVrmPoseableMesh))
  (bind _bp_vrmutilcomponent (Variables|Default|GetBP_VrmUtilComponent))
  (bind _targetactor (Variables|Default|GetTargetActor))
  (bind _bp_vrmutilcomponent_2 (Variables|Default|GetBP_VrmUtilComponent))
  (bind _buseperbonemotionblur (Variables|Default|GetbUsePerBoneMotionBlur))
  (bind _skeletalmesh (Variables|Default|GetSkeletalMesh))
  (Utilities|FlowControl|Sequence
    (:then_0
      (Variables|Default|SetPreview%28Auto%29 0))
    (:then_1
      (Variables|Default|GetTargetActor
        (:then
          (Utilities|FlowControl|Sequence
            (:then_0
              (if (Math|Boolean|ORBoolean (!= (Variables|Develop|GetTmpActor) (Variables|Default|GetTargetActor)) (not (Utilities|IsValid (Variables|Develop|GetTmpComponent))) (not (Utilities|IsValid (Variables|Develop|GetTmpVrmAsset))))
                (Utilities|FlowControl|Sequence
                  (:then_0
                    (bind _targetskinnedmeshcomponent (Variables|Default|GetTargetSkinnedMeshComponent)
                      (:then
                        (Default|SetActorbyComponent _bp_vrmutilcomponent _targetskinnedmeshcomponent))
                      (:else
                        (Default|SetActor _bp_vrmutilcomponent _targetactor))))
                  (:then_1
                    (Variables|Default|SetMeshAsSkinnedMesh (Variables|/VRM4U/Util/Actor/Misc/sub/BP_VrmUtilComponent.BP_VrmUtilComponent_C|GetTargetAsSkinnedMeshComponent _bp_vrmutilcomponent_2))
                    (Variables|Develop|SetTmpComponent (Variables|/VRM4U/Util/Actor/Misc/sub/BP_VrmUtilComponent.BP_VrmUtilComponent_C|GetTargetMeshComponent _bp_vrmutilcomponent_2))
                    (Variables|Develop|SetTmpVrmAsset (Variables|/VRM4U/Util/Actor/Misc/sub/BP_VrmUtilComponent.BP_VrmUtilComponent_C|GetVrmAssetList _bp_vrmutilcomponent_2))
                    (Variables|Develop|SetTmpActor _targetactor)))))
            (:then_1
              (Variables|Default|GetAssetListOverride
                (:then)
                (:else
                  (Variables|Default|SetAssetListOverride (Variables|/VRM4U/Util/Actor/Misc/sub/BP_VrmUtilComponent.BP_VrmUtilComponent_C|GetVrmAssetList (Variables|Default|GetBP_VrmUtilComponent))))))
            (:then_3
              (bind _assetlistoverride (Variables|Default|GetAssetListOverride)
                (:then
                  ;[1 1 1] override
                  (Utilities|FlowControl|Sequence
                    (:then_0
                      (Class|SkinnedMeshComponent|SetSkeletalMesh _skeletalmesh (Variables|/Script/VRM4U.VrmAssetListObject|GetSkeletalMesh _assetlistoverride) true)
                      (bind _asvrm_anim_instance_copy (Utilities|Casting|CastToVrmAnimInstanceCopy (Components|SkeletalMesh|GetAnimInstance _skeletalmesh)))
                      (Class|VrmAnimInstanceCopy|SetSkeletalMeshCopyData _asvrm_anim_instance_copy (Variables|Default|GetAssetListOverride) (Variables|Develop|GetTmpComponent) (select (Utilities|IsValid (Variables|Default|GetMeshAsSkinnedMesh)) (Variables|Default|GetMeshAsSkinnedMesh) (Actor|GetComponentbyClass (Variables|Default|GetTargetActor) "/Script/Engine.SkinnedMeshComponent")) (Variables|Develop|GetTmpVrmAsset))
                      (Default|SetSkeleton (Variables|Default|GetBP_VrmAnimControlComponent) (Variables|Develop|GetTmpComponent) (Variables|Default|GetSkeletalMesh) (Variables|Default|GetAssetListOverride))
                      (Variables|/Script/VRM4U.VrmAnimInstanceCopy|SetCenterLocationOffset _asvrm_anim_instance_copy (Variables|Default|GetLocationOffset))
                      (Class|VrmAnimInstanceCopy|SetVrmSpringBoneBool _asvrm_anim_instance_copy (Variables|Default|GetbSkipSpringBone) (Variables|Default|GetbSkipSpringBonePhysicsCollision) false false))
                    (:then_1
                      (for (_array_element _array_index) (Variables|/Script/Engine.SkeletalMesh|GetMaterials (Variables|/Script/VRM4U.VrmAssetListObject|GetSkeletalMesh _assetlistoverride))
                        (Rendering|Material|SetMaterial _skeletalmesh _array_index (.MaterialInterface (Utilities|Struct|BreakSkeletalMaterial _array_element)))))))
                (:else
                  ;[1 1 1] same model
                  (Utilities|FlowControl|Sequence
                    (:then_0
                      (bind _tmpvrmasset (Variables|Develop|GetTmpVrmAsset)
                        (:then
                          (Class|SkinnedMeshComponent|SetSkeletalMesh _vrmposeablemesh_2 (Variables|/Script/VRM4U.VrmAssetListObject|GetSkeletalMesh _tmpvrmasset) true))
                        (:else
                          (Class|SkinnedMeshComponent|SetSkeletalMesh _vrmposeablemesh_2 (Variables|/Script/Engine.SkinnedMeshComponent|GetSkeletalMesh (Variables|Develop|GetTmpComponent)) true))))
                    (:then_2
                      (if (not (Variables|Default|GetbSkipMaterialInit))
                        (if (not (Variables|Develop|GetcallFromBegin))
                          ;[1 1 1] material init
                          (for (_array_element_2 _array_index_2) (Variables|/Script/Engine.SkeletalMesh|GetMaterials (Variables|/Script/Engine.SkinnedMeshComponent|GetSkeletalMesh _vrmposeablemesh))
                            (bind _returnvalue (Rendering|Material|GetBaseMaterial (Rendering|Material|GetMaterial _vrmposeablemesh _array_index_2)))
                            (if (not (or (== _returnvalue (.MaterialInterface (Utilities|Struct|BreakSkeletalMaterial _array_element_2))) (== (Rendering|Material|GetMaterial _vrmposeablemesh _array_index_2) (.MaterialInterface (Utilities|Struct|BreakSkeletalMaterial _array_element_2)))))
                              (Rendering|Material|SetMaterial (Variables|Default|GetVrmPoseableMesh) _array_index_2 (.MaterialInterface (Utilities|Struct|BreakSkeletalMaterial _array_element_2))))))))))))
            (:then_4
              (Utilities|FlowControl|Sequence
                (:then_0
                  (for _array_element_3 (Actor|GetAttachedActors)
                    (bind _asmtoon_attach_actor (Utilities|Casting|CastToMToonAttachActor _array_element_3))
                    (Default|ReInit _asmtoon_attach_actor false)))))
            (:then_5
              (Variables|Default|GetAssetListOverride
                (:then
                  (Default|SetFrameLimit (Variables|Default|GetBP_VrmAnimControlComponent) (Variables|Default|GetEnableFrameLimit) (Variables|Default|GetFrameLimit%20%28frames/sec%29)))
                (:else
                  (if (Variables|Default|GetEnableFrameLimit)
                    (CallFunction|SetFrameLimit (Variables|Default|GetEnableFrameLimit) (Variables|Default|GetFrameLimit%20%28frames/sec%29))
                    (else
                      (Class|SkinnedMeshComponent|SetMasterPoseComponent (Variables|Default|GetVrmPoseableMesh) (Variables|Develop|GetTmpComponent) true))))))
            (:then_6
              (Utilities|FlowControl|Sequence
                (:then_0
                  (Class|VrmBPFunctionLibrary|VRMSetPerBoneMotionBlur (Variables|Default|GetSkeletalMesh) _buseperbonemotionblur)
                  (Class|VrmBPFunctionLibrary|VRMSetPerBoneMotionBlur (Variables|Default|GetVrmPoseableMesh) _buseperbonemotionblur))))))
        (:else
          (Class|SkinnedMeshComponent|SetSkeletalMesh (Variables|Default|GetVrmPoseableMesh) 0 true)
          (Variables|Develop|SetTmpComponent 0)
          (Variables|Develop|SetTmpActor 0)
          (Variables|Develop|SetTmpVrmAsset 0))))
    (:then_2
      (bind _assetlistoverride_2 (Variables|Default|GetAssetListOverride)
        (:then
          (Variables|Default|SetPreview%28Auto%29 (Variables|/Script/VRM4U.VrmAssetListObject|GetSkeletalMesh _assetlistoverride_2)))
        (:else
          (bind _tmpcomponent (Variables|Develop|GetTmpComponent)
            (:then
              (Variables|Default|SetPreview%28Auto%29 (Variables|/Script/Engine.SkinnedMeshComponent|GetSkeletalMesh _tmpcomponent)))
            (:else)))))
    (:then_3
      (bind _targetactor_2 (Variables|Default|GetTargetActor)
        (:then
          (Actor|Tick|AddTickPrerequisiteActor _targetactor_2))
        (:else)))
    (:then_4
      (Rendering|SetVisibility (Variables|Default|GetSkeletalMesh) (Utilities|IsValid (Variables|Default|GetAssetListOverride)) false)
      (Rendering|SetVisibility (Variables|Default|GetVrmPoseableMesh) (not (Utilities|IsValid (Variables|Default|GetAssetListOverride))) false))))

(event EventBeginPlay
  (Variables|Develop|SetcallFromBegin true)
  (CallFunction|Init false))

(event Collision|EventActorBeginOverlap
  (params (OtherActor :type Actor%20Object%20Reference)))

(event EventTick
  (params (DeltaSeconds :type Float%20%28single-precision%29))
  (Utilities|FlowControl|Sequence
    (:then_1
      (if (Variables|Default|GetCopyActorRotation)
        (Transformation|SetActorRotation (Transformation|GetActorRotation (Variables|Default|GetTargetActor)))))))

(event Custom|SetFrameLimit
  (params (bEnable :type Boolean) (FrameToFrame :type Float%20%28single-precision%29))
  (bind _returnvalue (Class|GameplayStatics|GetAudioTimeSeconds))
  (bind _self self)
  (bind _self_2 self)
  (bind _offset_sec_ (Variables|Default|GetOffset%28sec%29))
  (bind _returnvalue_2 (Transformation|GetActorTransform _self))
  (bind _returnvalue_3 (+ _returnvalue _offset_sec_))
  (bind _output_get (Variables|Default|SetEnableFrameLimit bEnable))
  (Variables|Default|SetFrameLimit%20%28frames/sec%29 FrameToFrame)
  (if _output_get
    ;[1 1 1] FrameLimit
    (Utilities|FlowControl|Sequence
      (:then_1
        (Utilities|FlowControl|Delay 0.0 :!label _label)
        (if (.bPlay (Class|VrmBPFunctionLibrary|VRMGetPlayMode)) :!label _label_2
          (if (>= _returnvalue_3 (Variables|Default|GetnextToPlay))
            (Utilities|FlowControl|Sequence
              (:then_0
                (Class|VrmPoseableMeshComponent|VRMCopyPoseandMorphfromSkeletalComponent (Variables|Default|GetVrmPoseableMesh) (Variables|Develop|GetTmpComponent)))
              (:then_1
                (bind _cameraforattach (Variables|Default|GetCameraForAttach)
                  (:then
                    (if (Variables|Default|GetUseAttachparent)
                      (if (== _cameraforattach (Actor|GetAttachParentActor self))
                        ;[1 1 1] Comment
                        (bind _actorforbasetransform (Variables|Default|GetActorForBaseTransform)
                          (:then
                            (Transformation|SetActorTransform _self_2 (Math|Transform|ComposeTransforms (Variables|Default|GetAttachBaseTrans) (Transformation|GetActorTransform _actorforbasetransform))))
                          (:else
                            (Transformation|SetActorTransform _self_2 (Variables|Default|GetAttachBaseTrans))))
                        (else
                          (Utilities|FlowControl|Sequence
                            (:then_0
                              (bind _actorforbasetransform_2 (Variables|Default|GetActorForBaseTransform)
                                (:then
                                  (Variables|Default|SetAttachBaseTrans (Class|KismetMathLibrary|ConvertTransformtoRelative (Transformation|GetActorTransform _actorforbasetransform_2) _returnvalue_2)))
                                (:else
                                  (Variables|Default|SetAttachBaseTrans _returnvalue_2))))
                            (:then_1
                              (Transformation|AttachActorToActor _self _cameraforattach "None" "KeepWorld" "KeepWorld" "KeepWorld" true)))))
                      (elif (== _cameraforattach (Actor|GetAttachParentActor self))
                        (Transformation|DetachFromActor self "KeepWorld" "KeepWorld" "KeepWorld"))))
                  (:else)))
              (:then_2
                (Variables|Default|SetnextToPlay (* (/ 1.0 (Variables|Default|GetFrameLimit%20%28frames/sec%29)) (Math|Conversions|ToFloat(Integer) (Math|Float|Ceil (/ _returnvalue_3 (/ 1.0 (Variables|Default|GetFrameLimit%20%28frames/sec%29)))))))
                (Default|CallOnFrameLimitUpdate)
                (Utilities|FlowControl|Delay 0.0)
                (Utilities|FlowControl|Sequence
                  (:then_0
                    (if (Variables|Default|GetCopyActorTransform)
                      (Transformation|SetWorldTransform (Variables|Default|GetVrmPoseableMesh) (Transformation|GetActorTransform (Variables|Default|GetTargetActor)) false false))
                    (if _output_get
                      (Utilities|FlowControl|Sequence
                        (:then_0
                          (goto _label_2))
                        (:then_1)))))))
            (else
              (goto _label))))))))

(fn ConstructionScript
  (Utilities|FlowControl|Sequence
    (:then_0
      (if (not (Variables|Default|GetbSkipConstructionInit))
        (CallFunction|Init false)))))