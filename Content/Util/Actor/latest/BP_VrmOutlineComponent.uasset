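; VRM outline component, a skeletal mesh that draws an MToon outline over its parent skeletal mesh.
; Init copies the parent's mesh, follows its pose as leader and negates relative scale.
; It assigns the VRM asset's outline materials or generates shared or per-slot dynamic instances, with overrides and excluded slots.
; Generated instances inherit source Z-offset and mask, then receive common width, color and fade distance.
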(event EventBeginPlay)

(event EventTick
  (params (DeltaSeconds :type Float%20%28single-precision%29)))

(event EventInit
  (Utilities|FlowControl|Sequence
    (:then_0
      (Utilities|Array|Clear (Variables|Default|GetMaterialList)))
    (:then_1
      (Components|SkinnedMesh|SetSkinnedAssetandUpdate 0 true)
      (bind _asskeletal_mesh_component (Utilities|Casting|CastToSkeletalMeshComponent (Transformation|GetAttachParent)))
      (if (!= _asskeletal_mesh_component self)
        (Utilities|FlowControl|Sequence
          (:then_0
            (Transformation|SetRelativeScale3D "-1.000000,-1.000000,-1.000000"))
          (:then_1
            (Components|SkinnedMesh|SetSkinnedAssetandUpdate (Class|SkinnedMeshComponent|GetSkinnedAsset _asskeletal_mesh_component) true)
            (Variables|VRM4U|SetVrmAssetList (Class|VrmBPFunctionLibrary|VRMGetVrmAssetListObjectfromAsset (Class|SkinnedMeshComponent|GetSkinnedAsset _asskeletal_mesh_component)))
            (Components|SkinnedMesh|SetLeaderPoseComponent _asskeletal_mesh_component false false))
          (:then_2
            (if (Variables|VRM4U|GetbUseCommonMaterial)
              (Utilities|FlowControl|Sequence :!label _label
                (:then_0
                  (if (Variables|VRM4U|GetbUseSameMaterial)
                    (bind _returnvalue (Rendering|Material|CreateDynamicMaterialInstance "/VRM4U/MaterialUtil/UE5/Material/MI_VrmMToonOptLitOutlineForce.MI_VrmMToonOptLitOutlineForce" "None" "None" :!class /Script/Engine.KismetMaterialLibrary))
                    (Variables|Default|SetMaterialList (Utilities|Array|MakeArray _returnvalue))
                    (for (_array_element _array_index) (Rendering|Material|GetMaterials (Variables|Default|GetLeaderPoseComponent))
                      (if (Utilities|Array|ContainsItem (Variables|VRM4U|GetNoOutlineList) _array_index)
                        (Rendering|Material|SetMaterial _array_index "/VRM4U/MaterialUtil/MToonUtil/M_VrmNone.M_VrmNone")
                        (else
                          (Rendering|Material|SetMaterial _array_index _returnvalue)
                          (CallFunction|SetOutlineParameter _array_element _returnvalue))))
                    (else
                      (for (_array_element_2 _array_index_2) (Rendering|Material|GetMaterials (Variables|Default|GetLeaderPoseComponent))
                        (if (Utilities|Array|ContainsItem (Variables|VRM4U|GetNoOutlineList) _array_index_2)
                          (Rendering|Material|SetMaterial _array_index_2 "/VRM4U/MaterialUtil/MToonUtil/M_VrmNone.M_VrmNone")
                          (elif (.ReturnValue (Utilities|Map|Find (Variables|VRM4U|GetOutlineOverrideMaterial) _array_index_2))
                            (bind _returnvalue_2 (Rendering|Material|CreateDynamicMaterialInstance (.Value (Utilities|Map|Find (Variables|VRM4U|GetOutlineOverrideMaterial) _array_index_2)) "None" "None" :!class /Script/Engine.KismetMaterialLibrary))
                            (Utilities|Array|Add (Variables|Default|GetMaterialList) _returnvalue_2)
                            (Rendering|Material|SetMaterial _array_index_2 _returnvalue_2)
                            (CallFunction|SetOutlineParameter _array_element_2 _returnvalue_2)
                            (else
                              (bind _returnvalue_3 (Rendering|Material|CreateDynamicMaterialInstance "/VRM4U/MaterialUtil/UE5/Material/MI_VrmMToonOptLitOutlineForce.MI_VrmMToonOptLitOutlineForce" "None" "None" :!class /Script/Engine.KismetMaterialLibrary))
                              (Utilities|Array|Add (Variables|Default|GetMaterialList) _returnvalue_3)
                              (Rendering|Material|SetMaterial _array_index_2 _returnvalue_3)
                              (CallFunction|SetOutlineParameter _array_element_2 _returnvalue_3)))))))))
              (else
                (bind _vrmassetlist (Variables|VRM4U|GetVrmAssetList)
                  (:then
                    (if (== (Utilities|Array|Length (Variables|/Script/VRM4U.VrmAssetListObject|GetOutlineMaterials _vrmassetlist)) (Utilities|Array|Length (Rendering|Material|GetMaterials)))
                      (for (_array_element_3 _array_index_3) (Variables|/Script/VRM4U.VrmAssetListObject|GetOutlineMaterials _vrmassetlist)
                        (if (Utilities|Array|ContainsItem (Variables|VRM4U|GetNoOutlineList) _array_index_3)
                          (Rendering|Material|SetMaterial _array_index_3 "/VRM4U/MaterialUtil/MToonUtil/M_VrmNone.M_VrmNone")
                          (else
                            (Rendering|Material|SetMaterial _array_index_3 _array_element_3))))
                      (else
                        (goto _label))))
                  (:else
                    (goto _label)))))))))
    (:then_2
      (for _array_element_4 (Variables|Default|GetMaterialList)
        (Rendering|Material|SetScalarParameterValue _array_element_4 "mtoon_OutlineWidth" (Variables|VRM4U|GetCommonWidth) :!class /Script/Engine.MaterialInstanceDynamic)
        (Rendering|Material|SetScalarParameterValue _array_element_4 "OutlineFadeDistance" (Variables|VRM4U|GetOutlineFadeDistance) :!class /Script/Engine.MaterialInstanceDynamic)
        (Rendering|Material|SetVectorParameterValue _array_element_4 "mtoon_OutlineColor" (Variables|VRM4U|GetCommonColor) :!class /Script/Engine.MaterialInstanceDynamic)))))

(fn SetOutlineParameter
  (params (SrcMaterial :type Material%20Interface%20Object%20Reference%20%28by%20ref%29) (DstMID :type Material%20Instance%20Dynamic%20Object%20Reference%20%28by%20ref%29))
  (Utilities|FlowControl|Sequence
    (:then_0
      (Utilities|FlowControl|Sequence
        (:then_0
          (bind _asmaterial_instance_constant (Utilities|Casting|CastToMaterialInstanceConstant SrcMaterial))
          (Utilities|FlowControl|Sequence
            (:then_0
              (bind _returnvalue (Rendering|Material|GetScalarParameterValue _asmaterial_instance_constant "ZOffset" :!class /Script/Engine.MaterialInstanceConstant))
              (bind _returnvalue_2 (Rendering|Material|GetScalarParameterValue _asmaterial_instance_constant "ZOffsetScale_Depth" :!class /Script/Engine.MaterialInstanceConstant))
              (LocalVariables|SetNewLocalVar (* _returnvalue_2 _returnvalue)))
            (:then_1
              (bind _returnvalue_3 (Rendering|Material|GetTextureParameterValue _asmaterial_instance_constant "ZOffsetMaskTexture" :!class /Script/Engine.MaterialInstanceConstant))
              (LocalVariables|SetNewLocalVar_0 _returnvalue_3))))
        (:then_1
          (bind _asmaterial_instance_dynamic (Utilities|Casting|CastToMaterialInstanceDynamic SrcMaterial))
          (Utilities|FlowControl|Sequence
            (:then_0
              (bind _returnvalue_4 (Rendering|Material|GetScalarParameterValue _asmaterial_instance_dynamic "ZOffset" :!class /Script/Engine.MaterialInstanceDynamic))
              (bind _returnvalue_5 (Rendering|Material|GetScalarParameterValue _asmaterial_instance_dynamic "ZOffsetScale_Depth" :!class /Script/Engine.MaterialInstanceDynamic))
              (LocalVariables|SetNewLocalVar (* _returnvalue_5 _returnvalue_4)))
            (:then_1
              (bind _returnvalue_6 (Rendering|Material|GetTextureParameterValue _asmaterial_instance_dynamic "ZOffsetMaskTexture" :!class /Script/Engine.MaterialInstanceDynamic))
              (LocalVariables|SetNewLocalVar_0 _returnvalue_6))))))
    (:then_1
      (bind _returnvalue_7 (Rendering|Material|GetScalarParameterValue DstMID "ZOffset" :!class /Script/Engine.MaterialInstanceDynamic))
      (Rendering|Material|SetScalarParameterValue DstMID "ZOffset" (+ _returnvalue_7 (* (LocalVariables|GetNewLocalVar) 1.0)) :!class /Script/Engine.MaterialInstanceDynamic)
      (Rendering|Material|SetTextureParameterValue DstMID "ZOffsetMaskTexture" (LocalVariables|GetNewLocalVar_0)))))