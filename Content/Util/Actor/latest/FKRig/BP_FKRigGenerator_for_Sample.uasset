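; BP_FKRigGenerator_for_Sample is a sample FK rig generator Blueprint that feeds bone overrides to a VRoid FK rig.
; Its AddKeyOverride event casts the target anim instance to ABP_VRoidFKRig, then either adds a key/value pair to that instance's BoneData map or, when Clear is set, empties the map.
; The construction script only calls its parent, and the default BeginPlay, overlap and Tick events are disabled.
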(event EventBeginPlay
  (|CallParentFunction) ; This node is disabled and will not be called.\nDrag off pins to build functionality.
)

(event Collision|EventActorBeginOverlap
  (params (OtherActor :type Actor%20Object%20Reference))
  (|CallParentFunction OtherActor) ; This node is disabled and will not be called.\nDrag off pins to build functionality.
)

(event EventTick
  (params (DeltaSeconds :type Float%20%28single-precision%29))
  (|CallParentFunction DeltaSeconds) ; This node is disabled and will not be called.\nDrag off pins to build functionality.
)

(event EventAddKeyOverride
  (params (Key :type String%20%28by%20ref%29) (Value :type Transform%20%28by%20ref%29) (bClear :type Boolean))
  (bind _asabp_vroid_fkrig (Utilities|Casting|CastToABP_VRoidFKRig (CallFunction|GetTargetAnimInstance)))
  (if bClear
    (Utilities|Map|Clear (Variables|/VRM4U/Util/BaseCharacter/Mesh/ABP_VRoidFKRig.ABP_VRoidFKRig_C|GetBoneData _asabp_vroid_fkrig))
    (else
      (Utilities|Map|Add (Variables|/VRM4U/Util/BaseCharacter/Mesh/ABP_VRoidFKRig.ABP_VRoidFKRig_C|GetBoneData _asabp_vroid_fkrig) Key Value))))

(fn ConstructionScript
  (|CallParentFunction))