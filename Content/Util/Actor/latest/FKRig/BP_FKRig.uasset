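; Rig handle actor that visualizes one bone, linked to a parent actor, in what appears to be an FK rig.
; When ready, init notifies its Controller and stretches the bone model between parent and self using midpoint, look-at and distance scaling.
; A shared dynamic material on cube and cylinder drives humanoid-bone tint and alpha, while ShowRig toggles actor scale.
; A helper returns the relative transform between parent and self.
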(event Custom|init
  (bind _returnvalue (Transformation|GetActorLocation))
  (bind _parent (Variables|Default|GetParent))
  (bind _returnvalue_2 (Transformation|GetActorLocation _parent))
  (Utilities|FlowControl|Sequence
    (:then_0
      (if (Variables|Default|GetbReady)
        (Utilities|FlowControl|Sequence
          (:then_0
            (bind _controller (Variables|Default|GetController)
              (:then
                (Default|OnUpdateRig _controller self))
              (:else)))
          (:then_1
            (Transformation|SetWorldTransform (Variables|Default|GetScene1) (Math|Transform|MakeTransform (Math|Vector|Lerp(Vector) _returnvalue_2 _returnvalue 0.5) (Math|Rotator|FindLookatRotation _returnvalue_2 _returnvalue) (Math|Vector|MakeVector 1.0 1.0 (Math|Float|Max(Float) (Math|Vector|Distance(Vector) _returnvalue_2 _returnvalue) 0.01))) false false)))))
    (:then_1
      (Variables|Default|GetMaterial
        (:then)
        (:else
          (bind _returnvalue_3 (Rendering|Material|CreateDynamicMaterialInstance "/VRM4U/Util/Actor/latest/FKRig/M_RigMaterial.M_RigMaterial" "None" "None" :!class /Script/Engine.KismetMaterialLibrary))
          (bind _output_get (Variables|Default|SetMaterial _returnvalue_3))
          (Rendering|Material|SetMaterial (Variables|Default|GetCube) 0 _output_get))))))

(event Custom|UpdateBoneModel
  (bind _returnvalue (Transformation|GetActorLocation))
  (bind _parent (Variables|Default|GetParent))
  (bind _returnvalue_2 (Transformation|GetActorLocation _parent))
  (Transformation|SetWorldTransform (Variables|Default|GetScene1) (Math|Transform|MakeTransform (Math|Vector|Lerp(Vector) _returnvalue_2 _returnvalue 0.5) (Math|Rotator|FindLookatRotation _returnvalue_2 _returnvalue) (Math|Vector|MakeVector 1.0 1.0 (Math|Float|Max(Float) (Math|Vector|Distance(Vector) _returnvalue_2 _returnvalue) 0.01))) false false))

(event Custom|SetHumanoidBone
  (bind _material (Variables|Default|GetMaterial)
    (:then
      (Rendering|Material|SetVectorParameterValue _material "Color" "(R=0.500000,G=0.500000,B=0.500000,A=0.900000)" :!class /Script/Engine.MaterialInstanceDynamic))
    (:else)))

(event Custom|ShowRig
  (params (Visible :type Boolean) (Alpha :type Float%20%28single-precision%29))
  (Transformation|SetActorScale3D (Math|Vector|SelectVector "1.000000,1.000000,1.000000" "0.100000,0.100000,0.100000" Visible))
  (bind _material (Variables|Default|GetMaterial)
    (:then
      (Rendering|Material|SetScalarParameterValue _material "Alpha" Alpha :!class /Script/Engine.MaterialInstanceDynamic))
    (:else)))

(event EventBeginPlay)

(event Collision|EventActorBeginOverlap
  (params (OtherActor :type Actor%20Object%20Reference)))

(event EventTick
  (params (DeltaSeconds :type Float%20%28single-precision%29)))

(fn ConstructionScript
  (CallFunction|Init))

(fn GetRelativeTranfsormParent
  (Utilities|FlowControl|Sequence
    (:then_2
      (return (Class|KismetMathLibrary|ConvertTransformtoRelative (Transformation|GetActorTransform (Variables|Default|GetParent)) (Transformation|GetActorTransform))))))