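; VRM4U utility actor that generates an FK control rig for a target skeletal mesh, for posing and animation baking.
; Spawns one BP_FKRig actor per bone, attached to mirror the bone hierarchy, optionally excluding VRM humanoid bones from the driven list.
; Rig updates pass parent-relative transforms by bone name to AddKey_Override, which is only a stub here.
; Numbered events generate, reapply, reset and bake via VRMBakeAnim.
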(event Custom|1_GenerateRig
  (bind _target (Variables|Default|GetTarget))
  (bind _skeletalmeshcomponent (Variables|/Script/Engine.SkeletalMeshActor|GetSkeletalMeshComponent _target))
  ;[1 1 1] Generate
  (bind _target_2 (Variables|Default|GetTarget)
    (:then
      (Components|SkeletalMesh|SetUpdateAnimationinEditor (Variables|/Script/Engine.SkeletalMeshActor|GetSkeletalMeshComponent _target_2) true)
      (Utilities|FlowControl|Sequence
        (:then_2
          (Default|SetActor (Variables|Default|GetBP_VrmUtilComponent) _target_2))
        (:then_3
          (Variables|Development|GetRootRig
            (:then)
            (:else
              (bind _returnvalue (Game|SpawnActorfromClass "/VRM4U/Util/Actor/latest/FKRig/BP_FKRig.BP_FKRig_C" (Math|Transform|MakeTransform "0, 0, 0") "Undefined" 0 self 0))
              (bind _output_get (Variables|Development|SetRootRig _returnvalue))
              (Class|VrmBPFunctionLibrary|VRMSetActorLabel _output_get "rig_SkeletalMeshRoot"))))
        (:then_4
          (bind _rootrig (Variables|Development|GetRootRig)
            (:then
              (Transformation|AttachActorToActor _rootrig (Variables|Default|GetTarget) "None" "SnapToTarget" "SnapToTarget" "SnapToTarget" true))
            (:else)))
        (:then_5
          (Utilities|FlowControl|Sequence
            (:then_0
              (for _index (range 0 (- (Class|SkinnedMeshComponent|GetNumBones _skeletalmeshcomponent) 1))
                (if (.ReturnValue (Utilities|Map|Find (Variables|Development|GetBoneRigList_All) (Class|SkinnedMeshComponent|GetBoneName _skeletalmeshcomponent _index)))
                  (Transformation|SetActorTransform (.Value (Utilities|Map|Find (Variables|Development|GetBoneRigList_All) (Class|SkinnedMeshComponent|GetBoneName _skeletalmeshcomponent _index))) (Transformation|GetSocketTransform _skeletalmeshcomponent (Class|SkinnedMeshComponent|GetBoneName _skeletalmeshcomponent _index) "RTS_World"))
                  (else
                    (bind _returnvalue_2 (Game|SpawnActorfromClass "/VRM4U/Util/Actor/latest/FKRig/BP_FKRig.BP_FKRig_C" (Transformation|GetSocketTransform _skeletalmeshcomponent (Class|SkinnedMeshComponent|GetBoneName _skeletalmeshcomponent _index) "RTS_World") "Undefined" 0 self 0))
                    (Utilities|FlowControl|Sequence
                      (:then_0
                        (Utilities|Map|Add (Variables|Development|GetBoneRigList_All) (Class|SkinnedMeshComponent|GetBoneName _skeletalmeshcomponent _index) _returnvalue_2)
                        (Class|VrmBPFunctionLibrary|VRMSetActorLabel _returnvalue_2 (Utilities|String|Append "rig_" (Utilities|String|ToString(Name) (Class|SkinnedMeshComponent|GetBoneName _skeletalmeshcomponent _index))))
                        (Variables|/VRM4U/Util/Actor/latest/FKRig/BP_FKRig.BP_FKRig_C|SetParent _returnvalue_2 (select (.ReturnValue (Utilities|Map|Find (Variables|Development|GetBoneRigList_All) (Class|SkinnedMeshComponent|GetParentBone _skeletalmeshcomponent (Class|SkinnedMeshComponent|GetBoneName _skeletalmeshcomponent _index)))) (.Value (Utilities|Map|Find (Variables|Development|GetBoneRigList_All) (Class|SkinnedMeshComponent|GetParentBone _skeletalmeshcomponent (Class|SkinnedMeshComponent|GetBoneName _skeletalmeshcomponent _index)))) (Variables|Development|GetRootRig))))
                      (:then_1
                        (Transformation|AttachActorToActor _returnvalue_2 (select (.ReturnValue (Utilities|Map|Find (Variables|Development|GetBoneRigList_All) (Class|SkinnedMeshComponent|GetParentBone _skeletalmeshcomponent (Class|SkinnedMeshComponent|GetBoneName _skeletalmeshcomponent _index)))) (.Value (Utilities|Map|Find (Variables|Development|GetBoneRigList_All) (Class|SkinnedMeshComponent|GetParentBone _skeletalmeshcomponent (Class|SkinnedMeshComponent|GetBoneName _skeletalmeshcomponent _index)))) (Variables|Development|GetRootRig)) "None" "KeepWorld" "KeepWorld" "KeepWorld" true))))))
              (Variables|Development|SetBoneRigList (Variables|Development|GetBoneRigList_All)))
            (:then_1
              ;[1 1 1] remove humanoid
              (if (Variables|Default|GetbSkipHumanoidBone)
                (bind _vrmassetlist (Variables|/VRM4U/Util/Actor/Misc/sub/BP_VrmUtilComponent.BP_VrmUtilComponent_C|GetVrmAssetList (Variables|Default|GetBP_VrmUtilComponent))
                  (:then
                    (bind _keys (Utilities|Map|Keys (Variables|Development|GetBoneRigList)))
                    (bind _values (Utilities|Map|Values (Variables|/Script/VRM4U.VrmMetaObject|GethumanoidBoneTable (Variables|/Script/VRM4U.VrmAssetListObject|GetVrmMetaObject _vrmassetlist))))
                    (for _array_element _keys
                      (if (>= (Utilities|Array|FindItem _values (Utilities|String|ToString(Name) _array_element)) 0)
                        (Default|SetHumanoidBone (.Value (Utilities|Map|Find (Variables|Development|GetBoneRigList) _array_element)))
                        (Utilities|Map|Remove (Variables|Development|GetBoneRigList) _array_element))))
                  (:else))))))
        (:then_6
          (Utilities|FlowControl|Sequence
            (:then_1
              (bind _values_2 (Utilities|Map|Values (Variables|Development|GetBoneRigList_All)))
              (for _array_element_2 _values_2
                (Variables|/VRM4U/Util/Actor/latest/FKRig/BP_FKRig.BP_FKRig_C|SetbReady _array_element_2 true)
                (Default|UpdateBoneModel _array_element_2)))))))
    (:else)))

(event Custom|3_Reset
  ;[1 1 1] reset
  (Utilities|FlowControl|Sequence
    (:then_0
      (bind _rootrig (Variables|Development|GetRootRig)
        (:then
          (CallFunction|RemoveChild _rootrig)
          (Utilities|Map|Clear (Variables|Development|GetBoneRigList))
          (Utilities|Map|Clear (Variables|Development|GetBoneRigList_All)))
        (:else)))
    (:then_1
      (CallFunction|AddKeyOverride (Utilities|String|MakeLiteralString) (Math|Transform|MakeTransform "0, 0, 0") true))))

(event Custom|2_ForceApply
  (bind _boneriglist (Variables|Development|GetBoneRigList))
  ;[1 1 1] apply
  (Variables|Default|GetTarget
    (:then
      (Utilities|FlowControl|Sequence
        (:then_0
          (Utilities|Map|Keys _boneriglist)
          (bind _values (Utilities|Map|Values _boneriglist)))
        (:then_1
          (for _array_element _values
            (CallFunction|OnUpdateRig _array_element)))))
    (:else)))

(event Custom|4_Bake
  (Class|VrmBPFunctionLibrary|VRMBakeAnim (Variables|/Script/Engine.SkeletalMeshActor|GetSkeletalMeshComponent (Variables|Default|GetTarget)) (Variables|Default|GetBakePath) (Variables|Default|GetBakeFileName)))

(event Custom|init
  (params (NewParam :type Boolean))
  ;[1 1 1] Alpha
  (Utilities|FlowControl|Sequence
    (:then_0
      (bind _values (Utilities|Map|Values (Variables|Development|GetBoneRigList_All)))
      (for _array_element _values
        (Default|ShowRig _array_element (Variables|Default|GetbShowRig) (Variables|Default|GetAlpha))))
    (:then_1
      (bind _target (Variables|Default|GetTarget)
        (:then
          (Components|SkeletalMesh|SetUpdateAnimationinEditor (Variables|/Script/Engine.SkeletalMeshActor|GetSkeletalMeshComponent _target) true))
        (:else)))
    (:then_2
      (CallFunction|MakeRandBakeFileName))))

(event Custom|OnUpdateRig
  (params (Rig :type BP%20FK%20Rig%20Object%20Reference))
  (bind _boneriglist (Variables|Development|GetBoneRigList))
  ;[1 1 1] callback
  (Utilities|FlowControl|Sequence
    (:then_0
      (bind _values (Utilities|Map|Values _boneriglist))
      (if (>= (Utilities|Array|FindItem _values Rig) 0)
        (bind _keys (Utilities|Map|Keys _boneriglist))
        (CallFunction|AddKeyOverride (Utilities|String|ToString(Name) (Utilities|Array|Get(acopy) _keys (Utilities|Array|FindItem _values Rig))) (Default|GetRelativeTranfsormParent Rig) false)))))

(event Custom|AddKey_Override
  (params (Key :type String%20%28by%20ref%29) (Value :type Transform%20%28by%20ref%29) (bClear :type Boolean))
  ;[1 1 1] Override
  (Utilities|IsValid (CallFunction|GetTargetAnimInstance)))

(event EventBeginPlay
  (bind _boneriglist (Variables|Development|GetBoneRigList))
  ;[1 1 1] apply
  (Variables|Default|GetTarget
    (:then
      (Utilities|FlowControl|Sequence
        (:then_0
          (Utilities|Map|Keys _boneriglist)
          (bind _values (Utilities|Map|Values _boneriglist)))
        (:then_1
          (for _array_element _values
            (CallFunction|OnUpdateRig _array_element)))))
    (:else)))

(event Collision|EventActorBeginOverlap
  (params (OtherActor :type Actor%20Object%20Reference)))

(event EventTick
  (params (DeltaSeconds :type Float%20%28single-precision%29)))

(fn ConstructionScript
  (CallFunction|Init false))

(fn RemoveChild
  (params (Target :type Actor%20Object%20Reference%20%28by%20ref%29))
  (bind _output_get (LocalVariables|SetNewLocalVar_0 (Actor|GetAttachedActors Target true)))
  (Utilities|FlowControl|Sequence
    (:then_0
      (for _array_element _output_get
        (bind _asbp_rig (Utilities|Casting|CastToBP_FKRig _array_element))
        (CallFunction|RemoveChild _asbp_rig)))
    (:then_1
      (bind _asbp_rig_2 (Utilities|Casting|CastToBP_FKRig Target))
      (Actor|DestroyActor _asbp_rig_2))))

(fn GetTargetAnimInstance
  (Utilities|FlowControl|Sequence
    (:then_0
      (bind _target (Variables|Default|GetTarget)
        (:then
          (LocalVariables|SetNewLocalVar_1 (Class|SkeletalMeshComponent|GetPostProcessInstance (Variables|/Script/Engine.SkeletalMeshActor|GetSkeletalMeshComponent _target))))
        (:else)))
    (:then_1
      (LocalVariables|GetNewLocalVar_1
        (:then)
        (:else
          (LocalVariables|SetNewLocalVar_1 (Components|SkeletalMesh|GetAnimInstance (Variables|/Script/Engine.SkeletalMeshActor|GetSkeletalMeshComponent _target))))))
    (:then_2
      (return (LocalVariables|GetNewLocalVar_1)))))

(fn MakeRandBakeFileName
  (bind _returnvalue (Class|KismetMathLibrary|Today))
  (bind _returnvalue_2 (Class|KismetMathLibrary|GetDay _returnvalue))
  (bind _returnvalue_3 (Class|KismetMathLibrary|GetMonth _returnvalue))
  (if (Utilities|Enum|Equal(Enum) (Variables|Default|GetBakeFileName) "")
    (Utilities|FlowControl|Sequence
      (:then_0
        (for _index (range 0 7)
          (bind _output_get (LocalVariables|SetNewLocalVar_2 (Utilities|String|Append (stale _output_get) (Utilities|String|ToString(Integer) (Math|Random|RandomIntegerinRange 0 9)))))))
      (:then_1
        (Variables|Default|SetBakeFileName (Utilities|String|Append "vrm4u_anim_" (Utilities|String|Append (Utilities|String|ToString(Integer) (Class|KismetMathLibrary|GetYear _returnvalue)) "_" (Utilities|String|ToString(Integer) (/ _returnvalue_3 10)) (Utilities|String|ToString(Integer) (Math|Integer|%(Integer) _returnvalue_3 10)) "_" (Utilities|String|ToString(Integer) (/ _returnvalue_2 10)) (Utilities|String|ToString(Integer) (Math|Integer|%(Integer) _returnvalue_2 10))) "_" (LocalVariables|GetNewLocalVar_2)))))))