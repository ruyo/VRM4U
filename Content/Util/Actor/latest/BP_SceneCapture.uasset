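; BP_SceneCapture is a utility actor that shows captured color overlay, depth and normal scene textures on three static meshes.
; It creates a render target for each, feeds it to a dynamic M_Texture material, and registers it with the VRM4U render subsystem as a capture texture.
; Construction first clears existing captures and extent history, while BeginPlay repeats only the creation and registration.
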(event Custom|init
  (bind _returnvalue (|VRM4URenderSubsystem))
  (bind _returnvalue_2 (|VRM4URenderSubsystem))
  (Utilities|FlowControl|Sequence
    (:then_0
      (Variables|Default|SetFinalColor 0)
      (Variables|Default|SetScenDepth 0)
      (Variables|Default|SetNormal 0)
      (Class|VRM4URenderSubsystem|RemoveAllCaptureTexture _returnvalue)
      (Class|VRM4URenderSubsystem|ResetSceneTextureExtentHistory _returnvalue))
    (:then_1
      (Utilities|FlowControl|Sequence
        (:then_0
          (Utilities|FlowControl|Sequence
            (:then_0
              (bind _returnvalue_3 (Rendering|CreateRenderTarget2D 256 256 "RTF_RGBA16f"))
              (bind _output_get (Variables|Default|SetFinalColor _returnvalue_3))
              (bind _returnvalue_4 (Rendering|Material|CreateDynamicMaterialInstance (Variables|Default|GetStaticMesh) 0 "/VRM4U/Util/Actor/latest/sub/M_Texture.M_Texture" "None" :!class /Script/Engine.PrimitiveComponent))
              (Rendering|Material|SetTextureParameterValue _returnvalue_4 "Texture" _output_get))
            (:then_1
              (bind _returnvalue_5 (Rendering|CreateRenderTarget2D 256 256 "RTF_RGBA16f"))
              (bind _output_get_2 (Variables|Default|SetScenDepth _returnvalue_5))
              (bind _returnvalue_6 (Rendering|Material|CreateDynamicMaterialInstance (Variables|Default|GetStaticMesh1) 0 "/VRM4U/Util/Actor/latest/sub/M_Texture.M_Texture" "None" :!class /Script/Engine.PrimitiveComponent))
              (Rendering|Material|SetTextureParameterValue _returnvalue_6 "Texture" _output_get_2))
            (:then_2
              (bind _returnvalue_7 (Rendering|CreateRenderTarget2D 256 256 "RTF_RGBA16f"))
              (bind _output_get_3 (Variables|Default|SetNormal _returnvalue_7))
              (bind _returnvalue_8 (Rendering|Material|CreateDynamicMaterialInstance (Variables|Default|GetStaticMesh2) 0 "/VRM4U/Util/Actor/latest/sub/M_Texture.M_Texture" "None" :!class /Script/Engine.PrimitiveComponent))
              (Rendering|Material|SetTextureParameterValue _returnvalue_8 "Texture" _output_get_3))))
        (:then_1)
        (:then_2
          (Class|VRM4URenderSubsystem|AddCaptureTexture _returnvalue_2 (Variables|Default|GetFinalColor) "ColorTextureOverlay")
          (Class|VRM4URenderSubsystem|AddCaptureTexture _returnvalue_2 (Variables|Default|GetScenDepth) "DepthTexture")
          (Class|VRM4URenderSubsystem|AddCaptureTexture _returnvalue_2 (Variables|Default|GetNormal) "NormalTexture"))))))

(event EventBeginPlay
  (bind _returnvalue (|VRM4URenderSubsystem))
  (Utilities|FlowControl|Sequence
    (:then_0
      (Utilities|FlowControl|Sequence
        (:then_0
          (bind _returnvalue_2 (Rendering|CreateRenderTarget2D 256 256 "RTF_RGBA16f"))
          (bind _output_get (Variables|Default|SetFinalColor _returnvalue_2))
          (bind _returnvalue_3 (Rendering|Material|CreateDynamicMaterialInstance (Variables|Default|GetStaticMesh) 0 "/VRM4U/Util/Actor/latest/sub/M_Texture.M_Texture" "None" :!class /Script/Engine.PrimitiveComponent))
          (Rendering|Material|SetTextureParameterValue _returnvalue_3 "Texture" _output_get))
        (:then_1
          (bind _returnvalue_4 (Rendering|CreateRenderTarget2D 256 256 "RTF_RGBA16f"))
          (bind _output_get_2 (Variables|Default|SetScenDepth _returnvalue_4))
          (bind _returnvalue_5 (Rendering|Material|CreateDynamicMaterialInstance (Variables|Default|GetStaticMesh1) 0 "/VRM4U/Util/Actor/latest/sub/M_Texture.M_Texture" "None" :!class /Script/Engine.PrimitiveComponent))
          (Rendering|Material|SetTextureParameterValue _returnvalue_5 "Texture" _output_get_2))
        (:then_2
          (bind _returnvalue_6 (Rendering|CreateRenderTarget2D 256 256 "RTF_RGBA16f"))
          (bind _output_get_3 (Variables|Default|SetNormal _returnvalue_6))
          (bind _returnvalue_7 (Rendering|Material|CreateDynamicMaterialInstance (Variables|Default|GetStaticMesh2) 0 "/VRM4U/Util/Actor/latest/sub/M_Texture.M_Texture" "None" :!class /Script/Engine.PrimitiveComponent))
          (Rendering|Material|SetTextureParameterValue _returnvalue_7 "Texture" _output_get_3))))
    (:then_1)
    (:then_2
      (Class|VRM4URenderSubsystem|AddCaptureTexture _returnvalue (Variables|Default|GetFinalColor) "ColorTextureOverlay")
      (Class|VRM4URenderSubsystem|AddCaptureTexture _returnvalue (Variables|Default|GetScenDepth) "DepthTexture")
      (Class|VRM4URenderSubsystem|AddCaptureTexture _returnvalue (Variables|Default|GetNormal) "NormalTexture"))))

(event Collision|EventActorBeginOverlap
  (params (OtherActor :type Actor%20Object%20Reference)))

(event EventTick
  (params (DeltaSeconds :type Float%20%28single-precision%29)))

(fn ConstructionScript
  (CallFunction|Init))