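; Placeable VRM4U actor that defines a rim light filter: color, scale, edge fade or binary edge, search width and light direction.
; BeginPlay and construction clear subsystem filter data at its Priority and build a new filter data object, which Tick refreshes.
; Direction comes from actor rotation or yaw/pitch offsets, optionally camera-relative.
; A camera-move callback keeps the Scene component's rotation aligned when following the camera.
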(event Custom|init
  (bind _returnvalue (Math|Rotator|MakeRotator 0.0 0.0 0.0))
  (bind _returnvalue_2 (Transformation|GetActorRotation))
  (bind _vrmcameracheck (Variables|Default|GetVrmCameraCheck))
  (bind _rotyaw (Variables|Default|GetRotYaw))
  (bind _rotpitch (Variables|Default|GetRotPitch))
  (bind _buseactorrotation (Variables|Default|GetbUseActorRotation))
  (bind _transform (Variables|Default|GetTransform))
  (bind _bfollowcamera (Variables|Default|GetbFollowCamera))
  (bind _bfollowcamera_2 (Variables|Default|GetbFollowCamera))
  (bind _benabled (Variables|Default|GetbEnabled))
  (bind _returnvalue_3 (Math|Rotator|CombineRotators "0.000000,180.000000,0.000000" _returnvalue_2))
  (bind _returnvalue_4 (and _benabled _bfollowcamera_2))
  (bind _returnvalue_5 (select _bfollowcamera (.rotation _transform) _returnvalue))
  (bind (_roll _pitch _yaw) (Math|Rotator|BreakRotator _returnvalue_5))
  (bind _returnvalue_6 (+ _rotyaw _yaw))
  (bind _returnvalue_7 (+ _rotpitch _pitch))
  (bind _returnvalue_8 (Math|Rotator|MakeRotator 0.0 _returnvalue_7 _returnvalue_6))
  (bind _returnvalue_9 (Math|Rotator|SelectRotator _returnvalue_3 _returnvalue_8 _buseactorrotation))
  (if (not (Class|VrmBPFunctionLibrary|VRMIsEditorPreviewObject self))
    (Utilities|FlowControl|Sequence
      (:then_0
        (Class|VRM4URenderSubsystem|RemoveRimFilterDatabyPriority (|VRM4URenderSubsystem) (Variables|Default|GetPriority)))
      (:then_1
        (Class|VrmCameraCheckComponent|SetCameraCheck (Variables|Default|GetVrmCameraCheck) _returnvalue_4)
        (if _returnvalue_4
          (EventDispatchers|AssignOnCameraMove _vrmcameracheck (delegate Custom|OnCameraMove_Event))
          (Class|VrmCameraCheckComponent|SetCameraCheck _vrmcameracheck _returnvalue_4)))
      (:then_2
        (bind _returnvalue_10 (Game|ConstructObjectfromClass "/Script/VRM4URender.VrmExtensionRimFilterData"))
        (bind _output_get (Variables|Default|SetNewVar _returnvalue_10))
        (Utilities|FlowControl|Sequence
          (:then_0
            (Variables|/Script/VRM4URender.VrmExtensionRimFilterData|SetbUseFilter _output_get (Variables|Default|GetbEnabled))
            (Variables|/Script/VRM4URender.VrmExtensionRimFilterData|SetPriority _output_get (Variables|Default|GetPriority)))
          (:then_1
            (Variables|/Script/VRM4URender.VrmExtensionRimFilterData|SetbUseCustomLighColor _output_get (Variables|Default|GetUseCustomLightColor)))
          (:then_2
            (Variables|/Script/VRM4URender.VrmExtensionRimFilterData|SetLightColor _output_get (Variables|Default|GetLightColor))
            (Variables|/Script/VRM4URender.VrmExtensionRimFilterData|SetLightScale _output_get (Variables|Default|GetLightScale)))
          (:then_3
            (Variables|/Script/VRM4URender.VrmExtensionRimFilterData|SetRimEdgeFade _output_get (Variables|Default|GetRim%20Edge%20Fade))
            (Variables|/Script/VRM4URender.VrmExtensionRimFilterData|SetbUseBinaryEdge _output_get (Variables|Default|GetUse%20Binary%20Edge))
            (Variables|/Script/VRM4URender.VrmExtensionRimFilterData|SetRimEdgeBinaryRange _output_get (Variables|Default|GetRim%20Edge%20Binary%20Range)))
          (:then_5
            (Variables|/Script/VRM4URender.VrmExtensionRimFilterData|SetLightDirection _output_get (* (Math|Vector|GetForwardVector _returnvalue_9) (Math|Float|MakeLiteralFloat -1.0)))
            (Variables|/Script/VRM4URender.VrmExtensionRimFilterData|SetSampleScreenScale _output_get (Variables|Default|GetEdgeSearchWidth)))
          (:then_6
            (Utilities|FlowControl|Sequence
              (:then_0
                (Transformation|SetWorldRotation (Variables|Default|GetScene) _returnvalue_9 false false)))))))))

(event Custom|ResetAll
  (Class|VRM4URenderSubsystem|RemoveRimFilterDatabyPriority (|VRM4URenderSubsystem) -1))

(event Custom|OnCameraMove_Event
  (Variables|Default|SetTransform (.transform (Class|VrmBPFunctionLibrary|VRMGetCameraTransform 0 false)))
  (CallFunction|CustomEvent))

(event Custom|CustomEvent
  (bind _returnvalue (Math|Rotator|MakeRotator 0.0 0.0 0.0))
  (bind _transform (Variables|Default|GetTransform))
  (bind _bfollowcamera (Variables|Default|GetbFollowCamera))
  (bind _returnvalue_2 (select _bfollowcamera (.rotation _transform) _returnvalue))
  (bind (_roll _pitch _yaw) (Math|Rotator|BreakRotator _returnvalue_2))
  (Utilities|FlowControl|Sequence
    (:then_0
      (Transformation|SetWorldRotation (Variables|Default|GetScene) (Math|Rotator|SelectRotator (Math|Rotator|CombineRotators "0.000000,180.000000,0.000000" (Transformation|GetActorRotation)) (Math|Rotator|MakeRotator 0.0 (+ (Variables|Default|GetRotPitch) _pitch) (+ (Variables|Default|GetRotYaw) _yaw)) (Variables|Default|GetbUseActorRotation)) false false))))

(event EventBeginPlay
  (bind _returnvalue (Math|Rotator|MakeRotator 0.0 0.0 0.0))
  (bind _returnvalue_2 (Transformation|GetActorRotation))
  (bind _vrmcameracheck (Variables|Default|GetVrmCameraCheck))
  (bind _rotyaw (Variables|Default|GetRotYaw))
  (bind _rotpitch (Variables|Default|GetRotPitch))
  (bind _buseactorrotation (Variables|Default|GetbUseActorRotation))
  (bind _transform (Variables|Default|GetTransform))
  (bind _bfollowcamera (Variables|Default|GetbFollowCamera))
  (bind _bfollowcamera_2 (Variables|Default|GetbFollowCamera))
  (bind _benabled (Variables|Default|GetbEnabled))
  (bind _returnvalue_3 (Math|Rotator|CombineRotators "0.000000,180.000000,0.000000" _returnvalue_2))
  (bind _returnvalue_4 (and _benabled _bfollowcamera_2))
  (bind _returnvalue_5 (select _bfollowcamera (.rotation _transform) _returnvalue))
  (bind (_roll _pitch _yaw) (Math|Rotator|BreakRotator _returnvalue_5))
  (bind _returnvalue_6 (+ _rotyaw _yaw))
  (bind _returnvalue_7 (+ _rotpitch _pitch))
  (bind _returnvalue_8 (Math|Rotator|MakeRotator 0.0 _returnvalue_7 _returnvalue_6))
  (bind _returnvalue_9 (Math|Rotator|SelectRotator _returnvalue_3 _returnvalue_8 _buseactorrotation))
  (if (not (Class|VrmBPFunctionLibrary|VRMIsEditorPreviewObject self))
    (Utilities|FlowControl|Sequence
      (:then_0
        (Class|VRM4URenderSubsystem|RemoveRimFilterDatabyPriority (|VRM4URenderSubsystem) (Variables|Default|GetPriority)))
      (:then_1
        (Class|VrmCameraCheckComponent|SetCameraCheck (Variables|Default|GetVrmCameraCheck) _returnvalue_4)
        (if _returnvalue_4
          (EventDispatchers|AssignOnCameraMove _vrmcameracheck (delegate Custom|OnCameraMove_Event))
          (Class|VrmCameraCheckComponent|SetCameraCheck _vrmcameracheck _returnvalue_4)))
      (:then_2
        (bind _returnvalue_10 (Game|ConstructObjectfromClass "/Script/VRM4URender.VrmExtensionRimFilterData"))
        (bind _output_get (Variables|Default|SetNewVar _returnvalue_10))
        (Utilities|FlowControl|Sequence
          (:then_0
            (Variables|/Script/VRM4URender.VrmExtensionRimFilterData|SetbUseFilter _output_get (Variables|Default|GetbEnabled))
            (Variables|/Script/VRM4URender.VrmExtensionRimFilterData|SetPriority _output_get (Variables|Default|GetPriority)))
          (:then_1
            (Variables|/Script/VRM4URender.VrmExtensionRimFilterData|SetbUseCustomLighColor _output_get (Variables|Default|GetUseCustomLightColor)))
          (:then_2
            (Variables|/Script/VRM4URender.VrmExtensionRimFilterData|SetLightColor _output_get (Variables|Default|GetLightColor))
            (Variables|/Script/VRM4URender.VrmExtensionRimFilterData|SetLightScale _output_get (Variables|Default|GetLightScale)))
          (:then_3
            (Variables|/Script/VRM4URender.VrmExtensionRimFilterData|SetRimEdgeFade _output_get (Variables|Default|GetRim%20Edge%20Fade))
            (Variables|/Script/VRM4URender.VrmExtensionRimFilterData|SetbUseBinaryEdge _output_get (Variables|Default|GetUse%20Binary%20Edge))
            (Variables|/Script/VRM4URender.VrmExtensionRimFilterData|SetRimEdgeBinaryRange _output_get (Variables|Default|GetRim%20Edge%20Binary%20Range)))
          (:then_5
            (Variables|/Script/VRM4URender.VrmExtensionRimFilterData|SetLightDirection _output_get (* (Math|Vector|GetForwardVector _returnvalue_9) (Math|Float|MakeLiteralFloat -1.0)))
            (Variables|/Script/VRM4URender.VrmExtensionRimFilterData|SetSampleScreenScale _output_get (Variables|Default|GetEdgeSearchWidth)))
          (:then_6
            (Utilities|FlowControl|Sequence
              (:then_0
                (Transformation|SetWorldRotation (Variables|Default|GetScene) _returnvalue_9 false false)))))))))

(event Collision|EventActorBeginOverlap
  (params (OtherActor :type Actor%20Object%20Reference)))

(event EventTick
  (params (DeltaSeconds :type Float%20%28single-precision%29))
  (bind _returnvalue (Math|Rotator|MakeRotator 0.0 0.0 0.0))
  (bind _returnvalue_2 (Transformation|GetActorRotation))
  (bind _rotyaw (Variables|Default|GetRotYaw))
  (bind _rotpitch (Variables|Default|GetRotPitch))
  (bind _buseactorrotation (Variables|Default|GetbUseActorRotation))
  (bind _transform (Variables|Default|GetTransform))
  (bind _bfollowcamera (Variables|Default|GetbFollowCamera))
  (bind _returnvalue_3 (Math|Rotator|CombineRotators "0.000000,180.000000,0.000000" _returnvalue_2))
  (bind _returnvalue_4 (select _bfollowcamera (.rotation _transform) _returnvalue))
  (bind (_roll _pitch _yaw) (Math|Rotator|BreakRotator _returnvalue_4))
  (bind _returnvalue_5 (+ _rotyaw _yaw))
  (bind _returnvalue_6 (+ _rotpitch _pitch))
  (bind _returnvalue_7 (Math|Rotator|MakeRotator 0.0 _returnvalue_6 _returnvalue_5))
  (bind _returnvalue_8 (Math|Rotator|SelectRotator _returnvalue_3 _returnvalue_7 _buseactorrotation))
  (Utilities|FlowControl|Sequence
    (:then_0
      (Variables|/Script/VRM4URender.VrmExtensionRimFilterData|SetbUseFilter (stale Custom|init _output_get) (Variables|Default|GetbEnabled))
      (Variables|/Script/VRM4URender.VrmExtensionRimFilterData|SetPriority (stale Custom|init _output_get) (Variables|Default|GetPriority)))
    (:then_1
      (Variables|/Script/VRM4URender.VrmExtensionRimFilterData|SetbUseCustomLighColor (stale Custom|init _output_get) (Variables|Default|GetUseCustomLightColor)))
    (:then_2
      (Variables|/Script/VRM4URender.VrmExtensionRimFilterData|SetLightColor (stale Custom|init _output_get) (Variables|Default|GetLightColor))
      (Variables|/Script/VRM4URender.VrmExtensionRimFilterData|SetLightScale (stale Custom|init _output_get) (Variables|Default|GetLightScale)))
    (:then_3
      (Variables|/Script/VRM4URender.VrmExtensionRimFilterData|SetRimEdgeFade (stale Custom|init _output_get) (Variables|Default|GetRim%20Edge%20Fade))
      (Variables|/Script/VRM4URender.VrmExtensionRimFilterData|SetbUseBinaryEdge (stale Custom|init _output_get) (Variables|Default|GetUse%20Binary%20Edge))
      (Variables|/Script/VRM4URender.VrmExtensionRimFilterData|SetRimEdgeBinaryRange (stale Custom|init _output_get) (Variables|Default|GetRim%20Edge%20Binary%20Range)))
    (:then_5
      (Variables|/Script/VRM4URender.VrmExtensionRimFilterData|SetLightDirection (stale Custom|init _output_get) (* (Math|Vector|GetForwardVector _returnvalue_8) (Math|Float|MakeLiteralFloat -1.0)))
      (Variables|/Script/VRM4URender.VrmExtensionRimFilterData|SetSampleScreenScale (stale Custom|init _output_get) (Variables|Default|GetEdgeSearchWidth)))
    (:then_6
      (Utilities|FlowControl|Sequence
        (:then_0
          (Transformation|SetWorldRotation (Variables|Default|GetScene) _returnvalue_8 false false))))))

(fn ConstructionScript
  (CallFunction|Init))