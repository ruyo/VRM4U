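; Actor that drives a VRM/VRoid character's face from a Live Link face-capture subject, targeting either a model actor or a skeletal mesh actor.
; ARKit mode hands the subject to the VRoid post-process AnimBP, or sets curves directly as morphs when none exists.
; Otherwise Tick converts ARKit blink, gaze, mouth and brow values into VRM groups or named morphs, smoothed against previous values.
; Gaze also moves the look-at target, with optional head rotation.
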(event Custom|init
  (Utilities|FlowControl|Sequence
    (:then_0
      (bind _targetactorbymodelactor (Variables|Default|GetTargetActorByModelActor)
        (:then
          (Default|SetActor (Variables|Default|GetBP_VrmUtilComponent) _targetactorbymodelactor)
          (Variables|Default|SetSkeletalMeshComponent (Variables|/VRM4U/Util/BaseCharacter/BP_VrmModelActor.BP_VrmModelActor_C|GetSkeletalMeshComponent_Dst _targetactorbymodelactor))
          (Variables|Default|SetTargetActorBySkeletalMesh 0))
        (:else
          (bind _targetactorbyskeletalmesh (Variables|Default|GetTargetActorBySkeletalMesh)
            (:then
              (Variables|Default|SetSkeletalMeshComponent (Variables|/Script/Engine.SkeletalMeshActor|GetSkeletalMeshComponent _targetactorbyskeletalmesh)))
            (:else)))))
    (:then_1
      ;[1 1 1] ARkitMode
      (if (Variables|Default|GetbUseArkitMorphCurveName)
        (bind _skeletalmeshcomponent (Variables|Default|GetSkeletalMeshComponent)
          (:then
            (bind _asabp_vroid_post_process (Utilities|Casting|CastToABP_VRoidPostProcess (Components|SkeletalMesh|GetAnimInstance _skeletalmeshcomponent)))
            (Variables|/VRM4U/Util/Actor/latest/ABP_VRoidPostProcess.ABP_VRoidPostProcess_C|SetLive%20Link%20Subject _asabp_vroid_post_process (Variables|Default|GetLiveLinkSubject))
            (Components|SkeletalMesh|SetUpdateAnimationinEditor (Variables|/Script/Engine.SkeletalMeshActor|GetSkeletalMeshComponent (Variables|Default|GetTargetActorBySkeletalMesh)) true))
          (:else))))))

(event Custom|SetMorphByName
  (params (BlendShapeGroupName :type String) (Value :type Float%20%28single-precision%29) (bFindSubStr :type Boolean) (bLastStrOnly :type Boolean))
  (bind _newmorph (Variables|Default|GetnewMorph))
  ;[1 1 1] VRM Mode
  ;;[1 1 1] morph
  ;;;[1 1 1] Original MorphTarget
  (if bFindSubStr
    (bind _array_element (Utilities|Array|ForEachLoopwithBreak (Class|VrmBPFunctionLibrary|VRMGetMorphTargetList (Variables|/Script/Engine.SkinnedMeshComponent|GetSkeletalMesh (Variables|Default|GetSkeletalMeshComponent))) :!label _label)
      (:LoopBody
        (if bLastStrOnly
          (if (== (- (Utilities|String|Len _array_element) (Utilities|String|Len BlendShapeGroupName)) (Utilities|String|FindSubstring _array_element BlendShapeGroupName false true)) ; found sub str last
            (Utilities|FlowControl|Sequence :!label _label_2
              (:then_0
                (Utilities|Map|Add _newmorph _array_element Value))
              (:then_1
                (goto _label Break))))
          (elif (>= (Utilities|String|FindSubstring _array_element BlendShapeGroupName false true) 0) ; found sub str
            (goto _label_2)))))
    (else
      (Utilities|Map|Add _newmorph BlendShapeGroupName Value))))

(event Custom|SetMorphByGroup
  (params (BlendShapeGroupName :type String) (Value :type Float%20%28single-precision%29))
  ;[1 1 1] VRM Mode
  ;;[1 1 1] morph
  ;;;[1 1 1] VRM MorphGroup
  (bind _vrmassetlist (Variables|/VRM4U/Util/Actor/Misc/sub/BP_VrmUtilComponent.BP_VrmUtilComponent_C|GetVrmAssetList (Variables|Default|GetBP_VrmUtilComponent))
    (:then
      (bind _array_element (Utilities|Array|ForEachLoopwithBreak (Variables|/Script/VRM4U.VrmMetaObject|GetBlendShapeGroup (Variables|/Script/VRM4U.VrmAssetListObject|GetVrmMetaObject _vrmassetlist)) :!label _label)
        (:LoopBody
          (if (Utilities|Enum|Equal(Enum) (.name (Utilities|Struct|BreakVrmBlendShapeGroup _array_element)) BlendShapeGroupName)
            (Utilities|FlowControl|Sequence
              (:then_0
                (for _array_element_2 (.BlendShape (Utilities|Struct|BreakVrmBlendShapeGroup _array_element))
                  (Utilities|Map|Add (Variables|Default|GetnewMorph) (.morphTargetName (Utilities|Struct|BreakVrmBlendShape _array_element_2)) Value)))
              (:then_2
                (goto _label Break)))))))
    (:else)))

(event EventBeginPlay
  (CallFunction|Init)
  (bind _targetactorbymodelactor (Variables|Default|GetTargetActorByModelActor)
    (:then
      (Default|SetBlinkEnable _targetactorbymodelactor false))
    (:else)))

(event EventTick
  (params (DeltaSeconds :type Float%20%28single-precision%29))
  (bind _returnvalue (Math|Float|MakeLiteralFloat 0.2))
  (bind _returnvalue_2 (Math|Trig|GetPI))
  (bind _returnvalue_3 (Math|Float|MakeLiteralFloat 0.0))
  (bind _returnvalue_4 (Math|Float|MakeLiteralFloat 1.5))
  (bind _eyedirection (Variables|Default|GeteyeDirection))
  (bind _skeletalmeshcomponent (Variables|Default|GetSkeletalMeshComponent))
  (bind _livelinksubject (Variables|Default|GetLiveLinkSubject))
  (bind _newmorph (Variables|Default|GetnewMorph))
  (bind _morphname_mouth (Variables|Default|GetMorphName_Mouth))
  (bind _morphname_eye (Variables|Default|GetMorphName_Eye))
  (bind _returnvalue_5 (/ 1.8e+02 _returnvalue_2))
  (bind _output (Utilities|Array|Get(acopy) _eyedirection 1))
  (bind _output_2 (Utilities|Array|Get(acopy) _eyedirection))
  (bind _returnvalue_6 (+ _output_2 _output))
  (bind (_x _y) (Math|Vector2D|BreakVector2D _returnvalue_6))
  (bind _returnvalue_7 (* _returnvalue_6 -1.0))
  (bind (_x_2 _y_2) (Math|Vector2D|BreakVector2D _returnvalue_6))
  (bind (_x_3 _y_3) (Math|Vector2D|BreakVector2D _returnvalue_7))
  (if (Utilities|Name|NotEqual(Name) (Utilities|Struct|BreakLiveLinkSubjectName _livelinksubject) "None")
    (bind _dataresult (|EvaluateLiveLinkFramewithSpecificRole _livelinksubject "/Script/LiveLinkInterface.LiveLinkBasicRole")
      (:then
        (if (Variables|Default|GetbUseArkitMorphCurveName)
          ;[1 1 1] ARKitMode
          (Utilities|FlowControl|Sequence
            (:then_0
              (for (_array_element _array_index) (Utilities|Struct|BreakLiveLinkBaseStaticData (.StaticData (Utilities|Struct|BreakLiveLinkBasicBlueprintData _dataresult)))
                (Utilities|IsValid (Class|SkeletalMeshComponent|GetPostProcessInstance _skeletalmeshcomponent)
                  (:Is%20Not%20Valid
                    (Components|SkeletalMesh|SetMorphTarget _skeletalmeshcomponent _array_element (Utilities|Array|Get(acopy) (.PropertyValues (Utilities|Struct|BreakLiveLinkBaseFrameData (.FrameData (Utilities|Struct|BreakLiveLinkBasicBlueprintData _dataresult)))) _array_index) false))))))
          (else
            ;[1 1 1] VRM Mode
            (Utilities|FlowControl|Sequence
              (:then_0
                (Utilities|Map|Clear (Variables|Default|GetnewMorph))
                (Variables|Default|SeteyeWeight (Utilities|Array|MakeArray 0.0 0.0)))
              (:then_2
                (Utilities|FlowControl|Sequence
                  (:then_1
                    ;;[1 1 1] blink
                    (if (Variables|Default|GetbUseCustomEye)
                      (Utilities|FlowControl|Sequence :!label _label
                        (:then_0
                          (CallFunction|SetMorphbyName (Utilities|Array|Get(acopy) _morphname_eye) (Math|Float|SelectFloat (Math|Float|Max(Float) (Math|Float|Lerp 0.0 (- (Math|Float|Clamp(Float) (* (/ (- (.Value (Class|LiveLinkBlueprintLibrary|GetPropertyValue _dataresult "EyeBlinkRight")) _returnvalue_3) (- 1.0 _returnvalue_3)) _returnvalue_4)) 0.0) (Math|Float|Clamp(Float) (* (/ (- (.Value (Class|LiveLinkBlueprintLibrary|GetPropertyValue _dataresult "EyeBlinkRight")) _returnvalue_3) (- 1.0 _returnvalue_3)) _returnvalue_4))) (Math|Float|Lerp 0.0 (- (Math|Float|Clamp(Float) (* (/ (.Value (Class|LiveLinkBlueprintLibrary|GetPropertyValue _dataresult "EyeBlinkLeft")) (- 1.0 (.Value (Class|LiveLinkBlueprintLibrary|GetPropertyValue _dataresult "EyeBlinkLeft")))) _returnvalue_4)) 0.0) (Math|Float|Clamp(Float) (* (/ (.Value (Class|LiveLinkBlueprintLibrary|GetPropertyValue _dataresult "EyeBlinkLeft")) (- 1.0 (.Value (Class|LiveLinkBlueprintLibrary|GetPropertyValue _dataresult "EyeBlinkLeft")))) _returnvalue_4)))) (Math|Float|Lerp 0.0 (- (Math|Float|Clamp(Float) (* (/ (- (.Value (Class|LiveLinkBlueprintLibrary|GetPropertyValue _dataresult "EyeBlinkRight")) _returnvalue_3) (- 1.0 _returnvalue_3)) _returnvalue_4)) 0.0) (Math|Float|Clamp(Float) (* (/ (- (.Value (Class|LiveLinkBlueprintLibrary|GetPropertyValue _dataresult "EyeBlinkRight")) _returnvalue_3) (- 1.0 _returnvalue_3)) _returnvalue_4))) (< (Math|Float|Absolute(Float) (- (Math|Float|Lerp 0.0 (- (Math|Float|Clamp(Float) (* (/ (- (.Value (Class|LiveLinkBlueprintLibrary|GetPropertyValue _dataresult "EyeBlinkRight")) _returnvalue_3) (- 1.0 _returnvalue_3)) _returnvalue_4)) 0.0) (Math|Float|Clamp(Float) (* (/ (- (.Value (Class|LiveLinkBlueprintLibrary|GetPropertyValue _dataresult "EyeBlinkRight")) _returnvalue_3) (- 1.0 _returnvalue_3)) _returnvalue_4))) (Math|Float|Lerp 0.0 (- (Math|Float|Clamp(Float) (* (/ (.Value (Class|LiveLinkBlueprintLibrary|GetPropertyValue _dataresult "EyeBlinkLeft")) (- 1.0 (.Value (Class|LiveLinkBlueprintLibrary|GetPropertyValue _dataresult "EyeBlinkLeft")))) _returnvalue_4)) 0.0) (Math|Float|Clamp(Float) (* (/ (.Value (Class|LiveLinkBlueprintLibrary|GetPropertyValue _dataresult "EyeBlinkLeft")) (- 1.0 (.Value (Class|LiveLinkBlueprintLibrary|GetPropertyValue _dataresult "EyeBlinkLeft")))) _returnvalue_4))))) 0.2)) false false)
                          ;;[1 1 1] 他との干渉用にBlinkの値を保存
                          (Utilities|Array|SetArrayElem (Variables|Default|GeteyeWeight) 1 (Math|Float|SelectFloat (Math|Float|Max(Float) (Math|Float|Lerp 0.0 (- (Math|Float|Clamp(Float) (* (/ (- (.Value (Class|LiveLinkBlueprintLibrary|GetPropertyValue _dataresult "EyeBlinkRight")) _returnvalue_3) (- 1.0 _returnvalue_3)) _returnvalue_4)) 0.0) (Math|Float|Clamp(Float) (* (/ (- (.Value (Class|LiveLinkBlueprintLibrary|GetPropertyValue _dataresult "EyeBlinkRight")) _returnvalue_3) (- 1.0 _returnvalue_3)) _returnvalue_4))) (Math|Float|Lerp 0.0 (- (Math|Float|Clamp(Float) (* (/ (.Value (Class|LiveLinkBlueprintLibrary|GetPropertyValue _dataresult "EyeBlinkLeft")) (- 1.0 (.Value (Class|LiveLinkBlueprintLibrary|GetPropertyValue _dataresult "EyeBlinkLeft")))) _returnvalue_4)) 0.0) (Math|Float|Clamp(Float) (* (/ (.Value (Class|LiveLinkBlueprintLibrary|GetPropertyValue _dataresult "EyeBlinkLeft")) (- 1.0 (.Value (Class|LiveLinkBlueprintLibrary|GetPropertyValue _dataresult "EyeBlinkLeft")))) _returnvalue_4)))) (Math|Float|Lerp 0.0 (- (Math|Float|Clamp(Float) (* (/ (- (.Value (Class|LiveLinkBlueprintLibrary|GetPropertyValue _dataresult "EyeBlinkRight")) _returnvalue_3) (- 1.0 _returnvalue_3)) _returnvalue_4)) 0.0) (Math|Float|Clamp(Float) (* (/ (- (.Value (Class|LiveLinkBlueprintLibrary|GetPropertyValue _dataresult "EyeBlinkRight")) _returnvalue_3) (- 1.0 _returnvalue_3)) _returnvalue_4))) (< (Math|Float|Absolute(Float) (- (Math|Float|Lerp 0.0 (- (Math|Float|Clamp(Float) (* (/ (- (.Value (Class|LiveLinkBlueprintLibrary|GetPropertyValue _dataresult "EyeBlinkRight")) _returnvalue_3) (- 1.0 _returnvalue_3)) _returnvalue_4)) 0.0) (Math|Float|Clamp(Float) (* (/ (- (.Value (Class|LiveLinkBlueprintLibrary|GetPropertyValue _dataresult "EyeBlinkRight")) _returnvalue_3) (- 1.0 _returnvalue_3)) _returnvalue_4))) (Math|Float|Lerp 0.0 (- (Math|Float|Clamp(Float) (* (/ (.Value (Class|LiveLinkBlueprintLibrary|GetPropertyValue _dataresult "EyeBlinkLeft")) (- 1.0 (.Value (Class|LiveLinkBlueprintLibrary|GetPropertyValue _dataresult "EyeBlinkLeft")))) _returnvalue_4)) 0.0) (Math|Float|Clamp(Float) (* (/ (.Value (Class|LiveLinkBlueprintLibrary|GetPropertyValue _dataresult "EyeBlinkLeft")) (- 1.0 (.Value (Class|LiveLinkBlueprintLibrary|GetPropertyValue _dataresult "EyeBlinkLeft")))) _returnvalue_4))))) 0.2)) :!label _label_2))
                        (:then_1
                          (CallFunction|SetMorphbyName (Utilities|Array|Get(acopy) _morphname_eye 1) (Math|Float|SelectFloat (Math|Float|Max(Float) (Math|Float|Lerp 0.0 (- (Math|Float|Clamp(Float) (* (/ (- (.Value (Class|LiveLinkBlueprintLibrary|GetPropertyValue _dataresult "EyeBlinkRight")) _returnvalue_3) (- 1.0 _returnvalue_3)) _returnvalue_4)) 0.0) (Math|Float|Clamp(Float) (* (/ (- (.Value (Class|LiveLinkBlueprintLibrary|GetPropertyValue _dataresult "EyeBlinkRight")) _returnvalue_3) (- 1.0 _returnvalue_3)) _returnvalue_4))) (Math|Float|Lerp 0.0 (- (Math|Float|Clamp(Float) (* (/ (.Value (Class|LiveLinkBlueprintLibrary|GetPropertyValue _dataresult "EyeBlinkLeft")) (- 1.0 (.Value (Class|LiveLinkBlueprintLibrary|GetPropertyValue _dataresult "EyeBlinkLeft")))) _returnvalue_4)) 0.0) (Math|Float|Clamp(Float) (* (/ (.Value (Class|LiveLinkBlueprintLibrary|GetPropertyValue _dataresult "EyeBlinkLeft")) (- 1.0 (.Value (Class|LiveLinkBlueprintLibrary|GetPropertyValue _dataresult "EyeBlinkLeft")))) _returnvalue_4)))) (Math|Float|Lerp 0.0 (- (Math|Float|Clamp(Float) (* (/ (.Value (Class|LiveLinkBlueprintLibrary|GetPropertyValue _dataresult "EyeBlinkLeft")) (- 1.0 (.Value (Class|LiveLinkBlueprintLibrary|GetPropertyValue _dataresult "EyeBlinkLeft")))) _returnvalue_4)) 0.0) (Math|Float|Clamp(Float) (* (/ (.Value (Class|LiveLinkBlueprintLibrary|GetPropertyValue _dataresult "EyeBlinkLeft")) (- 1.0 (.Value (Class|LiveLinkBlueprintLibrary|GetPropertyValue _dataresult "EyeBlinkLeft")))) _returnvalue_4))) (< (Math|Float|Absolute(Float) (- (Math|Float|Lerp 0.0 (- (Math|Float|Clamp(Float) (* (/ (- (.Value (Class|LiveLinkBlueprintLibrary|GetPropertyValue _dataresult "EyeBlinkRight")) _returnvalue_3) (- 1.0 _returnvalue_3)) _returnvalue_4)) 0.0) (Math|Float|Clamp(Float) (* (/ (- (.Value (Class|LiveLinkBlueprintLibrary|GetPropertyValue _dataresult "EyeBlinkRight")) _returnvalue_3) (- 1.0 _returnvalue_3)) _returnvalue_4))) (Math|Float|Lerp 0.0 (- (Math|Float|Clamp(Float) (* (/ (.Value (Class|LiveLinkBlueprintLibrary|GetPropertyValue _dataresult "EyeBlinkLeft")) (- 1.0 (.Value (Class|LiveLinkBlueprintLibrary|GetPropertyValue _dataresult "EyeBlinkLeft")))) _returnvalue_4)) 0.0) (Math|Float|Clamp(Float) (* (/ (.Value (Class|LiveLinkBlueprintLibrary|GetPropertyValue _dataresult "EyeBlinkLeft")) (- 1.0 (.Value (Class|LiveLinkBlueprintLibrary|GetPropertyValue _dataresult "EyeBlinkLeft")))) _returnvalue_4))))) 0.2)) false false)
                          (Utilities|Array|SetArrayElem (Variables|Default|GeteyeWeight) 0 (Math|Float|SelectFloat (Math|Float|Max(Float) (Math|Float|Lerp 0.0 (- (Math|Float|Clamp(Float) (* (/ (- (.Value (Class|LiveLinkBlueprintLibrary|GetPropertyValue _dataresult "EyeBlinkRight")) _returnvalue_3) (- 1.0 _returnvalue_3)) _returnvalue_4)) 0.0) (Math|Float|Clamp(Float) (* (/ (- (.Value (Class|LiveLinkBlueprintLibrary|GetPropertyValue _dataresult "EyeBlinkRight")) _returnvalue_3) (- 1.0 _returnvalue_3)) _returnvalue_4))) (Math|Float|Lerp 0.0 (- (Math|Float|Clamp(Float) (* (/ (.Value (Class|LiveLinkBlueprintLibrary|GetPropertyValue _dataresult "EyeBlinkLeft")) (- 1.0 (.Value (Class|LiveLinkBlueprintLibrary|GetPropertyValue _dataresult "EyeBlinkLeft")))) _returnvalue_4)) 0.0) (Math|Float|Clamp(Float) (* (/ (.Value (Class|LiveLinkBlueprintLibrary|GetPropertyValue _dataresult "EyeBlinkLeft")) (- 1.0 (.Value (Class|LiveLinkBlueprintLibrary|GetPropertyValue _dataresult "EyeBlinkLeft")))) _returnvalue_4)))) (Math|Float|Lerp 0.0 (- (Math|Float|Clamp(Float) (* (/ (.Value (Class|LiveLinkBlueprintLibrary|GetPropertyValue _dataresult "EyeBlinkLeft")) (- 1.0 (.Value (Class|LiveLinkBlueprintLibrary|GetPropertyValue _dataresult "EyeBlinkLeft")))) _returnvalue_4)) 0.0) (Math|Float|Clamp(Float) (* (/ (.Value (Class|LiveLinkBlueprintLibrary|GetPropertyValue _dataresult "EyeBlinkLeft")) (- 1.0 (.Value (Class|LiveLinkBlueprintLibrary|GetPropertyValue _dataresult "EyeBlinkLeft")))) _returnvalue_4))) (< (Math|Float|Absolute(Float) (- (Math|Float|Lerp 0.0 (- (Math|Float|Clamp(Float) (* (/ (- (.Value (Class|LiveLinkBlueprintLibrary|GetPropertyValue _dataresult "EyeBlinkRight")) _returnvalue_3) (- 1.0 _returnvalue_3)) _returnvalue_4)) 0.0) (Math|Float|Clamp(Float) (* (/ (- (.Value (Class|LiveLinkBlueprintLibrary|GetPropertyValue _dataresult "EyeBlinkRight")) _returnvalue_3) (- 1.0 _returnvalue_3)) _returnvalue_4))) (Math|Float|Lerp 0.0 (- (Math|Float|Clamp(Float) (* (/ (.Value (Class|LiveLinkBlueprintLibrary|GetPropertyValue _dataresult "EyeBlinkLeft")) (- 1.0 (.Value (Class|LiveLinkBlueprintLibrary|GetPropertyValue _dataresult "EyeBlinkLeft")))) _returnvalue_4)) 0.0) (Math|Float|Clamp(Float) (* (/ (.Value (Class|LiveLinkBlueprintLibrary|GetPropertyValue _dataresult "EyeBlinkLeft")) (- 1.0 (.Value (Class|LiveLinkBlueprintLibrary|GetPropertyValue _dataresult "EyeBlinkLeft")))) _returnvalue_4))))) 0.2)) :!label _label_3)))
                      (else
                        (Utilities|IsValid (Variables|Default|GetTargetActorByModelActor)
                          (:Is%20Valid
                            (Utilities|FlowControl|Sequence
                              (:then_0
                                (CallFunction|SetMorphbyGroup "Blink_R" (Math|Float|SelectFloat (Math|Float|Max(Float) (Math|Float|Lerp 0.0 (- (Math|Float|Clamp(Float) (* (/ (- (.Value (Class|LiveLinkBlueprintLibrary|GetPropertyValue _dataresult "EyeBlinkRight")) _returnvalue_3) (- 1.0 _returnvalue_3)) _returnvalue_4)) 0.0) (Math|Float|Clamp(Float) (* (/ (- (.Value (Class|LiveLinkBlueprintLibrary|GetPropertyValue _dataresult "EyeBlinkRight")) _returnvalue_3) (- 1.0 _returnvalue_3)) _returnvalue_4))) (Math|Float|Lerp 0.0 (- (Math|Float|Clamp(Float) (* (/ (.Value (Class|LiveLinkBlueprintLibrary|GetPropertyValue _dataresult "EyeBlinkLeft")) (- 1.0 (.Value (Class|LiveLinkBlueprintLibrary|GetPropertyValue _dataresult "EyeBlinkLeft")))) _returnvalue_4)) 0.0) (Math|Float|Clamp(Float) (* (/ (.Value (Class|LiveLinkBlueprintLibrary|GetPropertyValue _dataresult "EyeBlinkLeft")) (- 1.0 (.Value (Class|LiveLinkBlueprintLibrary|GetPropertyValue _dataresult "EyeBlinkLeft")))) _returnvalue_4)))) (Math|Float|Lerp 0.0 (- (Math|Float|Clamp(Float) (* (/ (- (.Value (Class|LiveLinkBlueprintLibrary|GetPropertyValue _dataresult "EyeBlinkRight")) _returnvalue_3) (- 1.0 _returnvalue_3)) _returnvalue_4)) 0.0) (Math|Float|Clamp(Float) (* (/ (- (.Value (Class|LiveLinkBlueprintLibrary|GetPropertyValue _dataresult "EyeBlinkRight")) _returnvalue_3) (- 1.0 _returnvalue_3)) _returnvalue_4))) (< (Math|Float|Absolute(Float) (- (Math|Float|Lerp 0.0 (- (Math|Float|Clamp(Float) (* (/ (- (.Value (Class|LiveLinkBlueprintLibrary|GetPropertyValue _dataresult "EyeBlinkRight")) _returnvalue_3) (- 1.0 _returnvalue_3)) _returnvalue_4)) 0.0) (Math|Float|Clamp(Float) (* (/ (- (.Value (Class|LiveLinkBlueprintLibrary|GetPropertyValue _dataresult "EyeBlinkRight")) _returnvalue_3) (- 1.0 _returnvalue_3)) _returnvalue_4))) (Math|Float|Lerp 0.0 (- (Math|Float|Clamp(Float) (* (/ (.Value (Class|LiveLinkBlueprintLibrary|GetPropertyValue _dataresult "EyeBlinkLeft")) (- 1.0 (.Value (Class|LiveLinkBlueprintLibrary|GetPropertyValue _dataresult "EyeBlinkLeft")))) _returnvalue_4)) 0.0) (Math|Float|Clamp(Float) (* (/ (.Value (Class|LiveLinkBlueprintLibrary|GetPropertyValue _dataresult "EyeBlinkLeft")) (- 1.0 (.Value (Class|LiveLinkBlueprintLibrary|GetPropertyValue _dataresult "EyeBlinkLeft")))) _returnvalue_4))))) 0.2)))
                                (goto _label_2))
                              (:then_1
                                (CallFunction|SetMorphbyGroup "Blink_L" (Math|Float|SelectFloat (Math|Float|Max(Float) (Math|Float|Lerp 0.0 (- (Math|Float|Clamp(Float) (* (/ (- (.Value (Class|LiveLinkBlueprintLibrary|GetPropertyValue _dataresult "EyeBlinkRight")) _returnvalue_3) (- 1.0 _returnvalue_3)) _returnvalue_4)) 0.0) (Math|Float|Clamp(Float) (* (/ (- (.Value (Class|LiveLinkBlueprintLibrary|GetPropertyValue _dataresult "EyeBlinkRight")) _returnvalue_3) (- 1.0 _returnvalue_3)) _returnvalue_4))) (Math|Float|Lerp 0.0 (- (Math|Float|Clamp(Float) (* (/ (.Value (Class|LiveLinkBlueprintLibrary|GetPropertyValue _dataresult "EyeBlinkLeft")) (- 1.0 (.Value (Class|LiveLinkBlueprintLibrary|GetPropertyValue _dataresult "EyeBlinkLeft")))) _returnvalue_4)) 0.0) (Math|Float|Clamp(Float) (* (/ (.Value (Class|LiveLinkBlueprintLibrary|GetPropertyValue _dataresult "EyeBlinkLeft")) (- 1.0 (.Value (Class|LiveLinkBlueprintLibrary|GetPropertyValue _dataresult "EyeBlinkLeft")))) _returnvalue_4)))) (Math|Float|Lerp 0.0 (- (Math|Float|Clamp(Float) (* (/ (.Value (Class|LiveLinkBlueprintLibrary|GetPropertyValue _dataresult "EyeBlinkLeft")) (- 1.0 (.Value (Class|LiveLinkBlueprintLibrary|GetPropertyValue _dataresult "EyeBlinkLeft")))) _returnvalue_4)) 0.0) (Math|Float|Clamp(Float) (* (/ (.Value (Class|LiveLinkBlueprintLibrary|GetPropertyValue _dataresult "EyeBlinkLeft")) (- 1.0 (.Value (Class|LiveLinkBlueprintLibrary|GetPropertyValue _dataresult "EyeBlinkLeft")))) _returnvalue_4))) (< (Math|Float|Absolute(Float) (- (Math|Float|Lerp 0.0 (- (Math|Float|Clamp(Float) (* (/ (- (.Value (Class|LiveLinkBlueprintLibrary|GetPropertyValue _dataresult "EyeBlinkRight")) _returnvalue_3) (- 1.0 _returnvalue_3)) _returnvalue_4)) 0.0) (Math|Float|Clamp(Float) (* (/ (- (.Value (Class|LiveLinkBlueprintLibrary|GetPropertyValue _dataresult "EyeBlinkRight")) _returnvalue_3) (- 1.0 _returnvalue_3)) _returnvalue_4))) (Math|Float|Lerp 0.0 (- (Math|Float|Clamp(Float) (* (/ (.Value (Class|LiveLinkBlueprintLibrary|GetPropertyValue _dataresult "EyeBlinkLeft")) (- 1.0 (.Value (Class|LiveLinkBlueprintLibrary|GetPropertyValue _dataresult "EyeBlinkLeft")))) _returnvalue_4)) 0.0) (Math|Float|Clamp(Float) (* (/ (.Value (Class|LiveLinkBlueprintLibrary|GetPropertyValue _dataresult "EyeBlinkLeft")) (- 1.0 (.Value (Class|LiveLinkBlueprintLibrary|GetPropertyValue _dataresult "EyeBlinkLeft")))) _returnvalue_4))))) 0.2)))
                                (goto _label_3))))
                          (:Is%20Not%20Valid
                            (goto _label))))))
                  (:then_2
                    ;;[1 1 1] eye direction
                    (Utilities|FlowControl|Sequence
                      (:then_0
                        ;;;[1 1 1] eye direction
                        (Utilities|Array|SetArrayElem (Variables|Default|GeteyeDirection) 0 (Math|Vector2D|MakeVector2D (- (.Value (Class|LiveLinkBlueprintLibrary|GetPropertyValue _dataresult "EyeLookOutLeft")) (.Value (Class|LiveLinkBlueprintLibrary|GetPropertyValue _dataresult "EyeLookInLeft"))) (- (.Value (Class|LiveLinkBlueprintLibrary|GetPropertyValue _dataresult "EyeLookUpLeft")) (.Value (Class|LiveLinkBlueprintLibrary|GetPropertyValue _dataresult "EyeLookDownLeft"))))))
                      (:then_1
                        (Utilities|Array|SetArrayElem (Variables|Default|GeteyeDirection) 1 (Math|Vector2D|MakeVector2D (- (.Value (Class|LiveLinkBlueprintLibrary|GetPropertyValue _dataresult "EyeLookInRight")) (.Value (Class|LiveLinkBlueprintLibrary|GetPropertyValue _dataresult "EyeLookOutRight"))) (- (.Value (Class|LiveLinkBlueprintLibrary|GetPropertyValue _dataresult "EyeLookUpRight")) (.Value (Class|LiveLinkBlueprintLibrary|GetPropertyValue _dataresult "EyeLookDownRight"))))))
                      (:then_2
                        ;;;[1 1 1] MorphTarget
                        (CallFunction|SetMorphbyGroup "LOOKUP" (Math|Float|Max(Float) _y_2 0.0))
                        (CallFunction|SetMorphbyGroup "LOOKDOWN" (Math|Float|Max(Float) _y_3 0.0))
                        (CallFunction|SetMorphbyGroup "LOOKLEFT" (Math|Float|Max(Float) _x_2 0.0))
                        (CallFunction|SetMorphbyGroup "LOOKRIGHT" (Math|Float|Max(Float) _x_3 0.0)))
                      (:then_3
                        (Utilities|FlowControl|Sequence
                          (:then_0
                            (bind _targetactorbymodelactor (Variables|Default|GetTargetActorByModelActor)
                              (:then
                                (Default|SetLookatTarget _targetactorbymodelactor (Math|Transform|TransformLocation (.transform (Default|GetVrmBoneTransform (Variables|Default|GetBP_VrmUtilComponent) "head" "RTS_World")) (Math|Vector|MakeVector (* (/ (* (- _x _returnvalue) _returnvalue) (- 1.0 _returnvalue)) -1e+03) 5e+02 (* (/ (* (- _y _returnvalue) _returnvalue) (- 1.0 _returnvalue)) 1e+03))))
                                (Default|SetLookatType _targetactorbymodelactor true false))
                              (:else)))))))
                  (:then_3
                    (if (Variables|Default|GetbUseCustomMorph)
                      (Utilities|FlowControl|Sequence :!label _label_4
                        (:then_0
                          (CallFunction|SetMorphbyName (Utilities|Array|Get(acopy) _morphname_mouth) (Math|Float|Min(Float) (Math|Float|Clamp(Float) (* (.Value (Class|LiveLinkBlueprintLibrary|GetPropertyValue _dataresult "JawOpen")) 1.5)) (/ (Math|Float|Clamp(Float) (* (.Value (Class|LiveLinkBlueprintLibrary|GetPropertyValue _dataresult "JawOpen")) 1.5)) (+ (Math|Float|Clamp(Float) (* (.Value (Class|LiveLinkBlueprintLibrary|GetPropertyValue _dataresult "JawOpen")) 1.5)) (Math|Float|Clamp(Float) (* (Math|Float|Max(Float) (.Value (Class|LiveLinkBlueprintLibrary|GetPropertyValue _dataresult "MouthSmileLeft")) (.Value (Class|LiveLinkBlueprintLibrary|GetPropertyValue _dataresult "MouthSmileRight"))) 1.5)) (Math|Float|Clamp(Float) (* (+ (.Value (Class|LiveLinkBlueprintLibrary|GetPropertyValue _dataresult "MouthPucker")) (.Value (Class|LiveLinkBlueprintLibrary|GetPropertyValue _dataresult "MouthFunnel"))) 1.5))))) true true))
                        (:then_1
                          (CallFunction|SetMorphbyName (Utilities|Array|Get(acopy) _morphname_mouth 1) (Math|Float|Min(Float) (Math|Float|Clamp(Float) (* (Math|Float|Max(Float) (.Value (Class|LiveLinkBlueprintLibrary|GetPropertyValue _dataresult "MouthSmileLeft")) (.Value (Class|LiveLinkBlueprintLibrary|GetPropertyValue _dataresult "MouthSmileRight"))) 1.5)) (/ (Math|Float|Clamp(Float) (* (Math|Float|Max(Float) (.Value (Class|LiveLinkBlueprintLibrary|GetPropertyValue _dataresult "MouthSmileLeft")) (.Value (Class|LiveLinkBlueprintLibrary|GetPropertyValue _dataresult "MouthSmileRight"))) 1.5)) (+ (Math|Float|Clamp(Float) (* (.Value (Class|LiveLinkBlueprintLibrary|GetPropertyValue _dataresult "JawOpen")) 1.5)) (Math|Float|Clamp(Float) (* (Math|Float|Max(Float) (.Value (Class|LiveLinkBlueprintLibrary|GetPropertyValue _dataresult "MouthSmileLeft")) (.Value (Class|LiveLinkBlueprintLibrary|GetPropertyValue _dataresult "MouthSmileRight"))) 1.5)) (Math|Float|Clamp(Float) (* (+ (.Value (Class|LiveLinkBlueprintLibrary|GetPropertyValue _dataresult "MouthPucker")) (.Value (Class|LiveLinkBlueprintLibrary|GetPropertyValue _dataresult "MouthFunnel"))) 1.5))))) true true))
                        (:then_2
                          (CallFunction|SetMorphbyName (Utilities|Array|Get(acopy) _morphname_mouth 2) (Math|Float|Min(Float) (Math|Float|Clamp(Float) (* (+ (.Value (Class|LiveLinkBlueprintLibrary|GetPropertyValue _dataresult "MouthPucker")) (.Value (Class|LiveLinkBlueprintLibrary|GetPropertyValue _dataresult "MouthFunnel"))) 1.5)) (/ (Math|Float|Clamp(Float) (* (+ (.Value (Class|LiveLinkBlueprintLibrary|GetPropertyValue _dataresult "MouthPucker")) (.Value (Class|LiveLinkBlueprintLibrary|GetPropertyValue _dataresult "MouthFunnel"))) 1.5)) (+ (Math|Float|Clamp(Float) (* (.Value (Class|LiveLinkBlueprintLibrary|GetPropertyValue _dataresult "JawOpen")) 1.5)) (Math|Float|Clamp(Float) (* (Math|Float|Max(Float) (.Value (Class|LiveLinkBlueprintLibrary|GetPropertyValue _dataresult "MouthSmileLeft")) (.Value (Class|LiveLinkBlueprintLibrary|GetPropertyValue _dataresult "MouthSmileRight"))) 1.5)) (Math|Float|Clamp(Float) (* (+ (.Value (Class|LiveLinkBlueprintLibrary|GetPropertyValue _dataresult "MouthPucker")) (.Value (Class|LiveLinkBlueprintLibrary|GetPropertyValue _dataresult "MouthFunnel"))) 1.5))))) true true)))
                      (else
                        (Utilities|IsValid (Variables|Default|GetTargetActorByModelActor)
                          (:Is%20Valid
                            ;;[1 1 1] Mouth
                            (Utilities|FlowControl|Sequence
                              (:then_0
                                (CallFunction|SetMorphbyGroup "A" (Math|Float|Clamp(Float) (* (.Value (Class|LiveLinkBlueprintLibrary|GetPropertyValue _dataresult "JawOpen")) 1.5))))
                              (:then_1
                                (CallFunction|SetMorphbyGroup "I" (Math|Float|Clamp(Float) (* (Math|Float|Max(Float) (.Value (Class|LiveLinkBlueprintLibrary|GetPropertyValue _dataresult "MouthSmileLeft")) (.Value (Class|LiveLinkBlueprintLibrary|GetPropertyValue _dataresult "MouthSmileRight"))) 1.5))))
                              (:then_2
                                (CallFunction|SetMorphbyGroup "U" (Math|Float|Clamp(Float) (* (+ (.Value (Class|LiveLinkBlueprintLibrary|GetPropertyValue _dataresult "MouthPucker")) (.Value (Class|LiveLinkBlueprintLibrary|GetPropertyValue _dataresult "MouthFunnel"))) 1.5))))))
                          (:Is%20Not%20Valid
                            (goto _label_4))))))
                  (:then_4
                    ;;[1 1 1] Brow And Eye
                    (Utilities|FlowControl|Sequence
                      (:then_0
                        (CallFunction|SetMorphbyName "Fcl_BRW_Sorrow" (Math|Float|Clamp(Float) (* (Math|Float|Max(Float) (.Value (Class|LiveLinkBlueprintLibrary|GetPropertyValue _dataresult "BrowDownLeft")) (.Value (Class|LiveLinkBlueprintLibrary|GetPropertyValue _dataresult "BrowDownRight"))) 1.5)) true true)
                        (CallFunction|SetMorphbyName "Fcl_EYE_Sorrow" (Math|Float|Lerp 0.0 (- 1.0 (Math|Float|Max(Float) (Utilities|Array|Get(acopy) (Variables|Default|GeteyeWeight)) (Utilities|Array|Get(acopy) (Variables|Default|GeteyeWeight) 1))) (Math|Float|Clamp(Float) (* (Math|Float|Max(Float) (.Value (Class|LiveLinkBlueprintLibrary|GetPropertyValue _dataresult "BrowDownLeft")) (.Value (Class|LiveLinkBlueprintLibrary|GetPropertyValue _dataresult "BrowDownRight"))) 2.0))) true true))
                      (:then_1
                        (CallFunction|SetMorphbyName "Fcl_BRW_Fun" (Math|Float|Clamp(Float) (* (Math|Float|Max(Float) (.Value (Class|LiveLinkBlueprintLibrary|GetPropertyValue _dataresult "BrowOuterUpLeft")) (.Value (Class|LiveLinkBlueprintLibrary|GetPropertyValue _dataresult "BrowOuterUpRight"))) 1.5)) true true)
                        (CallFunction|SetMorphbyName "Fcl_EYE_Surprised" (Math|Float|Lerp 0.0 (- 1.0 (Math|Float|Max(Float) (Utilities|Array|Get(acopy) (Variables|Default|GeteyeWeight)) (Utilities|Array|Get(acopy) (Variables|Default|GeteyeWeight) 1))) (Math|Float|Clamp(Float) (* (Math|Float|Max(Float) (.Value (Class|LiveLinkBlueprintLibrary|GetPropertyValue _dataresult "BrowOuterUpLeft")) (.Value (Class|LiveLinkBlueprintLibrary|GetPropertyValue _dataresult "BrowOuterUpRight"))) 1.5))) true true))))
                  (:then_5
                    (Utilities|FlowControl|Sequence))))
              (:then_3
                (if (!= (Utilities|Map|Length (Variables|Default|GetnewMorph)) (Utilities|Map|Length (Variables|Default|GetcurrentMorph)))
                  (Variables|Default|SetcurrentMorph (Variables|Default|GetnewMorph))))
              (:then_5
                ;;[1 1 1] apply morph
                ;; 補間
                (bind _keys (Utilities|Map|Keys _newmorph))
                (for _array_element_2 _keys
                  (Components|SkeletalMesh|SetMorphTarget (Variables|Default|GetSkeletalMeshComponent) (Utilities|String|StringToName _array_element_2) (Math|Float|Lerp (.Value (Utilities|Map|Find _newmorph _array_element_2)) (.Value (Utilities|Map|Find (Variables|Default|GetcurrentMorph) _array_element_2)) 0.5) true)
                  (Utilities|Map|Add (Variables|Default|GetcurrentMorph) _array_element_2 (Math|Float|Lerp (.Value (Utilities|Map|Find _newmorph _array_element_2)) (.Value (Utilities|Map|Find (Variables|Default|GetcurrentMorph) _array_element_2)) 0.5))))
              (:then_6
                (if (Variables|Default|GetbUseHeadRot)
                  ;;[1 1 1] head rot
                  (Utilities|FlowControl|Sequence
                    (:then_0
                      (bind _targetactorbymodelactor_2 (Variables|Default|GetTargetActorByModelActor)
                        (:then
                          (bind _asabp_vroid_simple (Utilities|Casting|CastToABP_VRoidSimple (Components|SkeletalMesh|GetAnimInstance (Variables|/VRM4U/Util/BaseCharacter/BP_VrmModelActor.BP_VrmModelActor_C|GetSkeletalMeshComponent_Src _targetactorbymodelactor_2))))
                          (Variables|/VRM4U/Util/BaseCharacter/Mesh/ABP_VRoidSimple.ABP_VRoidSimple_C|SetbHeadForce _asabp_vroid_simple true)
                          (Variables|/VRM4U/Util/BaseCharacter/Mesh/ABP_VRoidSimple.ABP_VRoidSimple_C|SetHeadForce _asabp_vroid_simple (Math|Rotator|CombineRotators (Math|Rotator|CombineRotators (Math|Rotator|MakeRotator 0.0 0.0 (* (.Value (Class|LiveLinkBlueprintLibrary|GetPropertyValue _dataresult "HeadYaw")) _returnvalue_5 -1.0)) (Math|Rotator|MakeRotator (* (.Value (Class|LiveLinkBlueprintLibrary|GetPropertyValue _dataresult "HeadPitch")) _returnvalue_5 -1.0) 0.0 0.0)) (Math|Rotator|MakeRotator 0.0 (* (.Value (Class|LiveLinkBlueprintLibrary|GetPropertyValue _dataresult "HeadRoll")) _returnvalue_5 1.0) 0.0))))
                        (:else)))))))))))))

(fn ConstructionScript
  (CallFunction|Init))