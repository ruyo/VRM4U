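; BP_BoneInfo describes one bone of a VRM skeletal mesh as a node in a bone hierarchy.
; CreateInfo stores name and mesh bone index, links to its parent with incremented depth, and flags humanoid bones found in the VRM meta object's HumanoidBoneTable values.
; UpdateExpand sets the Expand flag on a humanoid bone that has any non-humanoid child.
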(event Custom|CreateInfo
  (params (BoneName :type String) (Mesh :type Skeletal%20Mesh%20Component%20Object%20Reference) (AssetList :type Vrm%20Asset%20List%20Object%20Object%20Reference) (BoneParent :type BP%20Bone%20Info%20Object%20Reference))
  (Utilities|FlowControl|Sequence
    (:then_0
      (Variables|Default|SetBoneName BoneName)
      (Variables|Default|SetBoneIndex (Class|SkinnedMeshComponent|GetBoneIndex Mesh (Utilities|String|StringToName BoneName)))
      (Utilities|IsValid BoneParent
        (:Is%20Valid
          (Variables|Default|Setdepth (+ (Variables|BP_BoneInfo_C|Getdepth BoneParent) 1))
          (Variables|Default|SetBoneParent BoneParent)
          (Utilities|Array|AddUnique (Variables|BP_BoneInfo_C|GetBoneChildren BoneParent) self))))
    (:then_1
      (bind _values (Utilities|Map|Values (Variables|/Script/VRM4U.VrmMetaObject|GethumanoidBoneTable (Variables|/Script/VRM4U.VrmAssetListObject|GetVrmMetaObject AssetList))))
      (Variables|Default|SetbHumanoidBone (Utilities|Array|ContainsItem _values (Variables|Default|GetBoneName))))))

(event Custom|UpdateExpand
  (if (Variables|Default|GetbHumanoidBone)
    (for _array_element (Variables|Default|GetBoneChildren)
      (if (not (Variables|BP_BoneInfo_C|GetbHumanoidBone _array_element))
        (Variables|Default|SetbExpand true)))))