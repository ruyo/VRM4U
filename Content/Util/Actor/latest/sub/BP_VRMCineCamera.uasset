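; VRM cine camera actor that applies an off-center projection offset (lens shift) to its camera component, with optional compensation for the shift.
; The construction script hooks VrmCameraCheck's camera-move event, so settings reapply whenever it fires.
; FOV-tangent math derives an inverse rotation or, using target distance, an inverse location; TargetTransform refreshes only in rotation mode.
; ForceDefaultView clears offset and relative transform; otherwise FixPitch can lock actor pitch and zero roll.
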(event Custom|CustomEvent_0
  (bind _returnvalue (Class|VrmCineCameraActor|GetVrmCineCameraComponent))
  (bind _returnvalue_2 (Transformation|GetActorTransform))
  (bind _offcenterprojection_offset (Variables|Default|GetOffCenterProjection%20Offset))
  (bind _vrmcameracheck (Variables|Default|GetVrmCameraCheck))
  (bind _offcenterprojection_offset_2 (Variables|Default|GetOffCenterProjection%20Offset))
  (bind _returnvalue_3 (Class|CineCameraComponent|GetHorizontalFieldOfView _returnvalue))
  (bind _returnvalue_4 (Class|CineCameraComponent|GetVerticalFieldOfView _returnvalue))
  (bind (_location _rotation) (Math|Transform|BreakTransform _returnvalue_2))
  (bind (_x _y) (Math|Vector2D|BreakVector2D _offcenterprojection_offset_2))
  (bind _returnvalue_5 (* _offcenterprojection_offset "(X=-1.000000,Y=-1.000000)"))
  (bind (_x_2 _y_2) (Math|Vector2D|BreakVector2D _returnvalue_5))
  (bind _returnvalue_6 (/ _returnvalue_3 2.0))
  (bind _returnvalue_7 (/ _returnvalue_4 2.0))
  (bind _returnvalue_8 (Math|Trig|Tan(Degrees) _returnvalue_7))
  (bind _returnvalue_9 (Math|Trig|Tan(Degrees) _returnvalue_6))
  (Utilities|FlowControl|Sequence
    (:then_0
      (EventDispatchers|AssignOnCameraMove _vrmcameracheck (delegate Custom|OnCameraMove_Event_0))
      (Class|VrmCameraCheckComponent|SetCameraCheck _vrmcameracheck true))
    (:then_1
      (if (Variables|Default|GetbForceDefaultView)
        (Variables|/Script/VRM4U.VrmCineCameraComponent|SetOffCenterProjectionOffset _returnvalue "")
        (Transformation|ResetRelativeTransform _returnvalue :!label _label)
        (else
          (Utilities|FlowControl|Sequence
            (:then_0
              (Variables|/Script/VRM4U.VrmCineCameraComponent|SetOffCenterProjectionOffset _returnvalue (Variables|Default|GetOffCenterProjection%20Offset)))
            (:then_1
              (Utilities|FlowControl|Sequence
                (:then_0
                  (if (Variables|Default|GetbUseInverseRotMode)
                    (Utilities|FlowControl|Sequence
                      (:then_0
                        (bind _targetactor (Variables|Default|GetTargetActor)
                          (:then
                            (Variables|Default|SetTargetTransform (Transformation|GetActorTransform _targetactor)))
                          (:else
                            (Variables|Default|SetTargetTransform (Math|Transform|ComposeTransforms (Transformation|GetActorTransform) (Math|Transform|MakeTransform "100.000000, 0, 0"))))))
                      (:then_1
                        (Transformation|SetRelativeRotation _returnvalue (Math|Rotator|FindLookatRotation (Math|Vector|MakeVector 0.0 0.0 0.0) (* (Math|Vector|MakeVector 1.0 (* _returnvalue_9 _x) (* _returnvalue_8 _y)) "1.000000,-1.000000,-1.000000")) false false)))))
                (:then_1
                  (if (Variables|Default|GetbUseInverseLocationModeWithTargetActor)
                    (Transformation|SetWorldLocation _returnvalue (+ (+ (* (Math|Vector|GetRightVector _rotation) (* (Math|Vector|VectorLength (- (.Location (Math|Transform|BreakTransform (Variables|Default|GetTargetTransform))) _location)) _returnvalue_9) _x_2) (* (Math|Vector|GetUpVector _rotation) (* (Math|Vector|VectorLength (- (.Location (Math|Transform|BreakTransform (Variables|Default|GetTargetTransform))) _location)) _returnvalue_8) _y_2)) (.Location (Math|Transform|BreakTransform (Transformation|GetActorTransform)))) false false)))
                (:then_2
                  (if (not (or (Variables|Default|GetbUseInverseRotMode) (Variables|Default|GetbUseInverseLocationModeWithTargetActor)))
                    (goto _label)))))
            (:then_3
              (if (Variables|Default|GetbFixPitch)
                (Transformation|SetActorRotation (Math|Rotator|MakeRotator 0.0 (Variables|Default|GetY%20%28Pitch%29) (.Yaw (Math|Rotator|BreakRotator (Transformation|GetActorRotation)))))))))))))

(event Custom|OnCameraMove_Event_0
  (bind _returnvalue (Class|VrmCineCameraActor|GetVrmCineCameraComponent))
  (bind _returnvalue_2 (Transformation|GetActorTransform))
  (bind _offcenterprojection_offset (Variables|Default|GetOffCenterProjection%20Offset))
  (bind _offcenterprojection_offset_2 (Variables|Default|GetOffCenterProjection%20Offset))
  (bind _returnvalue_3 (Class|CineCameraComponent|GetHorizontalFieldOfView _returnvalue))
  (bind _returnvalue_4 (Class|CineCameraComponent|GetVerticalFieldOfView _returnvalue))
  (bind (_location _rotation) (Math|Transform|BreakTransform _returnvalue_2))
  (bind (_x _y) (Math|Vector2D|BreakVector2D _offcenterprojection_offset_2))
  (bind _returnvalue_5 (* _offcenterprojection_offset "(X=-1.000000,Y=-1.000000)"))
  (bind (_x_2 _y_2) (Math|Vector2D|BreakVector2D _returnvalue_5))
  (bind _returnvalue_6 (/ _returnvalue_3 2.0))
  (bind _returnvalue_7 (/ _returnvalue_4 2.0))
  (bind _returnvalue_8 (Math|Trig|Tan(Degrees) _returnvalue_7))
  (bind _returnvalue_9 (Math|Trig|Tan(Degrees) _returnvalue_6))
  (if (Variables|Default|GetbForceDefaultView)
    (Variables|/Script/VRM4U.VrmCineCameraComponent|SetOffCenterProjectionOffset _returnvalue "")
    (Transformation|ResetRelativeTransform _returnvalue :!label _label)
    (else
      (Utilities|FlowControl|Sequence
        (:then_0
          (Variables|/Script/VRM4U.VrmCineCameraComponent|SetOffCenterProjectionOffset _returnvalue (Variables|Default|GetOffCenterProjection%20Offset)))
        (:then_1
          (Utilities|FlowControl|Sequence
            (:then_0
              (if (Variables|Default|GetbUseInverseRotMode)
                (Utilities|FlowControl|Sequence
                  (:then_0
                    (bind _targetactor (Variables|Default|GetTargetActor)
                      (:then
                        (Variables|Default|SetTargetTransform (Transformation|GetActorTransform _targetactor)))
                      (:else
                        (Variables|Default|SetTargetTransform (Math|Transform|ComposeTransforms (Transformation|GetActorTransform) (Math|Transform|MakeTransform "100.000000, 0, 0"))))))
                  (:then_1
                    (Transformation|SetRelativeRotation _returnvalue (Math|Rotator|FindLookatRotation (Math|Vector|MakeVector 0.0 0.0 0.0) (* (Math|Vector|MakeVector 1.0 (* _returnvalue_9 _x) (* _returnvalue_8 _y)) "1.000000,-1.000000,-1.000000")) false false)))))
            (:then_1
              (if (Variables|Default|GetbUseInverseLocationModeWithTargetActor)
                (Transformation|SetWorldLocation _returnvalue (+ (+ (* (Math|Vector|GetRightVector _rotation) (* (Math|Vector|VectorLength (- (.Location (Math|Transform|BreakTransform (Variables|Default|GetTargetTransform))) _location)) _returnvalue_9) _x_2) (* (Math|Vector|GetUpVector _rotation) (* (Math|Vector|VectorLength (- (.Location (Math|Transform|BreakTransform (Variables|Default|GetTargetTransform))) _location)) _returnvalue_8) _y_2)) (.Location (Math|Transform|BreakTransform (Transformation|GetActorTransform)))) false false)))
            (:then_2
              (if (not (or (Variables|Default|GetbUseInverseRotMode) (Variables|Default|GetbUseInverseLocationModeWithTargetActor)))
                (goto _label)))))
        (:then_3
          (if (Variables|Default|GetbFixPitch)
            (Transformation|SetActorRotation (Math|Rotator|MakeRotator 0.0 (Variables|Default|GetY%20%28Pitch%29) (.Yaw (Math|Rotator|BreakRotator (Transformation|GetActorRotation)))))))))))

(event EventBeginPlay)

(event Collision|EventActorBeginOverlap
  (params (OtherActor :type Actor%20Object%20Reference)))

(event EventTick
  (params (DeltaSeconds :type Float%20%28single-precision%29)))

(fn ConstructionScript
  (CallFunction|CustomEvent0))