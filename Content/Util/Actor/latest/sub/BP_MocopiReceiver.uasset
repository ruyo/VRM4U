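; Receiver actor that listens for mocopi motion capture on an IP and port and feeds bone transforms to VRM4U's animation subsystem.
; At runtime Tick polls the server's frame buffer for the latest or next frame; ServerListen without BeginPlay also binds a receive callback and enables in-editor animation on the target's skeletal meshes.
; Frames also become port-keyed raw data by joint name, with optional debug cubes showing joints.
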(event Custom|ServerStop
  (bind _server (Variables|Default|Getserver)
    (:then
      (Class|VrmMocopiReceiver|Stop _server)
      (Variables|Default|Setserver 0))
    (:else)))

(event Custom|ServerListen
  (Utilities|FlowControl|Sequence
    (:then_0
      (Utilities|FlowControl|Sequence
        (:then_0
          (Utilities|FlowControl|Sequence
            (:then_0
              (bind _server (Variables|Default|Getserver)
                (:then
                  (EventDispatchers|UnbindallEventsfromOnReceived _server)
                  (Class|VrmMocopiReceiver|Stop _server)
                  (Variables|Default|Setserver 0))
                (:else)))
            (:then_1
              (bind _returnvalue (Class|VrmCaptureManager|CreateVrmMocopiReceiver (Variables|Default|GetReceive%20IPAddress) (Variables|Default|GetPort) false false "serv" self))
              (bind _output_get (Variables|Default|Setserver _returnvalue))
              (Class|VrmMocopiReceiver|SetBufferNum _output_get (Variables|Default|GetFrameCacheNum)))))
        (:then_1
          (Class|VrmMocopiReceiver|Listen (Variables|Default|Getserver))
          (if (not (Variables|Default|GetbCallBeginPlay))
            (EventDispatchers|AssignOnReceived (Variables|Default|Getserver) (delegate Custom|OnReceived_Event_0))))))
    (:then_2
      (bind _targetactor (Variables|Default|GetTargetActor)
        (:then
          (for _array_element (Actor|GetComponentsByClass _targetactor "/Script/Engine.SkeletalMeshComponent")
            (Components|SkeletalMesh|SetUpdateAnimationinEditor _array_element true)))
        (:else)))))

(event Custom|OnReceived_Event_0
  (params (data :type Struct%20Mocopi%20Data%20Structure))
  (bind (_frameno _time _mocopitransformworld _mocopitransformlocal _vrmtransformlocal _vrmtransformbonelist) (Utilities|Struct|BreakStructMocopiData data))
  (Variables|Default|SetTransformWorld _mocopitransformworld)
  (Variables|Default|SetBVHTransformLocal _vrmtransformlocal)
  (Class|VRM4UAnimSubsystem|SetBoneTransform (|VRM4UAnimSubsystem) (Variables|Default|GetPort) _vrmtransformbonelist)
  (CallFunction|UpdateRawData false))

(event Custom|UpdateBoneData
  (params (dummy :type Boolean))
  (bind _returnvalue (|VRM4UAnimSubsystem))
  (bind _port (Variables|Default|GetPort))
  (bind _server (Variables|Default|Getserver)
    (:then
      (Utilities|FlowControl|Sequence
        (:then_0
          (if (Variables|Default|GetbUseLatestBoneData)
            (bind (_data _benable) (Class|VrmMocopiReceiver|GetLatestFrameData _server))
            (if _benable
              (Variables|Default|SetTransformWorld (.MocopiTransformWorld (Utilities|Struct|BreakStructMocopiData _data)))
              (Variables|Default|SetBVHTransformLocal (.VrmTransformLocal (Utilities|Struct|BreakStructMocopiData _data)))
              (Class|VRM4UAnimSubsystem|SetBoneTransform _returnvalue _port (.VrmTransformBoneList (Utilities|Struct|BreakStructMocopiData _data))))
            (else
              (bind (_data_2 _benable_2) (Class|VrmMocopiReceiver|GetNextFrameData _server))
              (if _benable_2
                (Variables|Default|SetTransformWorld (.MocopiTransformWorld (Utilities|Struct|BreakStructMocopiData _data_2)))
                (Variables|Default|SetBVHTransformLocal (.VrmTransformLocal (Utilities|Struct|BreakStructMocopiData _data_2)))
                (Class|VRM4UAnimSubsystem|SetBoneTransform _returnvalue _port (.VrmTransformBoneList (Utilities|Struct|BreakStructMocopiData _data_2)))))))
        (:then_1
          (CallFunction|UpdateRawData false))))
    (:else)))

(event Custom|UpdateRawData
  (params (dummy :type Boolean))
  (bind _array (Utilities|Array|MakeArray "root" "torso_1" "torso_2" "torso_3" "torso_4" "torso_5" "torso_6" "torso_7" "neck_1" "neck_2" "head" "l_shoulder" "l_up_arm" "l_low_arm" "l_hand" "r_shoulder" "r_up_arm" "r_low_arm" "r_hand" "l_up_leg" "l_low_leg" "l_foot" "l_toes" "r_up_leg" "r_low_leg" "r_foot" "r_toes"))
  (bind _bvhtransformlocal (Variables|Default|GetBVHTransformLocal))
  (if (== (Utilities|Array|Length _array) (Utilities|Array|Length _bvhtransformlocal))
    (for (_array_element _array_index) _array
      (Utilities|Map|Add (Variables|Default|GetRawData) _array_element (Utilities|Array|Get(acopy) _bvhtransformlocal _array_index)))
    (Class|VRM4UAnimSubsystem|SetRawData (|VRM4UAnimSubsystem) (Variables|Default|GetPort) (Variables|Default|GetRawData))))

(event Custom|init
  (params (dummy :type Boolean))
  (bind _addresstable (Class|VrmNetworkBPFunctionLibrary|VRMGetIPAddressTable))
  (Variables|Default|SetIPAddressList _addresstable)
  (if (Utilities|Enum|Equal(Enum) (Variables|Default|GetReceive%20IPAddress) "")
    (if (Utilities|Array|IsValidIndex (Variables|Default|GetIPAddressList))
      (Variables|Default|SetReceive%20IPAddress (Utilities|Array|Get(acopy) (Variables|Default|GetIPAddressList))))))

(event EventBeginPlay
  (Variables|Default|SetbCallBeginPlay true)
  (Utilities|FlowControl|Sequence
    (:then_0
      (Utilities|FlowControl|Sequence
        (:then_0
          (bind _server (Variables|Default|Getserver)
            (:then
              (EventDispatchers|UnbindallEventsfromOnReceived _server)
              (Class|VrmMocopiReceiver|Stop _server)
              (Variables|Default|Setserver 0))
            (:else)))
        (:then_1
          (bind _returnvalue (Class|VrmCaptureManager|CreateVrmMocopiReceiver (Variables|Default|GetReceive%20IPAddress) (Variables|Default|GetPort) false false "serv" self))
          (bind _output_get (Variables|Default|Setserver _returnvalue))
          (Class|VrmMocopiReceiver|SetBufferNum _output_get (Variables|Default|GetFrameCacheNum)))))
    (:then_1
      (Class|VrmMocopiReceiver|Listen (Variables|Default|Getserver))
      (if (not (Variables|Default|GetbCallBeginPlay))
        (EventDispatchers|AssignOnReceived (Variables|Default|Getserver) (delegate Custom|OnReceived_Event_0))))))

(event Collision|EventActorBeginOverlap
  (params (OtherActor :type Actor%20Object%20Reference)))

(event EventTick
  (params (DeltaSeconds :type Float%20%28single-precision%29))
  (bind _transformworld (Variables|Default|GetTransformWorld))
  (Utilities|FlowControl|Sequence
    (:then_1
      (if (Variables|Default|GetbDebugBone)
        (Utilities|FlowControl|Sequence
          (:then_0
            (Utilities|FlowControl|DoOnce (not (Variables|Default|GetbDebugBone))
              (:Completed
                (for _index (range 0 26)
                  (bind _returnvalue (AddComponent|AddStaticMeshComponent false (Math|Transform|MakeTransform "0, 0, 0" "0, 0, 0" "0.050000,0.050000,0.050000")))
                  (Utilities|FlowControl|Sequence
                    (:then_0
                      (Components|StaticMesh|SetStaticMesh _returnvalue "/Engine/BasicShapes/Cube.Cube")
                      (Transformation|AttachComponentToComponent _returnvalue (Variables|Default|GetScene) "None" "SnapToTarget" "SnapToTarget" "SnapToTarget" true))
                    (:then_1
                      (Utilities|Array|AddUnique (Variables|Default|GetDebugBoneCube) _returnvalue)))))))
          (:then_1
            (for (_array_element _array_index) (Variables|Default|GetDebugBoneCube)
              (if (Utilities|Array|IsValidIndex _transformworld _array_index)
                (Transformation|SetRelativeTransform _array_element (Math|Transform|MakeTransform (.Location (Math|Transform|BreakTransform (Utilities|Array|Get(acopy) _transformworld _array_index))) (.Rotation (Math|Transform|BreakTransform (Utilities|Array|Get(acopy) _transformworld _array_index))) "0.050000,0.050000,0.050000") false false)))))))
    (:then_3
      (CallFunction|UpdateBoneData false))))

(event EventEndPlay
  (params (EndPlayReason :type EEndPlayReason%20Enum :default "Destroyed"))
  (bind _server (Variables|Default|Getserver)
    (:then
      (EventDispatchers|UnbindallEventsfromOnReceived _server)
      (Class|VrmMocopiReceiver|Stop _server)
      (Variables|Default|Setserver 0))
    (:else)))

(event EventDestroyed
  (bind _server (Variables|Default|Getserver)
    (:then
      (EventDispatchers|UnbindallEventsfromOnReceived _server)
      (Class|VrmMocopiReceiver|Stop _server)
      (Variables|Default|Setserver 0))
    (:else)))

(fn ConstructionScript
  (CallFunction|Init false))