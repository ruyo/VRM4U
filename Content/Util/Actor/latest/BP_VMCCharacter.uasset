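; Character actor that sets up a skeletal mesh to be driven by VMC bone data through the ABP_VRoidVMC_Bone Anim Blueprint.
; The Construction Script calls an init event that enables animation updates in the editor, so the mesh can animate outside of play.
; Init then casts the anim instance and copies the actor's VMC update flag, character index and port settings into it.
; The actor has no runtime logic of its own.
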(event Custom|init
  (params (dummy :type Boolean))
  (Utilities|FlowControl|Sequence
    (:then_0
      (Components|SkeletalMesh|SetUpdateAnimationinEditor (Variables|Default|GetSkeletalMesh) true))
    (:then_1
      (bind _asabp_vroid_vmc_bone (Utilities|Casting|CastToABP_VRoidVMC_Bone (Components|SkeletalMesh|GetAnimInstance (Variables|Default|GetSkeletalMesh))))
      (Variables|/VRM4U/Util/Actor/latest/ABP_VRoidVMC_Bone.ABP_VRoidVMC_Bone_C|SetbUpdateBone _asabp_vroid_vmc_bone (Variables|Default|GetbUpdateVMC))
      (Variables|/VRM4U/Util/Actor/latest/ABP_VRoidVMC_Bone.ABP_VRoidVMC_Bone_C|SetCharacterIndex _asabp_vroid_vmc_bone (Variables|Default|GetCharacterIndex))
      (Variables|/VRM4U/Util/Actor/latest/ABP_VRoidVMC_Bone.ABP_VRoidVMC_Bone_C|SetPortNo _asabp_vroid_vmc_bone (Variables|Default|GetPortNo))
      (Variables|/VRM4U/Util/Actor/latest/ABP_VRoidVMC_Bone.ABP_VRoidVMC_Bone_C|SetbUsePort _asabp_vroid_vmc_bone (Variables|Default|GetbUsePort)))))

(event EventBeginPlay)

(event Collision|EventActorBeginOverlap
  (params (OtherActor :type Actor%20Object%20Reference)))

(event EventTick
  (params (DeltaSeconds :type Float%20%28single-precision%29)))

(fn ConstructionScript
  (CallFunction|Init false))