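; Editor utility actor that copies a source material instance along with its whole parent chain, down to the base Material.
; CopyMaterial walks up the parents with a bounded loop, and Duplicate uses AssetTools to create "_copy"-prefixed assets in the source's folder.
; The copied instances are then re-parented to one another via VRMChangeMaterialParent, ending at the copied root Material, so the new hierarchy mirrors the original.
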(event Custom|CopyMaterial
  (bind _newvar_0 (Variables|Default|GetNewVar_0))
  (bind _newvar_0_2 (Variables|Default|GetNewVar_0))
  (bind _srcmaterial (Variables|Default|GetsrcMaterial)
    (:then
      (Utilities|Array|Clear (Variables|Default|GetNewVar_0))
      (bind _output_get (Variables|Default|Setcurrent_mat _srcmaterial))
      (CallFunction|Duplicate _output_get)
      (Utilities|FlowControl|ForLoopwithBreak 0 20 :!label _label
        (:LoopBody
          (if (.bSuccess (Utilities|Casting|CastToMaterialInstanceConstant (Variables|/Script/Engine.MaterialInstance|GetParent (Variables|Default|Getcurrent_mat))))
            (bind _output_get_2 (Variables|Default|Setcurrent_mat (.AsMaterial%20Instance%20Constant (Utilities|Casting|CastToMaterialInstanceConstant (Variables|/Script/Engine.MaterialInstance|GetParent (Variables|Default|Getcurrent_mat))))))
            (CallFunction|Duplicate _output_get_2)
            (else
              (Utilities|FlowControl|Sequence
                (:then_2
                  (CallFunction|Duplicate (.AsMaterial (Utilities|Casting|CastToMaterial (Variables|/Script/Engine.MaterialInstance|GetParent (Variables|Default|Getcurrent_mat)))))
                  ;[1 1 1] parent
                  (for (_ _array_index) _newvar_0_2
                    (if (!= _array_index (Utilities|Array|LastIndex _newvar_0_2))
                      (Class|VrmBPFunctionLibrary|VRMChangeMaterialParent (Utilities|Array|Get(acopy) _newvar_0 _array_index) (Utilities|Array|Get(acopy) _newvar_0 (+ _array_index 1)))
                      (else
                        (Class|VrmBPFunctionLibrary|VRMChangeMaterialParent (Utilities|Array|Get(acopy) _newvar_0 _array_index) (Variables|Default|GetRootMaterial))))))
                (:then_3
                  (goto _label Break))))))))
    (:else)))

(event Custom|Duplicate
  (params (NewParam :type Object%20Object%20Reference))
  ;[1 1 1] copy
  (bind _returnvalue (Class|AssetToolsHelpers|GetAssetTools))
  (bind _returnvalue_2 (Class|AssetTools|DuplicateAsset(Message) (Utilities|ToObject(Interface) _returnvalue) (Utilities|String|Append "_copy" (.RightS (Utilities|String|Split (Class|KismetSystemLibrary|GetPathName NewParam) "." "IgnoreCase" "FromEnd"))) (.LeftS (Utilities|String|Split (Class|KismetSystemLibrary|GetPathName (Variables|Default|GetsrcMaterial)) "/" "IgnoreCase" "FromEnd")) NewParam))
  (bind _asmaterial_instance_constant (Utilities|Casting|CastToMaterialInstanceConstant _returnvalue_2)
    (:then
      (Utilities|Array|Add (Variables|Default|GetNewVar_0) _asmaterial_instance_constant))
    (:CastFailed
      (bind _asmaterial (Utilities|Casting|CastToMaterial _returnvalue_2))
      (Variables|Default|SetRootMaterial _asmaterial))))

(event EventBeginPlay)

(event Collision|EventActorBeginOverlap
  (params (OtherActor :type Actor%20Object%20Reference)))

(event EventTick
  (params (DeltaSeconds :type Float%20%28single-precision%29)))

(fn ConstructionScript)