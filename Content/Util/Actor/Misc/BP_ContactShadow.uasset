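; Contact shadow actor that attaches to a target component or actor and projects a shadow for it with a decal.
; On construction, an orthographic SceneCapture2D renders only the target actor into a single-channel R16f render target created at runtime.
; That target feeds a dynamic decal material with a blend rate, and the shadow area size drives both capture width and decal scale.
; An optional debug cube displays the shadowmap and is otherwise destroyed.
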(event Custom|init
  (bind _scenecapturecomponent2d (Variables|Default|GetSceneCaptureComponent2D))
  (bind _shadowareasize (Variables|Default|GetShadowAreaSize))
  (bind _shadowmapsize (Variables|Default|GetShadowMapSize))
  (bind _returnvalue (Math|Float|Truncate _shadowmapsize))
  (Utilities|FlowControl|Sequence
    (:then_0
      (bind _attachtarget (Variables|Default|GetAttachTarget)
        (:then
          (Transformation|AttachComponentToComponent _attachtarget "None" "SnapToTarget" "SnapToTarget" "SnapToTarget" true))
        (:else
          (bind _targetactor (Variables|Default|GetTargetActor)
            (:then
              (Transformation|AttachActorToActor _targetactor "None" "SnapToTarget" "SnapToTarget" "SnapToTarget" true))
            (:else)))))
    (:then_1
      (Rendering|SceneCapture|ShowOnlyActorComponents _scenecapturecomponent2d (Variables|Default|GetTargetActor))
      (Utilities|FlowControl|Sequence
        (:then_0
          (Variables|/Script/Engine.SceneCaptureComponent2D|SetOrthoWidth _scenecapturecomponent2d _shadowareasize)
          (bind _returnvalue_2 (Class|VrmBPFunctionLibrary|VRMCreateRenderTarget2D _returnvalue _returnvalue "RTF_R16f" "(R=1.000000,G=1.000000,B=1.000000,A=1.000000)"))
          (Variables|/Script/Engine.SceneCaptureComponent2D|SetTextureTarget _scenecapturecomponent2d _returnvalue_2)
          (Transformation|SetWorldScale3D (Variables|Default|GetDecal) (Math|Conversions|ToVector(Float) (* 1.0 (/ _shadowareasize (Math|Float|MakeLiteralFloat 128.0))))))
        (:then_1
          (bind _cube (Variables|Default|GetCube)
            (:then
              (bind _returnvalue_3 (Rendering|Material|CreateDynamicMaterialInstance _cube 0 "/VRM4U/MaterialUtil/M_VrmDebugContactShadowmap.M_VrmDebugContactShadowmap" "None" :!class /Script/Engine.PrimitiveComponent))
              (Rendering|Material|SetTextureParameterValue _returnvalue_3 "Shadowmap" _returnvalue_2))
            (:else)))
        (:then_2
          (bind _returnvalue_4 (Rendering|Material|CreateDynamicMaterialInstance "/VRM4U/MaterialUtil/M_ContactShadow.M_ContactShadow" "None" :!class /Script/Engine.KismetMaterialLibrary))
          (Rendering|Material|SetTextureParameterValue _returnvalue_4 "Shadowmap" _returnvalue_2)
          (Rendering|Material|SetScalarParameterValue _returnvalue_4 "BlendRate" (Variables|Default|GetBlendRate) :!class /Script/Engine.MaterialInstanceDynamic)
          (Rendering|Components|Decal|SetDecalMaterial (Variables|Default|GetDecal) _returnvalue_4))))
    (:then_2
      (if (Variables|Default|GetbDebugCube)
        (Rendering|SetVisibility (Variables|Default|GetCube) true false)
        (else
          (bind _cube_2 (Variables|Default|GetCube)
            (:then
              (Components|DestroyComponent _cube_2))
            (:else)))))))

(event EventBeginPlay)

(event Collision|EventActorBeginOverlap
  (params (OtherActor :type Actor%20Object%20Reference)))

(event EventTick
  (params (DeltaSeconds :type Float%20%28single-precision%29)))

(fn ConstructionScript
  (CallFunction|Init))