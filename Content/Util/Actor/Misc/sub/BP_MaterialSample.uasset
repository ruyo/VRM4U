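; Material sample actor that previews the VRM MToon opaque material on a sphere and two static mesh components.
; The construction script creates a dynamic instance of the same material for each component, varying shade color, shade toony and, on the last, shade texture.
; A final loop over the collected instances applies one clothing texture as diffuse and shade, overriding that earlier white shade texture.
; The event graph has no active logic.
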(event EventBeginPlay)

(event Collision|EventActorBeginOverlap
  (params (OtherActor :type Actor%20Object%20Reference)))

(event EventTick
  (params (DeltaSeconds :type Float%20%28single-precision%29)))

(fn ConstructionScript
  (Utilities|FlowControl|Sequence
    (:then_0
      (bind _returnvalue (Rendering|Material|CreateDynamicMaterialInstance (Variables|Default|GetSphere) 0 "/VRM4U/MaterialUtil/MToonUtil/MI_VrmMToonOptUnlitOpaque.MI_VrmMToonOptUnlitOpaque" "None" :!class /Script/Engine.PrimitiveComponent))
      (Utilities|Array|Add (LocalVariables|GetNewLocalVar_0) _returnvalue)
      (Rendering|Material|SetVectorParameterValue _returnvalue "mtoon_ShadeColor" "(R=0.800000,G=0.200000,B=0.500000,A=1.000000)" :!class /Script/Engine.MaterialInstanceDynamic)
      (Rendering|Material|SetScalarParameterValue _returnvalue "mtoon_ShadeToony" 1.0 :!class /Script/Engine.MaterialInstanceDynamic))
    (:then_1
      (bind _returnvalue_2 (Rendering|Material|CreateDynamicMaterialInstance (Variables|Default|GetStaticMesh) 0 "/VRM4U/MaterialUtil/MToonUtil/MI_VrmMToonOptUnlitOpaque.MI_VrmMToonOptUnlitOpaque" "None" :!class /Script/Engine.PrimitiveComponent))
      (Utilities|Array|Add (LocalVariables|GetNewLocalVar_0) _returnvalue_2)
      (Rendering|Material|SetVectorParameterValue _returnvalue_2 "mtoon_ShadeColor" "(R=0.800000,G=0.200000,B=0.500000,A=1.000000)" :!class /Script/Engine.MaterialInstanceDynamic))
    (:then_2
      (bind _returnvalue_3 (Rendering|Material|CreateDynamicMaterialInstance (Variables|Default|GetStaticMesh1) 0 "/VRM4U/MaterialUtil/MToonUtil/MI_VrmMToonOptUnlitOpaque.MI_VrmMToonOptUnlitOpaque" "None" :!class /Script/Engine.PrimitiveComponent))
      (Utilities|Array|Add (LocalVariables|GetNewLocalVar_0) _returnvalue_3)
      (Rendering|Material|SetVectorParameterValue _returnvalue_3 "mtoon_ShadeColor" "(R=0.139805,G=0.395834,B=0.122657,A=1.000000)" :!class /Script/Engine.MaterialInstanceDynamic)
      (Rendering|Material|SetTextureParameterValue _returnvalue_3 "mtoon_tex_ShadeTexture" "/VRM4U/MaterialUtil/T_DummyWhite.T_DummyWhite")
      (Rendering|Material|SetScalarParameterValue _returnvalue_3 "mtoon_ShadeToony" 1.0 :!class /Script/Engine.MaterialInstanceDynamic))
    (:then_3
      (for _array_element (LocalVariables|GetNewLocalVar_0)
        (Rendering|Material|SetTextureParameterValue _array_element "gltf_tex_diffuse" "/VRM4U/Util/BaseCharacter/Mesh/T_F00_001_Tops_01.T_F00_001_Tops_01")
        (Rendering|Material|SetTextureParameterValue _array_element "mtoon_tex_shadeTexture" "/VRM4U/Util/BaseCharacter/Mesh/T_F00_001_Tops_01.T_F00_001_Tops_01")))))