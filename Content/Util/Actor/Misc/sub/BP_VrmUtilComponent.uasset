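; Utility component that resolves the VRM asset list and target mesh component for a given actor or skinned mesh component.
; SetActor special-cases VRM4U actor types, otherwise scanning attached actors' skinned meshes, optionally by component index.
; Asset lists are found via package-name lookups on the mesh, SK_-to-VA_ naming and first material, with VRoidSimple hardcoded.
; Helpers map humanoid bone names to mesh bones and transforms, and pick a main light by intensity.
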(event Custom|SetVRMAssetListFromMesh
  (params (NewParam :type Skeletal%20Mesh%20Object%20Reference))
  ;[1 1 1] old
  (Utilities|FlowControl|Sequence
    (:then_0
      (Utilities|IsValid NewParam
        (:Is%20Valid
          (Variables|Default|GetVRMAssetList
            (:then)
            (:else
              (Utilities|FlowControl|Sequence
                (:then_0
                  (bind _outassetdata (Class|VrmBPFunctionLibrary|VRMGetAssetsbyPackageName (Utilities|String|StringToName (.LeftS (Utilities|String|Split (Class|KismetSystemLibrary|GetPathName NewParam) "." "IgnoreCase" "FromEnd"))) false))
                  (for _array_element _outassetdata
                    (if (>= (Utilities|String|FindSubstring (Utilities|String|ToString(Name) (Class|VrmBPFunctionLibrary|VRMGetTopLevelAssetName _array_element)) "VrmAssetListObject") 0)
                      (Variables|Default|SetVRMAssetList (.AsVrm%20Asset%20List%20Object (Utilities|Casting|CastToVrmAssetListObject (Class|AssetRegistryHelpers|GetAsset _array_element)))))))
                (:then_1
                  (Variables|Default|GetVRMAssetList
                    (:then)
                    (:else
                      (if (== NewParam "/VRM4U/Util/BaseCharacter/Mesh/SK_VRoidSimple.SK_VRoidSimple")
                        (Variables|Default|SetVRMAssetList "/VRM4U/Util/BaseCharacter/Mesh/VRoidSimple_VrmAssetList.VRoidSimple_VrmAssetList")))))))))
        (:Is%20Not%20Valid
          (Variables|Default|SetVRMAssetList 0))))))

(event Custom|SetVRMAssetListFromMeshComponent
  (params (SkeletalMesh :type Skeletal%20Mesh%20Object%20Reference))
  (Utilities|FlowControl|Sequence
    (:then_0
      (CallFunction|Clear))
    (:then_1
      (bind _vrmassetlist (CallFunction|GetTargetVRMAssetList SkeletalMesh))
      (Utilities|IsValid _vrmassetlist
        (:Is%20Valid
          (Variables|Default|SetVrmAssetList _vrmassetlist))))))

(event Custom|clear
  (Variables|Default|SetVrmModelActor 0)
  (Variables|Default|SetVRMAssetList 0)
  (Variables|Default|SetTargetMeshComponent 0)
  (Variables|Default|SetTargetAsSceneComponent 0)
  (Utilities|Array|Clear (Variables|Default|Gettmp_targetActor)))

(event Custom|SetTargetMeshComponent
  (params (TargetMeshComponent :type Skeletal%20Mesh%20Component%20Object%20Reference) (TargetAsSkinnedMeshComponent :type Skinned%20Mesh%20Component%20Object%20Reference))
  (Utilities|FlowControl|Sequence
    (:then_0
      (Variables|Default|SetTargetMeshComponent TargetMeshComponent))
    (:then_1
      (Variables|Default|SetTargetAsSkinnedMeshComponent TargetAsSkinnedMeshComponent))
    (:then_2
      (bind _targetmeshcomponent (Variables|Default|GetTargetMeshComponent)
        (:then
          (Variables|Default|SetTargetAsSkinnedMeshComponent _targetmeshcomponent)
          (Variables|Default|SetTargetAsSceneComponent _targetmeshcomponent))
        (:else
          (bind _targetasskinnedmeshcomponent (Variables|Default|GetTargetAsSkinnedMeshComponent)
            (:then
              (Variables|Default|SetTargetAsSceneComponent _targetasskinnedmeshcomponent)
              (bind _asskeletal_mesh_component (Utilities|Casting|CastToSkeletalMeshComponent _targetasskinnedmeshcomponent))
              (Variables|Default|SetTargetMeshComponent _asskeletal_mesh_component))
            (:else)))))))

(event Custom|SetActorByComponent
  (params (TargetComponent :type Skinned%20Mesh%20Component%20Object%20Reference))
  (Utilities|FlowControl|Sequence
    (:then_1
      (Utilities|IsValid TargetComponent
        (:Is%20Valid
          (CallFunction|SetVRMAssetListfromMeshComponent (Class|VrmBPFunctionLibrary|VRMGetSkeletalMeshfromSkinnedMeshComponent TargetComponent))
          (Variables|Default|GetVrmAssetList
            (:then
              (CallFunction|SetTargetMeshComponent (.AsSkeletal%20Mesh%20Component (Utilities|Casting|CastToSkeletalMeshComponent TargetComponent)) TargetComponent))
            (:else)))))))

(event Custom|SetActor
  (params (TargetActor :type Actor%20Object%20Reference))
  (bind _returnvalue (Components|GetOwner))
  (Utilities|IsValid TargetActor
    (:Is%20Valid
      (Utilities|FlowControl|Sequence
        (:then_0
          (CallFunction|Clear))
        (:then_1
          (if (Variables|Default|GetbSimpleTargetMode)
            (Variables|Default|Settmp_targetActor (Utilities|Array|MakeArray TargetActor))
            (else
              ;[1 1 1] Search target
              (bind _asbp_vrm_model_actor (Utilities|Casting|CastToBP_VrmModelActor TargetActor)
                (:then
                  (Utilities|FlowControl|Sequence
                    (:then_0
                      (Variables|Default|SetVrmModelActor _asbp_vrm_model_actor))
                    (:then_1
                      (bind _attachmodeactor (Variables|/VRM4U/Util/BaseCharacter/BP_VrmModelActor.BP_VrmModelActor_C|GetAttachModeActor _asbp_vrm_model_actor)
                        (:then
                          (CallFunction|SetTargetMeshComponent (Variables|/Script/Engine.SkeletalMeshActor|GetSkeletalMeshComponent _attachmodeactor)))
                        (:else
                          (CallFunction|SetTargetMeshComponent (Variables|/VRM4U/Util/BaseCharacter/BP_VrmModelActor.BP_VrmModelActor_C|GetSkeletalMeshComponent_Dst _asbp_vrm_model_actor)))))
                    (:then_2
                      (Variables|Default|SetVRMAssetList (Variables|/VRM4U/Util/BaseCharacter/BP_VrmModelActor.BP_VrmModelActor_C|GetVrmAssetList _asbp_vrm_model_actor)))))
                (:CastFailed
                  (bind _asbp_vrm_character_base (Utilities|Casting|CastToBP_VrmCharacterBase TargetActor)
                    (:then
                      (CallFunction|SetTargetMeshComponent (Variables|/Script/Engine.Character|GetMesh _asbp_vrm_character_base))
                      (Variables|Default|SetVRMAssetList (Variables|/VRM4U/Util/BaseCharacter/BP_VrmCharacterBase.BP_VrmCharacterBase_C|GetVRMAssetList _asbp_vrm_character_base)))
                    (:CastFailed
                      (bind _asbp_vrm_pose_copy (Utilities|Casting|CastToBP_VrmPoseCopy TargetActor)
                        (:then
                          (bind _output_get (Variables|Default|Settmp_posecopy _asbp_vrm_pose_copy))
                          (bind _assetlistoverride (Variables|/VRM4U/Util/BaseCharacter/BP_VrmPoseCopy.BP_VrmPoseCopy_C|GetAssetListOverride _output_get)
                            (:then
                              (Utilities|FlowControl|Sequence
                                (:then_0
                                  (Variables|Default|SetVRMAssetList _assetlistoverride))
                                (:then_1
                                  (bind _skeletalmesh (Variables|/VRM4U/Util/BaseCharacter/BP_VrmPoseCopy.BP_VrmPoseCopy_C|GetSkeletalMesh _output_get)
                                    (:then
                                      (CallFunction|SetTargetMeshComponent _skeletalmesh))
                                    (:else)))))
                            (:else
                              (Utilities|FlowControl|Sequence
                                (:then_0
                                  (Variables|Default|SetVRMAssetList (Variables|BP_VrmUtilComponent_C|GetVrmAssetList (Variables|/VRM4U/Util/BaseCharacter/BP_VrmPoseCopy.BP_VrmPoseCopy_C|GetBP_VrmUtilComponent _output_get)))
                                  (Variables|Default|GetVrmAssetList
                                    (:then)
                                    (:else
                                      (Variables|Default|SetVRMAssetList (Variables|/VRM4U/Util/BaseCharacter/BP_VrmPoseCopy.BP_VrmPoseCopy_C|GetTmpVrmAsset _output_get)))))
                                (:then_1
                                  (CallFunction|SetTargetMeshComponent 0 (Variables|/VRM4U/Util/BaseCharacter/BP_VrmPoseCopy.BP_VrmPoseCopy_C|GetSkeletalMesh _output_get)))))))
                        (:CastFailed
                          (bind _asmtoon_actor (Utilities|Casting|CastToMToonActor TargetActor)
                            (:then
                              (CallFunction|SetTargetMeshComponent (Variables|/VRM4U/Util/Actor/MToonActor.MToonActor_C|GetSkeletalMesh _asmtoon_actor))
                              (Variables|Default|SetVRMAssetList (Variables|/VRM4U/Util/Actor/MToonActor.MToonActor_C|GetVRMAssetList _asmtoon_actor)))
                            (:CastFailed
                              (bind _asbp_model_attach (Utilities|Casting|CastToBP_ModelAttach TargetActor)
                                (:then
                                  (CallFunction|SetActor (Variables|/VRM4U/Util/BaseCharacter/Misc/BP_ModelAttach.BP_ModelAttach_C|GetVRMParent _asbp_model_attach)))
                                (:CastFailed
                                  (bind _asskeletal_mesh_actor (Utilities|Casting|CastToSkeletalMeshActor TargetActor)
                                    (:then
                                      (Variables|Default|Settmp_targetActor (Utilities|Array|MakeArray _asskeletal_mesh_actor)))
                                    (:CastFailed
                                      ;;[1 1 1] self and children
                                      (bind _children (CallFunction|GetAllAttachedActors TargetActor))
                                      (bind _output_get_2 (Variables|Default|Settmp_targetActor _children))
                                      (Utilities|Array|Insert _output_get_2 TargetActor))))))))))))))))
        (:then_2
          (bind _array_element (Utilities|Array|ForEachLoopwithBreak (Variables|Default|Gettmp_targetActor) :!label _label)
            (:LoopBody
              (if (and (!= (Actor|GetAttachParentActor _array_element) _returnvalue) (!= _array_element _returnvalue))
                (bind (_array_element_2 _array_index) (Utilities|Array|ForEachLoopwithBreak (Actor|GetComponentsByClass _array_element "/Script/Engine.SkinnedMeshComponent") :!label _label_2)
                  (:LoopBody
                    (if (< (Variables|Default|GetTargetComponentIndex) 0)
                      (bind _vrmassetlist (CallFunction|GetTargetVRMAssetList (Class|VrmBPFunctionLibrary|VRMGetSkeletalMeshfromSkinnedMeshComponent _array_element_2) :!label _label_3))
                      (bind _output_get_3 (Variables|Default|SetVRMAssetList _vrmassetlist))
                      (Utilities|IsValid _output_get_3
                        (:Is%20Valid
                          (Utilities|FlowControl|Sequence
                            (:then_0
                              (CallFunction|SetTargetMeshComponent (.AsSkeletal%20Mesh%20Component (Utilities|Casting|CastToSkeletalMeshComponent _array_element_2)) _array_element_2))
                            (:then_1
                              (goto _label Break))
                            (:then_2
                              (goto _label_2 Break)))))
                      (elif (== _array_index (Variables|Default|GetTargetComponentIndex))
                        (goto _label_3)))))))))
        (:then_3
          (Variables|Default|GetVrmAssetList
            (:then)
            (:else
              (Development|PrintString (Utilities|String|Append "!! Warning  No VrmAssetList" "   " (Utilities|GetDisplayName TargetActor))))))))
    (:Is%20Not%20Valid
      (CallFunction|Clear))))

(event EventBeginPlay)

(event EventTick
  (params (DeltaSeconds :type Float%20%28single-precision%29)))

(fn GetVrmBoneTransform
  (params (VrmBoneName :type Name) (TransformSpace :type ERelativeTransformSpace%20Enum :default "RTS_World"))
  (bind _returnvalue (Utilities|String|ToString(Name) VrmBoneName))
  (bind _vrmassetlist (Variables|Default|GetVrmAssetList))
  (bind _targetasscenecomponent (Variables|Default|GetTargetAsSceneComponent))
  (bind _vrmmetaobject (Variables|/Script/VRM4U.VrmAssetListObject|GetVrmMetaObject _vrmassetlist))
  (bind _humanoidbonetable (Variables|/Script/VRM4U.VrmMetaObject|GethumanoidBoneTable _vrmmetaobject))
  (bind (_value _returnvalue_2) (Utilities|Map|Find _humanoidbonetable _returnvalue))
  (bind _returnvalue_3 (Utilities|String|StringToName _value))
  (Variables|Default|GetVrmAssetList
    (:then
      (Utilities|FlowControl|Sequence
        (:then_0
          (if _returnvalue_2
            (if (Transformation|DoesSocketExist _targetasscenecomponent _returnvalue_3)
              (LocalVariables|SetNewLocalVar_0 (Transformation|GetSocketTransform _targetasscenecomponent _returnvalue_3 TransformSpace))
              (LocalVariables|SetfFound true))))
        (:then_1
          (return (LocalVariables|GetNewLocalVar_0) (LocalVariables|GetfFound)))))
    (:else
      (return (LocalVariables|GetNewLocalVar_0) (LocalVariables|GetfFound)))))

(fn GetAllAttachedActorInternal
  (params (RootActor :type Actor%20Object%20Reference) (Result :type Array%20of%20Actor%20Object%20References))
  (for _array_element (Actor|GetAttachedActors RootActor)
    (Utilities|FlowControl|Sequence
      (:then_0
        (Utilities|Array|Add Result _array_element))
      (:then_1
        (CallFunction|GetAllAttachedActorInternal _array_element Result)))))

(fn GetAllAttachedActors
  (params (RootActor :type Actor%20Object%20Reference))
  (bind _result (LocalVariables|GetResult))
  (CallFunction|GetAllAttachedActorInternal RootActor _result)
  (return _result))

(fn GetMainDirectionalLightComponent
  (Utilities|FlowControl|Sequence
    (:then_0
      (bind _outactors (Actor|GetAllActorsOfClass "/Script/Engine.DirectionalLight"))
      (for _array_element _outactors
        (bind _mainlightcomponent_local (LocalVariables|GetMainLightComponent_Local)
          (:then
            (if (and (Variables|/Script/Engine.LightComponentBase|GetbAffectsWorld _mainlightcomponent_local) (< (Variables|/Script/Engine.LightComponentBase|GetIntensity _mainlightcomponent_local) (Variables|/Script/Engine.LightComponentBase|GetIntensity (Variables|/Script/Engine.Light|GetLightComponent _array_element))))
              (LocalVariables|SetMainLightComponent_Local (Variables|/Script/Engine.Light|GetLightComponent _array_element) :!label _label)))
          (:else
            (goto _label)))))
    (:then_1
      (bind _outactors_2 (Class|VrmBPFunctionLibrary|VRMGetAllActorsHasSceneComponent "/Script/Engine.LightComponent"))
      (for _array_element_2 _outactors_2
        (if (not (Utilities|ClassIsChildOf (Utilities|GetClass _array_element_2) "/VRM4U/Util/Actor/Misc/sub/CharacterLightRigBase.CharacterLightRigBase_C"))
          (bind _mainlightcomponent_local_2 (LocalVariables|GetMainLightComponent_Local)
            (:then
              (if (and (Variables|/Script/Engine.LightComponentBase|GetbAffectsWorld _mainlightcomponent_local_2) (< (Variables|/Script/Engine.LightComponentBase|GetIntensity _mainlightcomponent_local_2) (Variables|/Script/Engine.LightComponentBase|GetIntensity (Actor|GetComponentbyClass _array_element_2 "/Script/Engine.LightComponent"))))
                (LocalVariables|SetMainLightComponent_Local (Actor|GetComponentbyClass _array_element_2 "/Script/Engine.LightComponent") :!label _label_2)))
            (:else
              (goto _label_2))))))
    (:then_2
      (return (LocalVariables|GetMainLightComponent_Local)))))

(fn GetMeshBoneName
  (params (VrmBoneName :type Name))
  (bind _returnvalue (Utilities|String|ToString(Name) VrmBoneName))
  (bind _vrmassetlist (Variables|Default|GetVrmAssetList))
  (bind _vrmmetaobject (Variables|/Script/VRM4U.VrmAssetListObject|GetVrmMetaObject _vrmassetlist))
  (bind _humanoidbonetable (Variables|/Script/VRM4U.VrmMetaObject|GethumanoidBoneTable _vrmmetaobject))
  (bind (_value _returnvalue_2) (Utilities|Map|Find _humanoidbonetable _returnvalue))
  (Utilities|FlowControl|Sequence
    (:then_0
      (Variables|Default|GetVrmAssetList
        (:then
          (Utilities|FlowControl|Sequence
            (:then_0
              (if _returnvalue_2
                (return true (Utilities|String|StringToName _value))))))
        (:else)))
    (:then_1
      (return false "None"))))

(fn GetTargetVRMAssetList
  (params (SkeletalMesh :type Skeletal%20Mesh%20Object%20Reference))
  (bind _returnvalue (Class|KismetSystemLibrary|GetPathName SkeletalMesh))
  (bind _materials (Variables|/Script/Engine.SkeletalMesh|GetMaterials SkeletalMesh))
  (bind _lefts (Utilities|String|Split _returnvalue "." "IgnoreCase" "FromEnd"))
  (bind _output (Utilities|Array|Get(acopy) _materials))
  (bind _materialinterface (Utilities|Struct|BreakSkeletalMaterial _output))
  (bind (_lefts_2 _rights) (Utilities|String|Split _lefts "/SK_" "IgnoreCase" "FromEnd"))
  (if (== SkeletalMesh "/VRM4U/Util/BaseCharacter/Mesh/SK_VRoidSimple.SK_VRoidSimple")
    (Utilities|FlowControl|Sequence
      (:then_0
        ;[1 1 1] VRoidSimple
        (return "/VRM4U/Util/BaseCharacter/Mesh/VRoidSimple_VrmAssetList.VRoidSimple_VrmAssetList")))
    (else
      (Utilities|FlowControl|Sequence
        (:then_0
          (bind _outassetdata (Class|VrmBPFunctionLibrary|VRMGetAssetsbyPackageName (Utilities|String|StringToName _lefts) false))
          (LocalVariables|SetNewLocalVar_1 _outassetdata)
          (bind _outassetdata_2 (Class|VrmBPFunctionLibrary|VRMGetAssetsbyPackageName (Utilities|String|StringToName (Utilities|String|Append _lefts_2 "/VA_" _rights "_VrmAssetList")) false))
          (Utilities|Array|AppendArray (LocalVariables|GetNewLocalVar_1) _outassetdata_2)
          (if (Utilities|Array|IsValidIndex _materials)
            (Utilities|IsValid _materialinterface
              (:Is%20Valid
                (bind _outassetdata_3 (Class|VrmBPFunctionLibrary|VRMGetAssetsbyPackageName (Utilities|String|StringToName (.LeftS (Utilities|String|Split (Class|KismetSystemLibrary|GetPathName _materialinterface) "." "IgnoreCase" "FromEnd"))) false))
                (Utilities|Array|AppendArray (LocalVariables|GetNewLocalVar_1) _outassetdata_3))
              (:Is%20Not%20Valid
                _)))
          (for _array_element (LocalVariables|GetNewLocalVar_1)
            (if (>= (Utilities|String|FindSubstring (Utilities|String|ToString(Name) (Class|VrmBPFunctionLibrary|VRMGetTopLevelAssetName _array_element)) "VrmAssetListObject") 0)
              (if (.bSuccess (Utilities|Casting|CastToVrmAssetListObject (Class|AssetRegistryHelpers|GetAsset _array_element)))
                (return (.AsVrm%20Asset%20List%20Object (Utilities|Casting|CastToVrmAssetListObject (Class|AssetRegistryHelpers|GetAsset _array_element))))))))))))