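; Actor that drives a target VRM avatar's head, hands and fingers from VrmHMDTracking headset and hand data.
; Each tick it remaps tracked transforms into avatar space and feeds ABP_VRoidSimple, plus a look-at target through the avatar's anim control component.
; Hands count as tracked only when away from the head; R recenters the tracking offset on the current head position.
; An optional debug mode draws hand bones as small cubes.
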(event EventBeginPlay)

(event Collision|EventActorBeginOverlap
  (params (OtherActor :type Actor%20Object%20Reference)))

(event EventTick
  (params (DeltaSeconds :type Float%20%28single-precision%29))
  (bind _vrmhmdtracking (Variables|Default|GetVrmHMDTracking))
  (Utilities|FlowControl|Sequence
    (:then_0
      (if (Variables|Default|GetbDebugHandVisible)
        ;[1 1 1] hand dummy model
        (Utilities|FlowControl|Sequence
          (:then_0
            (Utilities|Array|Resize (Variables|Default|GetleftH) (Utilities|Array|Length (Variables|/Script/VRM4U.VrmHMDTrackingComponent|GetleftHand _vrmhmdtracking)))
            (Utilities|Array|Resize (Variables|Default|GetRightH) (Utilities|Array|Length (Variables|/Script/VRM4U.VrmHMDTrackingComponent|GetrightHand _vrmhmdtracking))))
          (:then_1
            (for (_array_element _array_index) (Variables|/Script/VRM4U.VrmHMDTrackingComponent|GetleftHand (Variables|Default|GetVrmHMDTracking))
              (Utilities|IsValid (Utilities|Array|Get(acopy) (Variables|Default|GetleftH) _array_index)
                (:Is%20Valid
                  _)
                (:Is%20Not%20Valid
                  (bind _returnvalue (AddComponent|AddStaticMeshComponent false _array_element))
                  (Utilities|Array|SetArrayElem (Variables|Default|GetleftH) _array_index _returnvalue)
                  (Components|StaticMesh|SetStaticMesh _returnvalue "/Engine/BasicShapes/Cube.Cube")
                  (Development|SetHiddeninGame _returnvalue (not (Variables|Default|GetbDebugHandVisible)) false)))
              (Transformation|SetWorldTransform (Utilities|Array|Get(acopy) (Variables|Default|GetleftH) _array_index) (Math|Transform|MakeTransform (+ (.Location (Math|Transform|BreakTransform _array_element)) (.Location (Math|Transform|BreakTransform (Transformation|GetWorldTransform (Variables|Default|GetCube))))) (.Rotation (Math|Transform|BreakTransform _array_element)) (Math|Conversions|ToVector(Float) 0.02)) false false)))
          (:then_2
            (for (_array_element_2 _array_index_2) (Variables|/Script/VRM4U.VrmHMDTrackingComponent|GetrightHand (Variables|Default|GetVrmHMDTracking))
              (Utilities|IsValid (Utilities|Array|Get(acopy) (Variables|Default|GetRightH) _array_index_2)
                (:Is%20Valid
                  _)
                (:Is%20Not%20Valid
                  (bind _returnvalue_2 (AddComponent|AddStaticMeshComponent false _array_element_2))
                  (Utilities|Array|SetArrayElem (Variables|Default|GetRightH) _array_index_2 _returnvalue_2)
                  (Components|StaticMesh|SetStaticMesh _returnvalue_2 "/Engine/BasicShapes/Cube.Cube")
                  (Development|SetHiddeninGame _returnvalue_2 (not (Variables|Default|GetbDebugHandVisible)) false)))
              (Transformation|SetWorldTransform (Utilities|Array|Get(acopy) (Variables|Default|GetRightH) _array_index_2) (Math|Transform|MakeTransform (+ (.Location (Math|Transform|BreakTransform _array_element_2)) (.Location (Math|Transform|BreakTransform (Transformation|GetWorldTransform (Variables|Default|GetCube))))) (.Rotation (Math|Transform|BreakTransform _array_element_2)) (Math|Conversions|ToVector(Float) 0.02)) false false))))))
    (:then_1
      (CallFunction|UpdateTargetActor))))

(event Custom|updateTargetActor
  (bind _returnvalue (Math|Rotator|MakeRotator 0.0 0.0 9e+01))
  (bind _returnvalue_2 (Game|GetPlayerCameraManager 0))
  (bind _returnvalue_3 (Math|Rotator|MakeRotator 0.0 0.0 9e+01))
  (bind _self self)
  (bind _vrmhmdtracking (Variables|Default|GetVrmHMDTracking))
  (bind _targetactor (Variables|Default|GetTargetActor))
  (bind _vrmhmdtracking_2 (Variables|Default|GetVrmHMDTracking))
  (bind _targetactor_2 (Variables|Default|GetTargetActor))
  (bind _vrmhmdtracking_3 (Variables|Default|GetVrmHMDTracking))
  (bind _vrmhmdtracking_4 (Variables|Default|GetVrmHMDTracking))
  (bind _vrmhmdtracking_5 (Variables|Default|GetVrmHMDTracking))
  (bind _vrmhmdtracking_6 (Variables|Default|GetVrmHMDTracking))
  (bind _targetactor_3 (Variables|Default|GetTargetActor))
  (bind _trackingoffset (Variables|Default|GetTrackingOffset))
  (bind _returnvalue_4 (Transformation|GetActorLocation _self))
  (bind _returnvalue_5 (Transformation|GetActorTransform _returnvalue_2))
  (bind _skeletalmeshcomponent_dst (Variables|/VRM4U/Util/BaseCharacter/BP_VrmModelActor.BP_VrmModelActor_C|GetSkeletalMeshComponent_Dst _targetactor))
  (bind _skeletalmeshcomponent_dst_2 (Variables|/VRM4U/Util/BaseCharacter/BP_VrmModelActor.BP_VrmModelActor_C|GetSkeletalMeshComponent_Dst _targetactor_2))
  (bind _headpos (Variables|/Script/VRM4U.VrmHMDTrackingComponent|GetHeadPos _vrmhmdtracking_3))
  (bind _headpos_2 (Variables|/Script/VRM4U.VrmHMDTrackingComponent|GetHeadPos _vrmhmdtracking_2))
  (bind _headrot (Variables|/Script/VRM4U.VrmHMDTrackingComponent|GetHeadRot _vrmhmdtracking_3))
  (bind _headrot_2 (Variables|/Script/VRM4U.VrmHMDTrackingComponent|GetHeadRot _vrmhmdtracking_6))
  (bind _skeletalmeshcomponent_dst_3 (Variables|/VRM4U/Util/BaseCharacter/BP_VrmModelActor.BP_VrmModelActor_C|GetSkeletalMeshComponent_Dst _targetactor_3))
  (bind _returnvalue_6 (Transformation|GetWorldLocation _skeletalmeshcomponent_dst_3))
  (bind _returnvalue_7 (Transformation|GetWorldRotation _skeletalmeshcomponent_dst))
  (bind _location (Math|Transform|BreakTransform _returnvalue_5))
  (bind _returnvalue_8 (Math|Rotator|CombineRotators "-45.000000, 0,0.000000" _headrot_2))
  (bind _returnvalue_9 (Transformation|GetWorldRotation _skeletalmeshcomponent_dst_2))
  (bind _returnvalue_10 (+ _headpos _trackingoffset))
  (bind _returnvalue_11 (Math|Rotator|CombineRotators _returnvalue_7 _returnvalue))
  (bind _returnvalue_12 (Math|Transform|MakeTransform _location))
  (bind (_roll _pitch _yaw) (Math|Rotator|BreakRotator _returnvalue_8))
  (bind _returnvalue_13 (Math|Rotator|CombineRotators _returnvalue_9 _returnvalue_3))
  (bind _returnvalue_14 (Math|Vector|UnrotateVector _returnvalue_10 _headrot))
  (bind _returnvalue_15 (Math|Vector|GetForwardVector _returnvalue_11))
  (bind _returnvalue_16 (+ _returnvalue_14 "0, 0, 0"))
  (bind _returnvalue_17 (* _returnvalue_15 1e+01))
  (bind _returnvalue_18 (Math|Transform|TransformLocation _returnvalue_12 _returnvalue_16))
  (bind _returnvalue_19 (- _returnvalue_18 _returnvalue_4))
  (bind _returnvalue_20 (Math|Vector|RotateVector _returnvalue_19 _returnvalue_3))
  (bind _returnvalue_21 (* _returnvalue_20 "1.000000,1.000000, 0"))
  (bind (_x _y) (Math|Vector|BreakVector _returnvalue_21))
  (Variables|Default|GetTargetActor
    (:then
      (if (Class|VrmHMDTrackingComponent|IsEnable (Variables|Default|GetVrmHMDTracking))
        (Utilities|FlowControl|Sequence
          (:then_0
            (if (> (* (Utilities|Array|Length (Variables|/Script/VRM4U.VrmHMDTrackingComponent|GetleftHand _vrmhmdtracking_4)) (Utilities|Array|Length (Variables|/Script/VRM4U.VrmHMDTrackingComponent|GetrightHand _vrmhmdtracking_4))) 0)
              (Variables|Default|SetbLeftHandEnable (and (Variables|/Script/VRM4U.VrmHMDTrackingComponent|GetbEnableLeft (Variables|Default|GetVrmHMDTracking)) (> (Math|Vector|VectorLength (- (.Location (Math|Transform|BreakTransform (Utilities|Array|Get(acopy) (Variables|/Script/VRM4U.VrmHMDTrackingComponent|GetleftHand _vrmhmdtracking_2)))) _headpos_2)) 1e+01)))
              (Variables|Default|SetbRightHandEnable (and (> (Math|Vector|VectorLength (- (.Location (Math|Transform|BreakTransform (Utilities|Array|Get(acopy) (Variables|/Script/VRM4U.VrmHMDTrackingComponent|GetrightHand _vrmhmdtracking_2)))) _headpos_2)) 1e+01) (Variables|/Script/VRM4U.VrmHMDTrackingComponent|GetbEnableRight (Variables|Default|GetVrmHMDTracking))))))
          (:then_1
            (Utilities|FlowControl|Sequence
              (:then_0
                (Utilities|FlowControl|DoOnce false
                  (:Completed
                    (Input|EnableInput (Game|GetPlayerController 0)))))
              (:then_1
                (Variables|Default|SetTrackingOrign (+ (Transformation|GetWorldLocation (Variables|/VRM4U/Util/BaseCharacter/BP_VrmModelActor.BP_VrmModelActor_C|GetSkeletalMeshComponent_Dst (Variables|Default|GetTargetActor))) (Variables|Default|GetTrackingOffset)))
                (bind _asabp_vroid_simple (Utilities|Casting|CastToABP_VRoidSimple (Components|SkeletalMesh|GetAnimInstance (Variables|/VRM4U/Util/BaseCharacter/BP_VrmModelActor.BP_VrmModelActor_C|GetSkeletalMeshComponent_Src (Variables|Default|GetTargetActor)))))
                (bind _output_get (Variables|Default|SetABP_Simple _asabp_vroid_simple))
                (Variables|/VRM4U/Util/BaseCharacter/Mesh/ABP_VRoidSimple.ABP_VRoidSimple_C|SetisTrackHead _output_get true)
                (Variables|/VRM4U/Util/BaseCharacter/Mesh/ABP_VRoidSimple.ABP_VRoidSimple_C|SetisTrackLeftHand _output_get true)
                (Variables|/VRM4U/Util/BaseCharacter/Mesh/ABP_VRoidSimple.ABP_VRoidSimple_C|SetisTrackRightHand _output_get true)
                (Variables|/VRM4U/Util/BaseCharacter/Mesh/ABP_VRoidSimple.ABP_VRoidSimple_C|SetisFingerTrack _output_get true))
              (:then_3
                (Utilities|FlowControl|Sequence
                  (:then_0
                    ;[1 1 1] 手 顔相対
                    (Utilities|FlowControl|Sequence
                      (:then_0
                        (if (Variables|Default|GetbLeftHandEnable)
                          (bind _output_get_2 (Variables|Default|SetLeftHandTrans (Variables|/Script/VRM4U.VrmHMDTrackingComponent|GetleftHand _vrmhmdtracking)))
                          (for (_array_element _array_index) _output_get_2
                            (Utilities|Array|SetArrayElem _output_get_2 _array_index (Math|Transform|MakeTransform (+ (Math|Vector|RotateVector (+ (.Location (Math|Transform|BreakTransform _array_element)) (Variables|Default|GetTrackingOffset)) _returnvalue_11) _returnvalue_6 "0,0,150.000000" _returnvalue_17) (Math|Rotator|CombineRotators (.Rotation (Math|Transform|BreakTransform _array_element)) _returnvalue_11))))))
                      (:then_1
                        (if (Variables|Default|GetbRightHandEnable)
                          (bind _output_get_3 (Variables|Default|SetRightHandTrans (Variables|/Script/VRM4U.VrmHMDTrackingComponent|GetrightHand _vrmhmdtracking)))
                          (for (_array_element_2 _array_index_2) _output_get_3
                            (Utilities|Array|SetArrayElem _output_get_3 _array_index_2 (Math|Transform|MakeTransform (+ (Math|Vector|RotateVector (+ (.Location (Math|Transform|BreakTransform _array_element_2)) (Variables|Default|GetTrackingOffset)) _returnvalue_11) _returnvalue_6 "0,0,150.000000" _returnvalue_17) (Math|Rotator|CombineRotators (.Rotation (Math|Transform|BreakTransform _array_element_2)) _returnvalue_11))))))))
                  (:then_2
                    ;[1 1 1] 顔向き
                    (CallFunction|SetLookatTarget (Math|Vector|Lerp(Vector) (+ (Variables|Default|GetTrackingOrign) (Math|Vector|RotateVector (Math|Vector|MakeVector 1e+02 0.0 0.0) _returnvalue_13) "0,0,150.000000") (+ (Variables|Default|GetTrackingOrign) (Math|Vector|RotateVector (- (Math|Transform|TransformLocation _returnvalue_12 (+ _returnvalue_14 "100.000000, 0, 0")) _returnvalue_4) _returnvalue_13) "0,0,150.000000") 5.0))
                    (CallFunction|SetLookatForce 1.0)
                    (Variables|/VRM4U/Util/BaseCharacter/Mesh/ABP_VRoidSimple.ABP_VRoidSimple_C|Sethead_relative (Variables|Default|GetABP_Simple) (Math|Transform|MakeTransform (* (Math|Vector|MakeVector _x _y 0.0) 0.5))))))
              (:then_4
                (Utilities|FlowControl|Sequence
                  (:then_0
                    ;[1 1 1] 手　適用
                    (Utilities|FlowControl|Sequence
                      (:then_0
                        (if (Variables|Default|GetbLeftHandEnable)
                          (Variables|/VRM4U/Util/BaseCharacter/Mesh/ABP_VRoidSimple.ABP_VRoidSimple_C|Sethand_pos_l (Variables|Default|GetABP_Simple) (.Location (Math|Transform|BreakTransform (Utilities|Array|Get(acopy) (Variables|Default|GetLeftHandTrans)))))
                          (Variables|/VRM4U/Util/BaseCharacter/Mesh/ABP_VRoidSimple.ABP_VRoidSimple_C|Sethand_rot_l (Variables|Default|GetABP_Simple) (Math|Rotator|CombineRotators "0.000000,90.000000,180.000000" (.Rotation (Math|Transform|BreakTransform (Utilities|Array|Get(acopy) (Variables|Default|GetLeftHandTrans))))))))
                      (:then_1
                        (if (Variables|Default|GetbRightHandEnable)
                          (Variables|/VRM4U/Util/BaseCharacter/Mesh/ABP_VRoidSimple.ABP_VRoidSimple_C|Sethand_pos_r (Variables|Default|GetABP_Simple) (.Location (Math|Transform|BreakTransform (Utilities|Array|Get(acopy) (Variables|Default|GetRightHandTrans)))))
                          (Variables|/VRM4U/Util/BaseCharacter/Mesh/ABP_VRoidSimple.ABP_VRoidSimple_C|Sethand_rot_r (Variables|Default|GetABP_Simple) (Math|Rotator|CombineRotators "0.000000,90.000000,0.000000" (.Rotation (Math|Transform|BreakTransform (Utilities|Array|Get(acopy) (Variables|Default|GetRightHandTrans))))))))))
                  (:then_2
                    (Variables|/VRM4U/Util/BaseCharacter/Mesh/ABP_VRoidSimple.ABP_VRoidSimple_C|SetHandTransformCurrent (Variables|Default|GetABP_Simple) (Utilities|Struct|MakeVRMQuestHandBone (Variables|Default|GetLeftHandTrans) (Variables|Default|GetRightHandTrans)))
                    (Variables|/VRM4U/Util/BaseCharacter/Mesh/ABP_VRoidSimple.ABP_VRoidSimple_C|SetHandTransformReference (Variables|Default|GetABP_Simple) (Utilities|Struct|MakeVRMQuestHandBone (Variables|/Script/VRM4U.VrmHMDTrackingComponent|GetleftHandReference _vrmhmdtracking_5) (Variables|/Script/VRM4U.VrmHMDTrackingComponent|GetrightHandReference _vrmhmdtracking_5))))
                  (:then_3
                    ;[1 1 1] 頭回転
                    ;;[1 1 1] head
                    (Utilities|FlowControl|Sequence
                      (:then_0
                        (Variables|/VRM4U/Util/BaseCharacter/Mesh/ABP_VRoidSimple.ABP_VRoidSimple_C|Sethead_rot (Variables|Default|GetABP_Simple) (Math|Rotator|CombineRotators (Transformation|GetWorldRotation (Variables|/VRM4U/Util/BaseCharacter/BP_VrmModelActor.BP_VrmModelActor_C|GetSkeletalMeshComponent_Dst (Variables|Default|GetTargetActor))) (Math|Rotator|MakeRotator (* _roll -1.0) (* _pitch -1.0) _yaw)))))))))))))
    (:else)))

(event Custom|SetLookAtTarget
  (params (TargetLocation :type Vector))
  (Default|SetLookatTarget (Variables|/VRM4U/Util/BaseCharacter/BP_VrmModelActor.BP_VrmModelActor_C|GetBP_VrmAnimControlComponent (Variables|Default|GetTargetActor)) TargetLocation))

(event Custom|SetLookAtForce
  (params (LookAtForce :type Float%20%28single-precision%29))
  (Default|SetLookatForce (Variables|/VRM4U/Util/BaseCharacter/BP_VrmModelActor.BP_VrmModelActor_C|GetBP_VrmAnimControlComponent (Variables|Default|GetTargetActor)) LookAtForce))

(event Custom|SetLookAtType
  (params (Eye :type Boolean) (Head :type Boolean))
  (Default|SetLookatType (Variables|/VRM4U/Util/BaseCharacter/BP_VrmModelActor.BP_VrmModelActor_C|GetBP_VrmAnimControlComponent (Variables|Default|GetTargetActor)) Eye Head))

(event Input|KeyboardEvents|R
  (params (Key :type Key%20Structure))
  (:Pressed
    (Variables|Default|SetTrackingOffset (* (Variables|/Script/VRM4U.VrmHMDTrackingComponent|GetHeadPos (Variables|Default|GetVrmHMDTracking)) -1.0))))

(fn ConstructionScript)