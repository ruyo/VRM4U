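; Placeable look-at point actor that steers the eye and head gaze of a VRM character.
; While enabled, Tick feeds its own location or the camera's, plus look type and force, to the TargetActor character or BPVrmUtilComponent's model.
; LookAtLocal instead aims at an up/down, left/right offset from the neck socket.
; Construction binds the target and refreshes animation; helpers compute a head-offset-corrected point and upper-chest rate.
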(event Custom|LookAtLocal
  (params (UpDown :type Float%20%28single-precision%29) (LeftRight :type Float%20%28single-precision%29))
  (bind _bheadenable (Variables|Default|GetbHeadEnable))
  (if (not (Variables|Default|GetbIgnore))
    (bind _targetactor (Variables|Default|GetTargetActor)
      (:then
        (bind _asbp_vrm_character_base (Utilities|Casting|CastToBP_VrmCharacterBase _targetactor)
          (:then
            (Default|SetLookatType _asbp_vrm_character_base true _bheadenable)
            (Default|SetLookatTarget _asbp_vrm_character_base (Math|Transform|TransformLocation (Transformation|GetSocketTransform (Variables|/Script/Engine.Character|GetMesh _asbp_vrm_character_base) "J_Bip_C_Neck" "RTS_World") (Math|Vector|MakeVector (* LeftRight -1e+02) 0.0 (* UpDown 1e+02)))))
          (:CastFailed
            (bind _vrmmodelactor (Variables|/VRM4U/Util/Actor/Misc/sub/BP_VrmUtilComponent.BP_VrmUtilComponent_C|GetVrmModelActor (Variables|Default|GetBP_VrmUtilComponent))
              (:then
                (Default|SetLookatType _vrmmodelactor true _bheadenable)
                (Default|SetLookatTarget _vrmmodelactor (Math|Transform|TransformLocation (Transformation|GetSocketTransform (Variables|/Script/Engine.Character|GetMesh _asbp_vrm_character_base) "J_Bip_C_Neck" "RTS_World") (Math|Vector|MakeVector (* LeftRight -1e+02) 0.0 (* UpDown 1e+02)))))
              (:else)))))
      (:else))))

(event Custom|CustomEvent_0
  (Utilities|FlowControl|Sequence
    (:then_1
      (bind _vrmmodelactor (Variables|/VRM4U/Util/Actor/Misc/sub/BP_VrmUtilComponent.BP_VrmUtilComponent_C|GetVrmModelActor (Variables|Default|GetBP_VrmUtilComponent))
        (:then
          (Class|VrmBPFunctionLibrary|VRMInitAnim (Variables|/VRM4U/Util/BaseCharacter/BP_VrmModelActor.BP_VrmModelActor_C|GetSkeletalMeshComponent_Src _vrmmodelactor))
          (bind _attachmodeactor (Variables|/VRM4U/Util/BaseCharacter/BP_VrmModelActor.BP_VrmModelActor_C|GetAttachModeActor _vrmmodelactor)
            (:then
              (Default|UpdatePose _attachmodeactor))
            (:else)))
        (:else)))))

(event EventBeginPlay
  (bind _outactors (Actor|GetAllActorsOfClass "/VRM4U/Util/Actor/CharacterCamera.CharacterCamera_C")))

(event Collision|EventActorBeginOverlap
  (params (OtherActor :type Actor%20Object%20Reference)))

(event EventTick
  (params (DeltaSeconds :type Float%20%28single-precision%29))
  (bind _transform (Class|VrmBPFunctionLibrary|VRMGetCameraTransform 0 false))
  (bind _returnvalue (Transformation|GetActorLocation))
  (bind _beyeenable (Variables|Default|GetbEyeEnable))
  (bind _busecameraposition (Variables|Default|GetbUseCameraPosition))
  (bind _lookatforce (Variables|Default|GetLookAtForce))
  (bind _bheadenable (Variables|Default|GetbHeadEnable))
  (bind _location (Math|Transform|BreakTransform _transform))
  (bind _returnvalue_2 (select _busecameraposition _location _returnvalue))
  (if (not (Variables|Default|GetbIgnore))
    (if (Variables|Default|GetbEyeEnable)
      (Utilities|FlowControl|Sequence
        (:then_0
          _)
        (:then_1
          (goto _label Reset)))
      (else
        (Utilities|FlowControl|DoOnce false :!label _label
          (:Completed
            (Utilities|FlowControl|Sequence
              (:then_0
                _))))))
    (bind _targetactor (Variables|Default|GetTargetActor)
      (:then
        (bind _asbp_vrm_character_base (Utilities|Casting|CastToBP_VrmCharacterBase _targetactor)
          (:then
            (Default|SetLookatTarget _asbp_vrm_character_base _returnvalue_2)
            (Default|SetLookatType _asbp_vrm_character_base _beyeenable _bheadenable)
            (Default|SetLookatForce (Variables|/VRM4U/Util/BaseCharacter/BP_VrmCharacterBase.BP_VrmCharacterBase_C|GetBP_VrmAnimControlComponent _asbp_vrm_character_base) _lookatforce))
          (:CastFailed
            (bind _vrmmodelactor (Variables|/VRM4U/Util/Actor/Misc/sub/BP_VrmUtilComponent.BP_VrmUtilComponent_C|GetVrmModelActor (Variables|Default|GetBP_VrmUtilComponent))
              (:then
                (Default|SetLookatTarget _vrmmodelactor _returnvalue_2)
                (Default|SetLookatType _vrmmodelactor _beyeenable _bheadenable)
                (Default|SetLookatForce (Variables|/VRM4U/Util/BaseCharacter/BP_VrmModelActor.BP_VrmModelActor_C|GetBP_VrmAnimControlComponent _vrmmodelactor) _lookatforce))
              (:else)))))
      (:else))))

(fn ConstructionScript
  (Default|SetActor (Variables|Default|GetBP_VrmUtilComponent) (Variables|Default|GetTargetActor))
  (CallFunction|CustomEvent0))

(fn GetLookatPoint
  (bind _bp_vrmutilcomponent (Variables|Default|GetBP_VrmUtilComponent))
  (bind _vrmmodelactor (Variables|/VRM4U/Util/Actor/Misc/sub/BP_VrmUtilComponent.BP_VrmUtilComponent_C|GetVrmModelActor _bp_vrmutilcomponent))
  (return (+ (select (Variables|Default|GetbUseCameraPosition) (.Location (Math|Transform|BreakTransform (.transform (Class|VrmBPFunctionLibrary|VRMGetCameraTransform 0 false)))) (Transformation|GetActorLocation)) (- (.Location (Math|Transform|BreakTransform (Transformation|GetSocketTransform (Variables|/VRM4U/Util/BaseCharacter/BP_VrmModelActor.BP_VrmModelActor_C|GetSkeletalMeshComponent_Src _vrmmodelactor) "J_Bip_C_Head" "RTS_World"))) (.Location (Math|Transform|BreakTransform (Transformation|GetSocketTransform (Variables|/VRM4U/Util/BaseCharacter/BP_VrmModelActor.BP_VrmModelActor_C|GetSkeletalMeshComponent_Dst _vrmmodelactor) (Utilities|String|StringToName (.Value (Utilities|Map|Find (Variables|/Script/VRM4U.VrmMetaObject|GethumanoidBoneTable (Variables|/Script/VRM4U.VrmAssetListObject|GetVrmMetaObject (Variables|/VRM4U/Util/BaseCharacter/BP_VrmModelActor.BP_VrmModelActor_C|GetVrmAssetList _vrmmodelactor))) "head"))) "RTS_World")))))))

(fn GetUpperChestRate
  (Utilities|FlowControl|Sequence
    (:then_0
      (LocalVariables|SetNewLocalVar_0 1.0))
    (:then_1
      (bind _vrmassetlist (Variables|/VRM4U/Util/BaseCharacter/BP_VrmModelActor.BP_VrmModelActor_C|GetVrmAssetList (Variables|/VRM4U/Util/Actor/Misc/sub/BP_VrmUtilComponent.BP_VrmUtilComponent_C|GetVrmModelActor (Variables|Default|GetBP_VrmUtilComponent)))
        (:then
          (Utilities|FlowControl|Sequence
            (:then_0
              (if (.ReturnValue (Utilities|Map|Find (Variables|/Script/VRM4U.VrmMetaObject|GethumanoidBoneTable (Variables|/Script/VRM4U.VrmAssetListObject|GetVrmMetaObject _vrmassetlist)) "upperChest"))
                (if (Utilities|Enum|Equal(Enum) (.Value (Utilities|Map|Find (Variables|/Script/VRM4U.VrmMetaObject|GethumanoidBoneTable (Variables|/Script/VRM4U.VrmAssetListObject|GetVrmMetaObject _vrmassetlist)) "upperChest")) "")
                  ;[1 1 1] stop UpperChest
                  (LocalVariables|SetNewLocalVar_0 0.0 :!label _label))
                (else
                  (goto _label))))))
        (:else)))
    (:then_2
      (return (LocalVariables|GetNewLocalVar_0)))))