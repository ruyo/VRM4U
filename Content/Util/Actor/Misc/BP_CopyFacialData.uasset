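; Actor that drives facial morph targets on a target skeletal mesh every tick for brows, blinking and lip sync.
; Brow and blink values come from ARKit-style animation curves on MeshKiteBoy, written to both Face and blendShape morph names.
; Viseme weights are thresholded into five A/I/U/E/O mouth targets, smoothed by lerping current toward reference weights.
; The curve-driven mouth branches are disconnected and never run.
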(event EventBeginPlay)

(event Collision|EventActorBeginOverlap
  (params (OtherActor :type Actor%20Object%20Reference)))

(event EventTick
  (params (DeltaSeconds :type Float%20%28single-precision%29))
  (bind _array (Utilities|Array|MakeArray "blendShape.A" "blendShape.I" "blendShape.U" "blendShape.E" "blendShape.O"))
  (bind _weight_cur (Variables|Default|Getweight_cur))
  (bind _targetactor (Variables|Default|GetTargetActor))
  (bind _mesh_kite_boy (Variables|Default|GetMesh_kite_boy))
  (bind _weight_ref (Variables|Default|Getweight_ref))
  (bind _returnvalue (Actor|GetComponentbyClass _mesh_kite_boy "/Script/Engine.SkeletalMeshComponent"))
  (bind _skeletalmeshcomponent_dst (Variables|/VRM4U/Util/BaseCharacter/BP_VrmModelActor.BP_VrmModelActor_C|GetSkeletalMeshComponent_Dst _targetactor))
  (bind _returnvalue_2 (Components|SkeletalMesh|GetAnimInstance _returnvalue))
  (bind _returnvalue_3 (Animation|Curves|GetCurveValue _returnvalue_2 "eyeBlinkLeft"))
  (bind _returnvalue_4 (Animation|Curves|GetCurveValue _returnvalue_2 "eyeBlinkRight"))
  (Utilities|FlowControl|Sequence
    (:then_0
      (Variables|Default|GetMesh_kite_boy
        (:then
          (Utilities|FlowControl|Sequence
            (:then_0
              ;[1 1 1] 眉
              (Components|SkeletalMesh|SetMorphTarget _skeletalmeshcomponent_dst "Face.M_F00_000_00_Fcl_BRW_Fun" (Animation|Curves|GetCurveValue _returnvalue_2 "browOuterUpLeft") true))
            (:then_1
              ;[1 1 1] 目
              (Components|SkeletalMesh|SetMorphTarget _skeletalmeshcomponent_dst "Face.M_F00_000_00_Fcl_EYE_Close_R" _returnvalue_4 false)
              (Components|SkeletalMesh|SetMorphTarget _skeletalmeshcomponent_dst "Face.M_F00_000_00_Fcl_EYE_Close_L" _returnvalue_3 false))
            (:then_2
              (Components|SkeletalMesh|SetMorphTarget _skeletalmeshcomponent_dst "blendShape.BLINK_R" _returnvalue_4 false)
              (Components|SkeletalMesh|SetMorphTarget _skeletalmeshcomponent_dst "blendShape.BLINK_L" _returnvalue_3 false))))
        (:else)))
    (:then_1
      (for _array_element _array
        ;[1 1 1] 初期化
        (Components|SkeletalMesh|SetMorphTarget (Variables|/VRM4U/Util/BaseCharacter/BP_VrmModelActor.BP_VrmModelActor_C|GetSkeletalMeshComponent_Dst (Variables|Default|GetTargetActor)) (Utilities|String|StringToName _array_element) 0.0 false)))
    (:then_3
      (for (_array_element_2 _array_index) (Variables|Default|Getvisemes_name_dummy)
        (Utilities|FlowControl|Sequence
          (:then_1
            (for (_array_element_3 _array_index_2) (Utilities|Array|MakeArray "aa" "ih" "PP" "E" "oh" "nn")
              (if (Utilities|Enum|Equal(Enum) _array_element_2 _array_element_3)
                (if (> (Utilities|Array|Get(acopy) (Variables|Default|Getvisemes_dummy) _array_index) 0.1)
                  ;[1 1 1] リップシンク決定
                  (Utilities|Array|SetArrayElem _weight_ref (Math|Integer|Clamp(Integer) _array_index_2 0 4) 0.5)
                  (else
                    (Utilities|Array|SetArrayElem _weight_ref (Math|Integer|Clamp(Integer) _array_index_2 0 4) 0.0)))))))))
    (:then_4
      (for (_array_element_4 _array_index_3) _array
        ;[1 1 1] リップシンク適用
        (Components|SkeletalMesh|SetMorphTarget (Variables|/VRM4U/Util/BaseCharacter/BP_VrmModelActor.BP_VrmModelActor_C|GetSkeletalMeshComponent_Dst (Variables|Default|GetTargetActor)) (Utilities|String|StringToName _array_element_4) (Utilities|Array|Get(acopy) (Variables|Default|Getweight_cur) _array_index_3) true)
        (if (> (Utilities|Array|Get(acopy) (Variables|Default|Getweight_cur) _array_index_3) 0.4)
          _)))
    (:then_5
      ;[1 1 1] リップシンク補完
      (for (_array_element_5 _array_index_4) _weight_cur
        (Utilities|Array|SetArrayElem _weight_cur _array_index_4 (Math|Float|Lerp _array_element_5 (Utilities|Array|Get(acopy) (Variables|Default|Getweight_ref) _array_index_4) 0.8))))))

(fn ConstructionScript
  (Utilities|Array|Resize (Variables|Default|Getweight_cur) 5)
  (Utilities|Array|Resize (Variables|Default|Getweight_ref) 5))