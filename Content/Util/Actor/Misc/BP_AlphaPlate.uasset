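; BP_AlphaPlate is a utility actor that displays a plane with configurable color, alpha scale and camera offset.
; Its construction script creates a dynamic material instance on the plane and passes those settings to it as parameters.
; It then attaches itself to an optional TargetActor, keeping its world transform.
; When Ignore is set, it destroys the plane and skips all setup.
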(fn ConstructionScript
  (if (Variables|Default|GetbIgnore)
    (Components|DestroyComponent (Variables|Default|GetPlane))
    (else
      (Utilities|FlowControl|Sequence
        (:then_0
          (bind _returnvalue (Rendering|Material|CreateDynamicMaterialInstance (Variables|Default|GetPlane) 0 0 "None" :!class /Script/Engine.PrimitiveComponent))
          (bind _output_get (Variables|Default|SetNewVar_0 _returnvalue))
          (Rendering|Material|SetVectorParameterValue _output_get "Color" (Variables|Default|GetColor) :!class /Script/Engine.MaterialInstanceDynamic)
          (Rendering|Material|SetScalarParameterValue _output_get "AlphaScale" (Variables|Default|GetAlphaScale) :!class /Script/Engine.MaterialInstanceDynamic)
          (Rendering|Material|SetScalarParameterValue _output_get "CameraOffset" (Variables|Default|GetCameraOffset) :!class /Script/Engine.MaterialInstanceDynamic))
        (:then_1
          (bind _targetactor (Variables|Default|GetTargetActor)
            (:then
              (Transformation|AttachActorToActor _targetactor "None" "KeepWorld" "KeepWorld" "KeepWorld" true))
            (:else)))))))