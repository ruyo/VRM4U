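; Utility actor that makes the game window transparent through VRM's color-key window function, with a color-only mode that applies just the effect.
; On init it marks visible primitives of MaskActorList actors in custom depth stencil and builds an unbound post-process from M_WindowTransparent using CrKey.
; T cycles transparent, off, color-only, off, toggling the post-process and warning to use New Editor Window play when the window call fails.
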(event Custom|init
  (Utilities|FlowControl|Sequence
    (:then_0
      (for _array_element (Variables|Default|GetMaskActorList)
        (Utilities|FlowControl|Sequence
          (:then_0
            (for _array_element_2 (Actor|GetComponentsByClass _array_element "/Script/Engine.PrimitiveComponent")
              (if (Rendering|IsVisible _array_element_2)
                (if (not (Variables|/Script/Engine.PrimitiveComponent|GetbRenderCustomDepth _array_element_2))
                  (if (== (Variables|/Script/Engine.PrimitiveComponent|GetCustomDepthStencilValue _array_element_2) 0)
                    (Rendering|SetRenderCustomDepth _array_element_2 true)
                    (Rendering|SetCustomDepthStencilValue _array_element_2 1)))))))))
    (:then_1
      (bind _returnvalue (Rendering|Material|CreateDynamicMaterialInstance "/VRM4U/Util/Actor/Misc/sub/M_WindowTransparent.M_WindowTransparent" "None" :!class /Script/Engine.KismetMaterialLibrary))
      (Utilities|Struct|SetmembersinPostProcessSettings (Variables|/Script/Engine.PostProcessComponent|GetSettings (Variables|Default|GetPostProcess)) (Utilities|Struct|MakeWeightedBlendables (Utilities|Array|MakeArray (Utilities|Struct|MakeWeightedBlendable 1.0 _returnvalue))))
      (Rendering|Material|SetVectorParameterValue _returnvalue "crKey" (Variables|Default|GetcrKey) :!class /Script/Engine.MaterialInstanceDynamic))))

(event Custom|SetTransparentWindow
  (params (bEnable :type Boolean) (ColorOnly :type Boolean))
  (Utilities|FlowControl|Sequence
    (:then_0
      (if bEnable
        (bind _returnvalue (Class|VrmBPFunctionLibrary|VRMSetTransparentWindow (not ColorOnly) (Variables|Default|GetcrKey)))
        (Variables|Default|SetNewVar_0 _returnvalue)
        (else
          (bind _returnvalue_2 (Class|VrmBPFunctionLibrary|VRMSetTransparentWindow false))
          (Variables|Default|SetNewVar_0 _returnvalue_2))))
    (:then_1
      (Variables|/Script/Engine.PostProcessComponent|SetbEnabled (Variables|Default|GetPostProcess) bEnable))))

(event EventBeginPlay
  (Input|EnableInput (Game|GetPlayerController 0))
  (Utilities|FlowControl|Sequence
    (:then_0
      (for _array_element (Variables|Default|GetMaskActorList)
        (Utilities|FlowControl|Sequence
          (:then_0
            (for _array_element_2 (Actor|GetComponentsByClass _array_element "/Script/Engine.PrimitiveComponent")
              (if (Rendering|IsVisible _array_element_2)
                (if (not (Variables|/Script/Engine.PrimitiveComponent|GetbRenderCustomDepth _array_element_2))
                  (if (== (Variables|/Script/Engine.PrimitiveComponent|GetCustomDepthStencilValue _array_element_2) 0)
                    (Rendering|SetRenderCustomDepth _array_element_2 true)
                    (Rendering|SetCustomDepthStencilValue _array_element_2 1)))))))))
    (:then_1
      (bind _returnvalue (Rendering|Material|CreateDynamicMaterialInstance "/VRM4U/Util/Actor/Misc/sub/M_WindowTransparent.M_WindowTransparent" "None" :!class /Script/Engine.KismetMaterialLibrary))
      (Utilities|Struct|SetmembersinPostProcessSettings (Variables|/Script/Engine.PostProcessComponent|GetSettings (Variables|Default|GetPostProcess)) (Utilities|Struct|MakeWeightedBlendables (Utilities|Array|MakeArray (Utilities|Struct|MakeWeightedBlendable 1.0 _returnvalue))))
      (Rendering|Material|SetVectorParameterValue _returnvalue "crKey" (Variables|Default|GetcrKey) :!class /Script/Engine.MaterialInstanceDynamic))))

(event Collision|EventActorBeginOverlap
  (params (OtherActor :type Actor%20Object%20Reference)))

(event EventTick
  (params (DeltaSeconds :type Float%20%28single-precision%29)))

(event Input|KeyboardEvents|T
  (params (Key :type Key%20Structure))
  (:Pressed
    (Utilities|FlowControl|Sequence
      (:then_0
        (bind _isa (Utilities|FlowControl|FlipFlop)
          (:A
            (bind _isa_2 (Utilities|FlowControl|FlipFlop)))))
      (:then_1
        (CallFunction|SetTransparentWindow _isa (not _isa_2))
        (if (not (Variables|Default|GetNewVar_0))
          (Development|PrintString "!!Warning!! 
Use 'Play in 'NewEditorWindow' mode for transparent"))))))

(fn ConstructionScript
  (bind _postprocess (Variables|Default|GetPostProcess))
  (Variables|/Script/Engine.PostProcessComponent|SetbEnabled _postprocess false)
  (Variables|/Script/Engine.PostProcessComponent|SetbUnbound _postprocess true)
  (if (.bPlay (Class|VrmBPFunctionLibrary|VRMGetPlayMode))
    (CallFunction|Init)))