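; Utility actor that relays VRM editor global time changes and refreshes the MToon material system's camera, apparently for use in the editor.
; BeginBind clears and rebinds the VrmEditorEvent time-change delegate, then turns global time checking off.
; A custom event forwards the current time through OnGlobalTimeChange.
; EditorTickChecker finds the first MToonMaterialSystem actor and calls UpdateCamera, while EditorTickEvent reuses that lookup, skipping the validity check.
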(event Custom|CustomEvent_0
  (params (CurrentTime :type Float%20%28single-precision%29))
  (Default|CallOnGlobalTimeChange CurrentTime))

(event Custom|BeginBind
  (bind _vrmeditorevent (Variables|Default|GetVrmEditorEvent))
  (EventDispatchers|UnbindallEventsfromOnGlobalTimeChange _vrmeditorevent)
  (EventDispatchers|BindEventtoOnGlobalTimeChange _vrmeditorevent (EventDispatchers|CreateEvent :!event Custom|CustomEvent_0))
  (Class|VrmEditorEventComponent|SetGlobalTimeCheck _vrmeditorevent false))

(event Custom|EditorTickChecker
  (bind _outactors (Actor|GetAllActorsOfClass "/VRM4U/Util/Actor/MToonMaterialSystem.MToonMaterialSystem_C"))
  (if (Utilities|Array|IsValidIndex _outactors)
    (Default|UpdateCamera (Utilities|Array|Get(acopy) _outactors))))

(event Custom|EditorTickEvent
  (Default|UpdateCamera (Utilities|Array|Get(acopy) (stale Custom|EditorTickChecker _outactors))))

(event EventBeginPlay)

(event Collision|EventActorBeginOverlap
  (params (OtherActor :type Actor%20Object%20Reference)))

(event EventTick
  (params (DeltaSeconds :type Float%20%28single-precision%29)))

(fn ConstructionScript)