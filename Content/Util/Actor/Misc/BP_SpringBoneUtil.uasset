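; BP_SpringBoneUtil is a utility actor that generates VRM spring bone settings into a duplicated TargetMeta, warning if it is the original.
; Construction binds VrmUtilComponent to the target actor's mesh.
; GenerateSpringParam rebuilds limb colliders as sphere rows interpolated toward each child bone, with axis and unit conversion.
; It then builds springs from SpringParamSet and bone-to-param maps, linking every collider and optionally creating tail bones.
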(event Custom|GenerateSpringParam
  (bind _returnvalue (Class|KismetSystemLibrary|MakeLiteralInteger 5))
  (bind _bone_to_springparamaddtail (Variables|Default|GetBone_To_SpringParamAddTail))
  (bind _targetmeta (Variables|Default|GetTargetMeta))
  (bind _humanoidcollistionbonelist (Variables|Default|GetHumanoidCollistionBoneList))
  (bind _humanoidcollistionbonelist_2 (Variables|Default|GetHumanoidCollistionBoneList))
  (bind _collisioninexlist_all_ (Variables|Tmp|GetCollisionInexList%28all%29))
  (bind _collistiongroup (Variables|Tmp|GetcollistionGroup))
  (bind _bone_childall (Variables|Tmp|Getbone_childAll))
  (bind _vrmutilcomponent (Variables|Default|GetVrmUtilComponent))
  (bind _bone_to_springparam (Variables|Default|GetBone_To_SpringParam))
  (bind _vrmcollidermeta (Variables|/Script/VRM4U.VrmMetaObject|GetVRMColliderMeta _targetmeta))
  ;[1 1 1] Generate Check
  (Variables|Default|GetTargetActor
    (:then
      (bind _targetmeta_2 (Variables|Default|GetTargetMeta)
        (:then
          (Utilities|FlowControl|Sequence
            (:then_0
              (Default|SetVRMAssetListfromMeshComponent _vrmutilcomponent (Variables|/Script/VRM4U.VrmMetaObject|GetSkeletalMesh _targetmeta_2))
              (Default|SetTargetMeshComponent _vrmutilcomponent (Variables|/Script/Engine.SkeletalMeshActor|GetSkeletalMeshComponent (Variables|Default|GetTargetActor)))
              (bind _vrmassetlist (Variables|/VRM4U/Util/Actor/Misc/sub/BP_VrmUtilComponent.BP_VrmUtilComponent_C|GetVrmAssetList _vrmutilcomponent)
                (:then
                  (if (== (Variables|Default|GetTargetMeta) (Variables|/Script/VRM4U.VrmAssetListObject|GetVrmMetaObject _vrmassetlist))
                    (Development|PrintString "Warning! 
Please duplicate VrmMeta and change params!!")
                    (else
                      (Utilities|FlowControl|Sequence
                        (:then_0
                          ;[1 1 1] Body collision
                          (Utilities|FlowControl|Sequence
                            (:then_0
                              (Utilities|Array|Clear (Variables|Default|GetHumanoidCollistionBoneList))
                              (Utilities|Array|Clear (Variables|/Script/VRM4U.VrmMetaObject|GetVRMColliderMeta (Variables|Default|GetTargetMeta))))
                            (:then_1
                              (Utilities|Array|AppendArray _humanoidcollistionbonelist_2 (Utilities|Array|MakeArray "leftUpperArm" "leftLowerArm" "leftHand" ""))
                              (Utilities|Array|AppendArray _humanoidcollistionbonelist_2 (Utilities|Array|MakeArray "rightUpperArm" "rightLowerArm" "rightHand" ""))
                              (Utilities|Array|AppendArray _humanoidcollistionbonelist_2 (Utilities|Array|MakeArray "leftUpperLeg" "leftLowerLeg" "leftFoot" ""))
                              (Utilities|Array|AppendArray _humanoidcollistionbonelist_2 (Utilities|Array|MakeArray "rightUpperLeg" "rightLowerLeg" "rightFoot" "")))
                            (:then_3
                              (for _index (range 0 (- (Utilities|Array|Length (Variables|Default|GetHumanoidCollistionBoneList)) 1))
                                (if (not (or (Utilities|Enum|Equal(Enum) (Utilities|Array|Get(acopy) _humanoidcollistionbonelist _index) "") (Utilities|Enum|Equal(Enum) (Utilities|Array|Get(acopy) _humanoidcollistionbonelist (+ _index 1)) "")))
                                  (Utilities|Array|Add (Variables|/Script/VRM4U.VrmMetaObject|GetVRMColliderMeta (Variables|Default|GetTargetMeta)) (Utilities|Struct|MakeVRMColliderMeta 0 "" (Utilities|Array|MakeArray "")))
                                  (Utilities|FlowControl|Sequence
                                    (:then_0
                                      (Utilities|Array|Clear _collistiongroup)
                                      (Utilities|Array|Resize _collistiongroup _returnvalue)
                                      (for (_ _array_index) _collistiongroup
                                        (Utilities|Array|SetArrayElem _collistiongroup _array_index (Utilities|Struct|MakeVRMSpringColliderData (Math|Vector|MakeVector (* (.X (Math|Vector|BreakVector (/ (Math|Vector|Lerp(Vector) (Math|Vector|MakeVector 0.0 0.0 0.0) (.Location (Math|Transform|BreakTransform (.transform (Default|GetVrmBoneTransform (Variables|Default|GetVrmUtilComponent) (Utilities|String|StringToName (Utilities|Array|Get(acopy) (Variables|Default|GetHumanoidCollistionBoneList) (+ _index 1))) "RTS_ParentBoneSpace")))) (/ (Math|Conversions|ToFloat(Integer) _array_index) (Math|Conversions|ToFloat(Integer) _returnvalue))) 1e+02))) -1.0) (.Z (Math|Vector|BreakVector (/ (Math|Vector|Lerp(Vector) (Math|Vector|MakeVector 0.0 0.0 0.0) (.Location (Math|Transform|BreakTransform (.transform (Default|GetVrmBoneTransform (Variables|Default|GetVrmUtilComponent) (Utilities|String|StringToName (Utilities|Array|Get(acopy) (Variables|Default|GetHumanoidCollistionBoneList) (+ _index 1))) "RTS_ParentBoneSpace")))) (/ (Math|Conversions|ToFloat(Integer) _array_index) (Math|Conversions|ToFloat(Integer) _returnvalue))) 1e+02))) (.Y (Math|Vector|BreakVector (/ (Math|Vector|Lerp(Vector) (Math|Vector|MakeVector 0.0 0.0 0.0) (.Location (Math|Transform|BreakTransform (.transform (Default|GetVrmBoneTransform (Variables|Default|GetVrmUtilComponent) (Utilities|String|StringToName (Utilities|Array|Get(acopy) (Variables|Default|GetHumanoidCollistionBoneList) (+ _index 1))) "RTS_ParentBoneSpace")))) (/ (Math|Conversions|ToFloat(Integer) _array_index) (Math|Conversions|ToFloat(Integer) _returnvalue))) 1e+02)))) (select (> (Utilities|String|FindSubstring (Utilities|Array|Get(acopy) _humanoidcollistionbonelist _index) "arm") 0) (Variables|Default|GetHumanoidArmCollisionRadius) (Variables|Default|GetHumanoidLegCollisionRadius))))))
                                    (:then_1
                                      (Utilities|Struct|SetmembersinVRMColliderMeta (Utilities|Array|Get(acopy) _vrmcollidermeta (Utilities|Array|LastIndex _vrmcollidermeta)) -1 (.Value (Utilities|Map|Find (Variables|/Script/VRM4U.VrmMetaObject|GethumanoidBoneTable (Variables|/Script/VRM4U.VrmAssetListObject|GetVrmMetaObject (Variables|/VRM4U/Util/Actor/Misc/sub/BP_VrmUtilComponent.BP_VrmUtilComponent_C|GetVrmAssetList (Variables|Default|GetVrmUtilComponent)))) (Utilities|Array|Get(acopy) _humanoidcollistionbonelist _index))) (Variables|Tmp|GetcollistionGroup)))))))))
                        (:then_1
                          (Utilities|FlowControl|Sequence
                            (:then_0
                              (bind _values (Utilities|Map|Values (Variables|Default|GetSpringParamSet))))
                            (:then_1
                              (Variables|/Script/VRM4U.VrmMetaObject|SetVRMSpringMeta (Variables|Default|GetTargetMeta) _values))
                            (:then_2
                              (for (_ _array_index_2) _values
                                (Utilities|FlowControl|Sequence
                                  (:then_0
                                    (Utilities|Array|Clear (Variables|tmp|Getspr_boneIndexList))
                                    (Utilities|Array|Clear (Variables|tmp|Getspr_boneNameList)))
                                  (:then_1
                                    (Utilities|FlowControl|Sequence
                                      (:then_0
                                        (bind _values_2 (Utilities|Map|Values _bone_to_springparamaddtail))
                                        (bind _keys (Utilities|Map|Keys _bone_to_springparamaddtail))
                                        (for (_array_element _array_index_3) _values_2
                                          (Utilities|FlowControl|Sequence
                                            (:then_0
                                              (Utilities|Array|Clear _bone_childall)
                                              (Utilities|Array|Add _bone_childall (Utilities|Array|Get(acopy) _keys _array_index_3)))
                                            (:then_1
                                              ;[1 1 1] tail bone
                                              (if (Variables|Default|GetbGenerateTailBone)
                                                (Utilities|FlowControl|Sequence
                                                  (:then_0
                                                    (bind _returnvalue_2 (Class|VrmBPFunctionLibrary|VRMRenderingThreadEnable false)))
                                                  (:then_1
                                                    (Class|LoaderBPFunctionLibrary|CreateTailBone (Variables|Default|GetPreview%28Auto%29) _keys))
                                                  (:then_2
                                                    (Class|VrmBPFunctionLibrary|VRMRenderingThreadEnable _returnvalue_2)))))
                                            (:then_2
                                              (if (== _array_element _array_index_2)
                                                ;[1 1 1] add bonename
                                                (Utilities|Array|AddUnique (Variables|tmp|Getspr_boneNameList) (Utilities|Array|Get(acopy) _keys _array_index_3)))))))
                                      (:then_1
                                        (bind _values_3 (Utilities|Map|Values _bone_to_springparam))
                                        (bind _keys_2 (Utilities|Map|Keys _bone_to_springparam))
                                        (for (_array_element_2 _array_index_4) _values_3
                                          (if (== _array_element_2 _array_index_2)
                                            (Utilities|Array|AddUnique (Variables|tmp|Getspr_boneNameList) (Utilities|Array|Get(acopy) _keys_2 _array_index_4)))))))
                                  (:then_2
                                    ;[1 1 1] bone index
                                    (for _array_element_3 (Variables|tmp|Getspr_boneNameList)
                                      (Utilities|Array|Add (Variables|tmp|Getspr_boneIndexList) (.OutIndex (Class|SkeletalMesh|FindSocketandIndex (Variables|/Script/VRM4U.VrmMetaObject|GetSkeletalMesh (Variables|Default|GetTargetMeta)) (Utilities|String|StringToName _array_element_3))))))
                                  (:then_3
                                    ;[1 1 1] add spring meta
                                    (Utilities|FlowControl|Sequence
                                      (:then_0
                                        (Utilities|Array|Clear _collisioninexlist_all_)
                                        (for (_ _array_index_5) (Variables|/Script/VRM4U.VrmMetaObject|GetVRMColliderMeta (Variables|Default|GetTargetMeta))
                                          (Utilities|Array|Add _collisioninexlist_all_ _array_index_5)))
                                      (:then_1
                                        (Utilities|Struct|SetmembersinVRMSpringMeta (Utilities|Array|Get(acopy) (Variables|/Script/VRM4U.VrmMetaObject|GetVRMSpringMeta (Variables|Default|GetTargetMeta)) _array_index_2) (Variables|tmp|Getspr_boneIndexList) (Variables|tmp|Getspr_boneNameList) (Variables|Tmp|GetCollisionInexList%28all%29))))))))))))))
                (:else)))))
        (:else)))
    (:else
      (Development|PrintString "!Warning! 
SetTargetActor!!"))))

(event Custom|init
  (bind _vrmutilcomponent (Variables|Default|GetVrmUtilComponent))
  (bind _targetactor (Variables|Default|GetTargetActor))
  (bind _skeletalmeshcomponent (Variables|/Script/Engine.SkeletalMeshActor|GetSkeletalMeshComponent _targetactor))
  (Variables|Default|SetPreview%28Auto%29 (Variables|/Script/VRM4U.VrmMetaObject|GetSkeletalMesh (Variables|Default|GetTargetMeta)))
  (Default|SetVRMAssetListfromMeshComponent _vrmutilcomponent (Variables|/Script/Engine.SkinnedMeshComponent|GetSkeletalMesh _skeletalmeshcomponent))
  (Default|SetTargetMeshComponent _vrmutilcomponent _skeletalmeshcomponent))

(event EventBeginPlay)

(event Collision|EventActorBeginOverlap
  (params (OtherActor :type Actor%20Object%20Reference)))

(event EventTick
  (params (DeltaSeconds :type Float%20%28single-precision%29)))

(fn ConstructionScript
  (CallFunction|Init))