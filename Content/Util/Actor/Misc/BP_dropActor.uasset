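; Actor that loads model files dropped through VrmDropFiles at runtime, replacing the previously spawned model.
; Imports synchronously or asynchronously into a new unsaved VRM asset list, using a smaller scale for non-.vrm files.
; Optionally spawns an attached MToonActor, then after a short delay sets its VrmAnimInstanceCopy to copy the pose from a BP_VrmCharacterBase player pawn.
; Broadcasts OnApplyNewVRM with the loaded asset list, with or without the sample actor.
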(event Custom|LoadVrmFronFilePath
  (params (FileName :type String))
  (bind _returnvalue (Game|Player|GetPlayerPawn 0))
  (bind _importoption (Variables|Default|GetImportOption))
  (bind (_asbp_vrm_character_base _bsuccess) (Utilities|Casting|CastToBP_VrmCharacterBase _returnvalue))
  (Utilities|FlowControl|Sequence
    (:then_0
      (bind _spawnedactor (Variables|Default|GetSpawnedActor)
        (:then
          (Actor|DestroyActor _spawnedactor))
        (:else)))
    (:then_1
      (bind _returnvalue_2 (Game|ConstructObjectfromClass "/VRM4U/VrmAssetListObjectBP.VrmAssetListObjectBP_C" self))
      (Utilities|FlowControl|Sequence
        (:then_0
          (Utilities|Struct|SetmembersinImportOptionData _importoption (select (>= (Utilities|String|FindSubstring FileName ".vrm") 0) 1.0 0.1)))
        (:then_1
          (Variables|/Script/VRM4U.VrmAssetListObject|SetbAssetSave _returnvalue_2 false))
        (:then_2
          (if (Variables|Default|GetbAsyncMode)
            (bind _outvrmasset (Class|LoaderBPFunctionLibrary|LoadVRMFileAsync _returnvalue_2 FileName _importoption))
            (Variables|Default|SetNewVar_0 _outvrmasset)
            (else
              (bind _outvrmasset_2 (Class|LoaderBPFunctionLibrary|LoadVRMFile _returnvalue_2 FileName _importoption))
              (Variables|Default|SetNewVar_0 _outvrmasset_2)))
          ;[1 1 1] Mesh Clear
          (Class|SkinnedMeshComponent|SetSkeletalMesh (Variables|Default|GetSkeletalMesh) 0 true)
          (if (Variables|Default|GetbSpawnSampleActor)
            (bind _returnvalue_3 (Game|SpawnActorfromClass "/VRM4U/Util/Actor/MToonActor.MToonActor_C" (Transformation|GetActorTransform) "Undefined" 0 (Variables|Default|GetNewVar_0) 5e+02 false true 0 false 0 0))
            (bind _output_get (Variables|Default|SetSpawnedActor _returnvalue_3))
            (Transformation|AttachActorToActor _output_get self "None" "SnapToTarget" "SnapToTarget" "SnapToTarget" true)
            (Utilities|FlowControl|Delay 0.2)
            (Utilities|FlowControl|Sequence
              (:then_0
                (Components|SkeletalMesh|SetAnimInstanceClass (Variables|/VRM4U/Util/Actor/MToonActor.MToonActor_C|GetSkeletalMesh _output_get) "/Script/VRM4U.VrmAnimInstanceCopy")
                (Class|SkinnedMeshComponent|SetSkeletalMesh (Variables|/VRM4U/Util/Actor/MToonActor.MToonActor_C|GetSkeletalMesh _output_get) (Variables|/Script/VRM4U.VrmAssetListObject|GetSkeletalMesh (Variables|Default|GetNewVar_0)) true)
                (bind _asvrm_anim_instance_copy (Utilities|Casting|CastToVrmAnimInstanceCopy (Components|SkeletalMesh|GetAnimInstance (Variables|/VRM4U/Util/Actor/MToonActor.MToonActor_C|GetSkeletalMesh _output_get))))
                (if _bsuccess
                  (Class|VrmAnimInstanceCopy|SetSkeletalMeshCopyData _asvrm_anim_instance_copy (Variables|Default|GetNewVar_0) (Variables|/Script/Engine.Character|GetMesh _asbp_vrm_character_base) 0 "/VRM4U/Util/BaseCharacter/Mesh/VRoidSimple_VrmAssetList.VRoidSimple_VrmAssetList")))
              (:then_1
                (Default|CallOnApplyNewVRM (Variables|Default|GetNewVar_0) :!label _label)))
            (else
              (goto _label))))))))

(event EventBeginPlay
  (EventDispatchers|AssignOnDropFiles (Variables|Default|GetVrmDropFiles) (delegate Custom|LoadVrmFronFilePath)))

(event Collision|EventActorBeginOverlap
  (params (OtherActor :type Actor%20Object%20Reference)))

(event EventTick
  (params (DeltaSeconds :type Float%20%28single-precision%29)))

(fn ConstructionScript)