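; BP_EyeWhite is an actor that renders eye whites on a VRM character using decals or planes.
; Its construction script resolves the mesh through a cached VRM utility lookup, attaches to the head bone and places both sides at the eye bones with mirrored offsets.
; It feeds color, mask, shadow and fade settings into a translucent or masked dynamic material, destroying the unused component type.
; Tick mirrors the target's visibility.
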(event Custom|CustomEvent_0
  (params (dummy :type Boolean))
  (bind _offsettransform (Variables|Default|GetOffsetTransform))
  (bind _decalleft (Variables|Default|GetDecalLeft))
  (bind _bp_vrmutilcomponent (Variables|Default|GetBP_VrmUtilComponent))
  (bind _decalright (Variables|Default|GetDecalRight))
  (bind _targetactor (Variables|Default|GetTargetActor))
  (bind _bp_vrmutilcomponent_2 (Variables|Default|GetBP_VrmUtilComponent))
  (bind _bp_vrmutilcomponent_3 (Variables|Default|GetBP_VrmUtilComponent))
  (bind (_location _rotation _scale) (Math|Transform|BreakTransform _offsettransform))
  (bind (_transform _found) (Default|GetVrmBoneTransform _bp_vrmutilcomponent_3 "rightEye" "RTS_World"))
  (bind (_found_2 _meshbonename) (Default|GetMeshBoneName _bp_vrmutilcomponent_3 "head"))
  (bind (_transform_2 _found_3) (Default|GetVrmBoneTransform _bp_vrmutilcomponent_3 "head" "RTS_World"))
  (bind (_transform_3 _found_4) (Default|GetVrmBoneTransform _bp_vrmutilcomponent_3 "leftEye" "RTS_World"))
  (bind (_x _y _z) (Math|Vector|BreakVector _location))
  (bind (_roll _pitch _yaw) (Math|Rotator|BreakRotator _rotation))
  (bind _rotation_2 (Math|Transform|BreakTransform _transform_2))
  (bind (_x_2 _y_2 _z_2) (Math|Vector|BreakVector _scale))
  (bind _location_2 (Math|Transform|BreakTransform _transform_3))
  (bind _location_3 (Math|Transform|BreakTransform _transform))
  (bind _returnvalue (Math|Vector|MakeVector 0.0 _y 0.0))
  (bind _returnvalue_2 (Math|Vector|MakeVector _x_2 _y_2 _z_2))
  (if (Variables|Default|GetbIgnore)
    (Rendering|SetVisibility (Variables|Default|GetScene) false true)
    (else
      (bind _targetactor_2 (Variables|Default|GetTargetActor)
        (:then
          (Utilities|FlowControl|Sequence
            (:then_0
              (if (!= (Variables|Development|Get%28auto%29TargetActor_latest) _targetactor_2)
                (Variables|Development|Set%28auto%29TargetComponent 0 :!label _label)
                (Variables|Development|Set%28auto%29TargetActor_latest 0)))
            (:then_1
              (Utilities|FlowControl|Sequence
                (:then_0
                  (Variables|Development|Get%28auto%29VrmAssetList
                    (:then
                      (bind __auto_targetcomponent (Variables|Development|Get%28auto%29TargetComponent)
                        (:then
                          (Variables|/VRM4U/Util/Actor/Misc/sub/BP_VrmUtilComponent.BP_VrmUtilComponent_C|SetVrmAssetList _bp_vrmutilcomponent_2 (Variables|Development|Get%28auto%29VrmAssetList))
                          (Default|SetTargetMeshComponent _bp_vrmutilcomponent_2 0 __auto_targetcomponent))
                        (:else
                          (Default|SetActor _bp_vrmutilcomponent (Variables|Default|GetTargetActor) :!label _label_2)
                          (Variables|Development|Set%28auto%29VrmAssetList (Variables|/VRM4U/Util/Actor/Misc/sub/BP_VrmUtilComponent.BP_VrmUtilComponent_C|GetVrmAssetList _bp_vrmutilcomponent))
                          (Variables|Development|Set%28auto%29TargetComponent (Variables|/VRM4U/Util/Actor/Misc/sub/BP_VrmUtilComponent.BP_VrmUtilComponent_C|GetTargetAsSkinnedMeshComponent _bp_vrmutilcomponent)))))
                    (:else
                      (goto _label_2))))
                (:then_1
                  (if _found_2
                    (if (!= (Actor|GetAttachParentActor self) _targetactor)
                      (Transformation|AttachActorToActor _targetactor _meshbonename "SnapToTarget" "SnapToTarget" "SnapToTarget" true))))
                (:then_2
                  (if (Math|Boolean|ANDBoolean _found_3 _found_4 _found)
                    (if (not (== (Math|Vector|VectorLength (- _location_2 _location_3)) 0.0))
                      (Utilities|FlowControl|Sequence
                        (:then_0
                          (Transformation|SetWorldTransform (Variables|Default|GetDecalLeft) (Math|Transform|MakeTransform _location_2 _rotation_2) false false))
                        (:then_1
                          (Transformation|SetWorldTransform (Variables|Default|GetDecalRight) (Math|Transform|MakeTransform _location_3 _rotation_2) false false))))))
                (:then_3
                  (Transformation|SetRelativeLocation (Variables|Default|GetScene) (Math|Vector|MakeVector 0.0 _x _z) false false)
                  (Utilities|FlowControl|Sequence
                    (:then_0
                      (Transformation|AddRelativeLocation _decalright _returnvalue false false)
                      (Transformation|AddRelativeLocation _decalleft (* _returnvalue -1.0) false false))
                    (:then_1
                      (Transformation|AddRelativeRotation _decalright _rotation false false)
                      (Transformation|AddRelativeRotation _decalleft (Math|Rotator|MakeRotator _roll (* _pitch -1.0) (* _yaw -1.0)) false false))
                    (:then_2
                      (Transformation|SetRelativeScale3D _decalright _returnvalue_2)
                      (Transformation|SetRelativeScale3D _decalleft _returnvalue_2))))
                (:then_4
                  (Utilities|FlowControl|Sequence
                    (:then_0
                      (if (Variables|Default|GetbUseTranslucent)
                        (bind _returnvalue_3 (Rendering|Material|CreateDynamicMaterialInstance "/VRM4U/Util/Actor/Misc/sub/M_EyeWhiteTranslucent.M_EyeWhiteTranslucent" "None" :!class /Script/Engine.KismetMaterialLibrary))
                        (Variables|Default|SetNewVar_0 _returnvalue_3)
                        (else
                          (bind _returnvalue_4 (Rendering|Material|CreateDynamicMaterialInstance "/VRM4U/Util/Actor/Misc/sub/M_EyeWhiteMask.M_EyeWhiteMask" "None" :!class /Script/Engine.KismetMaterialLibrary))
                          (Variables|Default|SetNewVar_0 _returnvalue_4))))
                    (:then_1
                      (Rendering|Material|SetVectorParameterValue (Variables|Default|GetNewVar_0) "Col1" (Variables|Default|GetOverrideBaseColor) :!class /Script/Engine.MaterialInstanceDynamic)
                      (Rendering|Material|SetVectorParameterValue (Variables|Default|GetNewVar_0) "Col2" (Variables|Default|GetOverrideEmissiveColor) :!class /Script/Engine.MaterialInstanceDynamic)
                      (Rendering|Material|SetScalarParameterValue (Variables|Default|GetNewVar_0) "MaskScale" (Variables|Default|GetMaskScale) :!class /Script/Engine.MaterialInstanceDynamic)
                      (Rendering|Material|SetScalarParameterValue (Variables|Default|GetNewVar_0) "ShadowCenter" (Variables|Default|GetShcadowCenter) :!class /Script/Engine.MaterialInstanceDynamic)
                      (Rendering|Material|SetScalarParameterValue (Variables|Default|GetNewVar_0) "ShadowScale" (Variables|Default|GetShdowScale) :!class /Script/Engine.MaterialInstanceDynamic)
                      (Rendering|Material|SetScalarParameterValue (Variables|Default|GetNewVar_0) "FadeDistance" (Variables|Default|GetFadeDistance) :!class /Script/Engine.MaterialInstanceDynamic)
                      (Rendering|Components|Decal|SetDecalMaterial (Variables|Default|GetDecalLeft) (Variables|Default|GetNewVar_0))
                      (Rendering|Material|SetMaterial (Variables|Default|GetPlaneLeft) 0 (Variables|Default|GetNewVar_0)))))
                (:then_5
                  (if (Variables|Default|GetbUsePlane)
                    (Components|DestroyComponent (Variables|Default|GetDecalRight))
                    (else
                      (Components|DestroyComponent (Variables|Default|GetPlaneLeft)))))))))
        (:else
          (goto _label))))))

(event EventBeginPlay)

(event Collision|EventActorBeginOverlap
  (params (OtherActor :type Actor%20Object%20Reference)))

(event EventTick
  (params (DeltaSeconds :type Float%20%28single-precision%29))
  (bind _scene (Variables|Default|GetScene))
  (bind _targetactor (Variables|Default|GetTargetActor)
    (:then
      (if (Math|Boolean|NotEqual(Boolean) (and (not (Variables|/Script/Engine.Actor|GetbHidden _targetactor)) (Rendering|IsVisible (Actor|GetComponentbyClass _targetactor "/Script/Engine.SkeletalMeshComponent"))) (Rendering|IsVisible _scene))
        (Rendering|SetVisibility _scene (and (not (Variables|/Script/Engine.Actor|GetbHidden _targetactor)) (Rendering|IsVisible (Actor|GetComponentbyClass _targetactor "/Script/Engine.SkeletalMeshComponent"))) true)))
    (:else)))

(fn ConstructionScript
  (CallFunction|CustomEvent0 false))