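; Utility actor that drives a target VRM character's blend shape groups by named weight.
; Init, run from construction, builds the weight lists from VRM metadata.
; Each weight, the larger of the map value and a parallel Sequencer array, scales morph targets and lerps dynamic material vector parameters from parent defaults to group colors.
; Changes can mirror to a preview mesh, hidden on BeginPlay; setter and reset events re-apply weights.
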(event Custom|init
  (params (reset :type Boolean) (TargetActor :type Actor%20Object%20Reference))
  (bind _param_for_sequencer (Variables|Default|Getparam_for_sequencer))
  (bind _blendshapelist_param (Variables|Default|GetBlendShapeList_param))
  (bind _blendshapelist_param_2 (Variables|Default|GetBlendShapeList_param))
  (bind _bp_vrmutilcomponent (Variables|Default|GetBP_VrmUtilComponent))
  (bind _bp_vrmutilcomponent_2 (Variables|Default|GetBP_VrmUtilComponent))
  (bind _blendshapelist_param_3 (Variables|Default|GetBlendShapeList_param))
  (bind _skeletalmesh_preview_ (Variables|Default|GetSkeletalMesh%28Preview%29))
  (bind _returnvalue (Utilities|Map|Length _blendshapelist_param))
  (bind _targetmeshcomponent (Variables|/VRM4U/Util/Actor/Misc/sub/BP_VrmUtilComponent.BP_VrmUtilComponent_C|GetTargetMeshComponent _bp_vrmutilcomponent_2))
  (Utilities|FlowControl|Sequence
    (:then_0
      (Utilities|IsValid TargetActor
        (:Is%20Valid
          (Variables|Default|SetTargetActor TargetActor)
          (Variables|Default|Setreset true))))
    (:then_1
      (bind _output_get (Variables|Default|Setreset (or (stale _output_get) reset)))
      (Variables|Default|GetTargetActor
        (:then
          (Utilities|FlowControl|Sequence
            (:then_1
              ;[1 1 1] create morphgrouplist
              (if (Variables|Default|Getreset)
                (Utilities|Map|Clear (Variables|Default|GetBlendShapeList_param))
                (Utilities|Map|Clear (Variables|develop|GetMorphList_param_tmp))
                (Utilities|Array|Clear (Variables|Default|Getparam_for_sequencer))))
            (:then_2
              (Default|SetActor _bp_vrmutilcomponent (Variables|Default|GetTargetActor))
              (Utilities|FlowControl|Sequence
                (:then_0
                  (Utilities|Map|Remove _blendshapelist_param_2 ""))
                (:then_1
                  (bind _array_element (Utilities|Array|ForEachLoopwithBreak (Variables|/Script/VRM4U.VrmMetaObject|GetBlendShapeGroup (Variables|/Script/VRM4U.VrmAssetListObject|GetVrmMetaObject (Variables|/VRM4U/Util/Actor/Misc/sub/BP_VrmUtilComponent.BP_VrmUtilComponent_C|GetVrmAssetList _bp_vrmutilcomponent))))
                    (:LoopBody
                      (if (not (.ReturnValue (Utilities|Map|Find _blendshapelist_param_2 (.name (Utilities|Struct|BreakVrmBlendShapeGroup _array_element)))))
                        (Utilities|Map|Add _blendshapelist_param_2 (.name (Utilities|Struct|BreakVrmBlendShapeGroup _array_element)) 0.0)
                        (Utilities|Map|Add (Variables|develop|GetMorphList_param_tmp) (.name (Utilities|Struct|BreakVrmBlendShapeGroup _array_element)) 0.0)
                        (Utilities|Map|Add (Variables|develop|GetBlendShapeList_Group) (.name (Utilities|Struct|BreakVrmBlendShapeGroup _array_element)) _array_element)))
                    (:Completed
                      (if (!= (Utilities|Array|Length _param_for_sequencer) _returnvalue)
                        (Utilities|Array|Resize _param_for_sequencer _returnvalue)))))))
            (:then_3
              (if (Variables|Default|Getreset)
                (Utilities|FlowControl|Sequence
                  (:then_0
                    (for _array_element_2 (Class|VrmBPFunctionLibrary|VRMGetMorphTargetList (Variables|/Script/Engine.SkinnedMeshComponent|GetSkeletalMesh _targetmeshcomponent))
                      (Components|SkeletalMesh|SetMorphTarget _targetmeshcomponent (Utilities|String|StringToName _array_element_2) 0.0 true)))
                  (:then_1
                    (Components|SkeletalMesh|SetUpdateAnimationinEditor _targetmeshcomponent true)))))
            (:then_4
              (if (not (Variables|Default|GetbBeginPlay))
                ;[1 1 1] preview
                (bind _targetmeshcomponent_2 (Variables|/VRM4U/Util/Actor/Misc/sub/BP_VrmUtilComponent.BP_VrmUtilComponent_C|GetTargetMeshComponent (Variables|Default|GetBP_VrmUtilComponent))
                  (:then
                    (Class|SkinnedMeshComponent|SetSkeletalMesh _skeletalmesh_preview_ (Variables|/Script/Engine.SkinnedMeshComponent|GetSkeletalMesh _targetmeshcomponent_2) true)
                    (for (_ _array_index) (Rendering|Material|GetMaterials _skeletalmesh_preview_)
                      (Rendering|Material|CreateDynamicMaterialInstance _skeletalmesh_preview_ _array_index 0 "None" :!class /Script/Engine.PrimitiveComponent)))
                  (:else))))
            (:then_5
              (bind _values (Utilities|Map|Values (Variables|develop|GetMorphList_param_tmp)))
              (bind _keys (Utilities|Map|Keys _blendshapelist_param_3))
              (bind _values_2 (Utilities|Map|Values _blendshapelist_param_3))
              (for (_array_element_3 _array_index_2) _values_2
                (Utilities|FlowControl|Sequence
                  (:then_0
                    (if (or (> (Utilities|Array|Get(acopy) _values _array_index_2) 0.0) (> (Math|Float|Max(Float) _array_element_3 (Utilities|Array|Get(acopy) (Variables|Default|Getparam_for_sequencer) _array_index_2)) 0.0))
                      (Utilities|FlowControl|Sequence
                        (:then_0
                          ;[1 1 1] MaterialList
                          (if (not (Variables|Default|GetbSkipMaterialList))
                            (bind _array_element_4 (Utilities|Array|ForEachLoopwithBreak (.MaterialList (Utilities|Struct|BreakVrmBlendShapeGroup (.Value (Utilities|Map|Find (Variables|develop|GetBlendShapeList_Group) (Utilities|Array|Get(acopy) _keys _array_index_2))))) :!label _label)
                              (:LoopBody
                                (bind (_array_element_5 _array_index_3) (Utilities|Array|ForEachLoopwithBreak (Rendering|Material|GetMaterials (Variables|/VRM4U/Util/Actor/Misc/sub/BP_VrmUtilComponent.BP_VrmUtilComponent_C|GetTargetMeshComponent (Variables|Default|GetBP_VrmUtilComponent))))
                                  (:LoopBody
                                    (bind _asmaterial_instance_dynamic (Utilities|Casting|CastToMaterialInstanceDynamic _array_element_5)
                                      (:then
                                        (if (Utilities|Enum|Equal(Enum) (Utilities|GetObjectName (Variables|/Script/Engine.MaterialInstance|GetParent _asmaterial_instance_dynamic)) (.materialName (Utilities|Struct|BreakVrmBlendShapeMaterialList _array_element_4)))
                                          (bind _returnvalue_2 (Rendering|Material|GetVectorParameterValue (.AsMaterial%20Instance%20Constant (Utilities|Casting|CastToMaterialInstanceConstant (Variables|/Script/Engine.MaterialInstance|GetParent _asmaterial_instance_dynamic))) (Utilities|String|StringToName (.propertyName (Utilities|Struct|BreakVrmBlendShapeMaterialList _array_element_4))) :!class /Script/Engine.MaterialInstanceConstant))
                                          (Rendering|Material|SetVectorParameterValue _asmaterial_instance_dynamic (Utilities|String|StringToName (.propertyName (Utilities|Struct|BreakVrmBlendShapeMaterialList _array_element_4))) (Math|Color|Lerp(LinearColor) _returnvalue_2 (Math|Color|MakeColor (.R (Math|Color|BreakColor (.color (Utilities|Struct|BreakVrmBlendShapeMaterialList _array_element_4)))) (.G (Math|Color|BreakColor (.color (Utilities|Struct|BreakVrmBlendShapeMaterialList _array_element_4)))) (.B (Math|Color|BreakColor (.color (Utilities|Struct|BreakVrmBlendShapeMaterialList _array_element_4)))) (select (Variables|Default|GetbUseDefaultAlpha) (.A (Utilities|Struct|BreakLinearColor _returnvalue_2)) (.A (Math|Color|BreakColor (.color (Utilities|Struct|BreakVrmBlendShapeMaterialList _array_element_4)))))) (Math|Float|Max(Float) _array_element_3 (Utilities|Array|Get(acopy) (Variables|Default|Getparam_for_sequencer) _array_index_2))) :!class /Script/Engine.MaterialInstanceDynamic)
                                          (Utilities|FlowControl|Sequence
                                            (:then_0
                                              (if (not (Variables|Default|GetbBeginPlay))
                                                (Rendering|Material|SetVectorParameterValue (.AsMaterial%20Instance%20Dynamic (Utilities|Casting|CastToMaterialInstanceDynamic (Utilities|Array|Get(acopy) (Rendering|Material|GetMaterials (Variables|Default|GetSkeletalMesh%28Preview%29)) _array_index_3))) (Utilities|String|StringToName (.propertyName (Utilities|Struct|BreakVrmBlendShapeMaterialList _array_element_4))) (Math|Color|Lerp(LinearColor) _returnvalue_2 (Math|Color|MakeColor (.R (Math|Color|BreakColor (.color (Utilities|Struct|BreakVrmBlendShapeMaterialList _array_element_4)))) (.G (Math|Color|BreakColor (.color (Utilities|Struct|BreakVrmBlendShapeMaterialList _array_element_4)))) (.B (Math|Color|BreakColor (.color (Utilities|Struct|BreakVrmBlendShapeMaterialList _array_element_4)))) (select (Variables|Default|GetbUseDefaultAlpha) (.A (Utilities|Struct|BreakLinearColor _returnvalue_2)) (.A (Math|Color|BreakColor (.color (Utilities|Struct|BreakVrmBlendShapeMaterialList _array_element_4)))))) (Math|Float|Max(Float) _array_element_3 (Utilities|Array|Get(acopy) (Variables|Default|Getparam_for_sequencer) _array_index_2))) :!class /Script/Engine.MaterialInstanceDynamic)))
                                            (:then_1
                                              (goto _label Break)))))
                                      (:CastFailed
                                        (Development|PrintString (Utilities|String|Append "warning: not dynamic material  ->  " (Utilities|GetDisplayName _array_element_5) " 
use  TargetActor with MToonAttachActor"))))))))))
                        (:then_1
                          ;[1 1 1] MorphGroup
                          (if (not (Variables|Default|GetbSkipMorphTarget))
                            (bind _array_element_6 (Utilities|Array|ForEachLoopwithBreak (.BlendShape (Utilities|Struct|BreakVrmBlendShapeGroup (.Value (Utilities|Map|Find (Variables|develop|GetBlendShapeList_Group) (Utilities|Array|Get(acopy) _keys _array_index_2))))))
                              (:LoopBody
                                (Components|SkeletalMesh|SetMorphTarget (Variables|/VRM4U/Util/Actor/Misc/sub/BP_VrmUtilComponent.BP_VrmUtilComponent_C|GetTargetMeshComponent (Variables|Default|GetBP_VrmUtilComponent)) (Utilities|String|StringToName (.morphTargetName (Utilities|Struct|BreakVrmBlendShape _array_element_6))) (* (Math|Float|Max(Float) _array_element_3 (Utilities|Array|Get(acopy) (Variables|Default|Getparam_for_sequencer) _array_index_2)) (/ (Math|Conversions|ToFloat(Integer) (.weight (Utilities|Struct|BreakVrmBlendShape _array_element_6))) 1e+02)) true)
                                (if (not (Variables|Default|GetbBeginPlay))
                                  (Components|SkeletalMesh|SetMorphTarget (Variables|Default|GetSkeletalMesh%28Preview%29) (Utilities|String|StringToName (.morphTargetName (Utilities|Struct|BreakVrmBlendShape _array_element_6))) (* (Math|Float|Max(Float) _array_element_3 (Utilities|Array|Get(acopy) (Variables|Default|Getparam_for_sequencer) _array_index_2)) (/ (Math|Conversions|ToFloat(Integer) (.weight (Utilities|Struct|BreakVrmBlendShape _array_element_6))) 1e+02)) true)))))))))
                  (:then_1
                    (Utilities|Map|Add (Variables|develop|GetMorphList_param_tmp) (Utilities|Array|Get(acopy) _keys _array_index_2) (Math|Float|Max(Float) _array_element_3 (Utilities|Array|Get(acopy) (Variables|Default|Getparam_for_sequencer) _array_index_2)))))))))
        (:else
          (Variables|Default|Setreset true))))
    (:then_2
      (Variables|Default|Setreset false))))

(event Custom|SetBlendShapeGroupWeight
  (params (BlendshapeGroup :type String) (Weight :type Float%20%28single-precision%29))
  (bind _blendshapelist_param (Variables|Default|GetBlendShapeList_param))
  (bind _blendshapelist_param_2 (Variables|Default|GetBlendShapeList_param))
  (if (.ReturnValue (Utilities|Map|Find _blendshapelist_param_2 BlendshapeGroup))
    (Utilities|Map|Add _blendshapelist_param_2 BlendshapeGroup Weight)
    (bind _values (Utilities|Map|Values (Variables|develop|GetMorphList_param_tmp)))
    (bind _keys (Utilities|Map|Keys _blendshapelist_param))
    (bind _values_2 (Utilities|Map|Values _blendshapelist_param))
    (for (_array_element _array_index) _values_2
      (Utilities|FlowControl|Sequence
        (:then_0
          (if (or (> (Utilities|Array|Get(acopy) _values _array_index) 0.0) (> (Math|Float|Max(Float) _array_element (Utilities|Array|Get(acopy) (Variables|Default|Getparam_for_sequencer) _array_index)) 0.0))
            (Utilities|FlowControl|Sequence
              (:then_0
                ;[1 1 1] MaterialList
                (if (not (Variables|Default|GetbSkipMaterialList))
                  (bind _array_element_2 (Utilities|Array|ForEachLoopwithBreak (.MaterialList (Utilities|Struct|BreakVrmBlendShapeGroup (.Value (Utilities|Map|Find (Variables|develop|GetBlendShapeList_Group) (Utilities|Array|Get(acopy) _keys _array_index))))) :!label _label)
                    (:LoopBody
                      (bind (_array_element_3 _array_index_2) (Utilities|Array|ForEachLoopwithBreak (Rendering|Material|GetMaterials (Variables|/VRM4U/Util/Actor/Misc/sub/BP_VrmUtilComponent.BP_VrmUtilComponent_C|GetTargetMeshComponent (Variables|Default|GetBP_VrmUtilComponent))))
                        (:LoopBody
                          (bind _asmaterial_instance_dynamic (Utilities|Casting|CastToMaterialInstanceDynamic _array_element_3)
                            (:then
                              (if (Utilities|Enum|Equal(Enum) (Utilities|GetObjectName (Variables|/Script/Engine.MaterialInstance|GetParent _asmaterial_instance_dynamic)) (.materialName (Utilities|Struct|BreakVrmBlendShapeMaterialList _array_element_2)))
                                (bind _returnvalue (Rendering|Material|GetVectorParameterValue (.AsMaterial%20Instance%20Constant (Utilities|Casting|CastToMaterialInstanceConstant (Variables|/Script/Engine.MaterialInstance|GetParent _asmaterial_instance_dynamic))) (Utilities|String|StringToName (.propertyName (Utilities|Struct|BreakVrmBlendShapeMaterialList _array_element_2))) :!class /Script/Engine.MaterialInstanceConstant))
                                (Rendering|Material|SetVectorParameterValue _asmaterial_instance_dynamic (Utilities|String|StringToName (.propertyName (Utilities|Struct|BreakVrmBlendShapeMaterialList _array_element_2))) (Math|Color|Lerp(LinearColor) _returnvalue (Math|Color|MakeColor (.R (Math|Color|BreakColor (.color (Utilities|Struct|BreakVrmBlendShapeMaterialList _array_element_2)))) (.G (Math|Color|BreakColor (.color (Utilities|Struct|BreakVrmBlendShapeMaterialList _array_element_2)))) (.B (Math|Color|BreakColor (.color (Utilities|Struct|BreakVrmBlendShapeMaterialList _array_element_2)))) (select (Variables|Default|GetbUseDefaultAlpha) (.A (Utilities|Struct|BreakLinearColor _returnvalue)) (.A (Math|Color|BreakColor (.color (Utilities|Struct|BreakVrmBlendShapeMaterialList _array_element_2)))))) (Math|Float|Max(Float) _array_element (Utilities|Array|Get(acopy) (Variables|Default|Getparam_for_sequencer) _array_index))) :!class /Script/Engine.MaterialInstanceDynamic)
                                (Utilities|FlowControl|Sequence
                                  (:then_0
                                    (if (not (Variables|Default|GetbBeginPlay))
                                      (Rendering|Material|SetVectorParameterValue (.AsMaterial%20Instance%20Dynamic (Utilities|Casting|CastToMaterialInstanceDynamic (Utilities|Array|Get(acopy) (Rendering|Material|GetMaterials (Variables|Default|GetSkeletalMesh%28Preview%29)) _array_index_2))) (Utilities|String|StringToName (.propertyName (Utilities|Struct|BreakVrmBlendShapeMaterialList _array_element_2))) (Math|Color|Lerp(LinearColor) _returnvalue (Math|Color|MakeColor (.R (Math|Color|BreakColor (.color (Utilities|Struct|BreakVrmBlendShapeMaterialList _array_element_2)))) (.G (Math|Color|BreakColor (.color (Utilities|Struct|BreakVrmBlendShapeMaterialList _array_element_2)))) (.B (Math|Color|BreakColor (.color (Utilities|Struct|BreakVrmBlendShapeMaterialList _array_element_2)))) (select (Variables|Default|GetbUseDefaultAlpha) (.A (Utilities|Struct|BreakLinearColor _returnvalue)) (.A (Math|Color|BreakColor (.color (Utilities|Struct|BreakVrmBlendShapeMaterialList _array_element_2)))))) (Math|Float|Max(Float) _array_element (Utilities|Array|Get(acopy) (Variables|Default|Getparam_for_sequencer) _array_index))) :!class /Script/Engine.MaterialInstanceDynamic)))
                                  (:then_1
                                    (goto _label Break)))))
                            (:CastFailed
                              (Development|PrintString (Utilities|String|Append "warning: not dynamic material  ->  " (Utilities|GetDisplayName _array_element_3) " 
use  TargetActor with MToonAttachActor"))))))))))
              (:then_1
                ;[1 1 1] MorphGroup
                (if (not (Variables|Default|GetbSkipMorphTarget))
                  (bind _array_element_4 (Utilities|Array|ForEachLoopwithBreak (.BlendShape (Utilities|Struct|BreakVrmBlendShapeGroup (.Value (Utilities|Map|Find (Variables|develop|GetBlendShapeList_Group) (Utilities|Array|Get(acopy) _keys _array_index))))))
                    (:LoopBody
                      (Components|SkeletalMesh|SetMorphTarget (Variables|/VRM4U/Util/Actor/Misc/sub/BP_VrmUtilComponent.BP_VrmUtilComponent_C|GetTargetMeshComponent (Variables|Default|GetBP_VrmUtilComponent)) (Utilities|String|StringToName (.morphTargetName (Utilities|Struct|BreakVrmBlendShape _array_element_4))) (* (Math|Float|Max(Float) _array_element (Utilities|Array|Get(acopy) (Variables|Default|Getparam_for_sequencer) _array_index)) (/ (Math|Conversions|ToFloat(Integer) (.weight (Utilities|Struct|BreakVrmBlendShape _array_element_4))) 1e+02)) true)
                      (if (not (Variables|Default|GetbBeginPlay))
                        (Components|SkeletalMesh|SetMorphTarget (Variables|Default|GetSkeletalMesh%28Preview%29) (Utilities|String|StringToName (.morphTargetName (Utilities|Struct|BreakVrmBlendShape _array_element_4))) (* (Math|Float|Max(Float) _array_element (Utilities|Array|Get(acopy) (Variables|Default|Getparam_for_sequencer) _array_index)) (/ (Math|Conversions|ToFloat(Integer) (.weight (Utilities|Struct|BreakVrmBlendShape _array_element_4))) 1e+02)) true)))))))))
        (:then_1
          (Utilities|Map|Add (Variables|develop|GetMorphList_param_tmp) (Utilities|Array|Get(acopy) _keys _array_index) (Math|Float|Max(Float) _array_element (Utilities|Array|Get(acopy) (Variables|Default|Getparam_for_sequencer) _array_index))))))))

(event Custom|ResetWeight
  (bind _blendshapelist_param (Variables|Default|GetBlendShapeList_param))
  (bind _blendshapelist_param_2 (Variables|Default|GetBlendShapeList_param))
  (bind _keys (Utilities|Map|Keys _blendshapelist_param))
  (for _array_element _keys
    (Utilities|Map|Add _blendshapelist_param _array_element 0.0))
  (bind _values (Utilities|Map|Values (Variables|develop|GetMorphList_param_tmp)))
  (bind _keys_2 (Utilities|Map|Keys _blendshapelist_param_2))
  (bind _values_2 (Utilities|Map|Values _blendshapelist_param_2))
  (for (_array_element_2 _array_index) _values_2
    (Utilities|FlowControl|Sequence
      (:then_0
        (if (or (> (Utilities|Array|Get(acopy) _values _array_index) 0.0) (> (Math|Float|Max(Float) _array_element_2 (Utilities|Array|Get(acopy) (Variables|Default|Getparam_for_sequencer) _array_index)) 0.0))
          (Utilities|FlowControl|Sequence
            (:then_0
              ;[1 1 1] MaterialList
              (if (not (Variables|Default|GetbSkipMaterialList))
                (bind _array_element_3 (Utilities|Array|ForEachLoopwithBreak (.MaterialList (Utilities|Struct|BreakVrmBlendShapeGroup (.Value (Utilities|Map|Find (Variables|develop|GetBlendShapeList_Group) (Utilities|Array|Get(acopy) _keys_2 _array_index))))) :!label _label)
                  (:LoopBody
                    (bind (_array_element_4 _array_index_2) (Utilities|Array|ForEachLoopwithBreak (Rendering|Material|GetMaterials (Variables|/VRM4U/Util/Actor/Misc/sub/BP_VrmUtilComponent.BP_VrmUtilComponent_C|GetTargetMeshComponent (Variables|Default|GetBP_VrmUtilComponent))))
                      (:LoopBody
                        (bind _asmaterial_instance_dynamic (Utilities|Casting|CastToMaterialInstanceDynamic _array_element_4)
                          (:then
                            (if (Utilities|Enum|Equal(Enum) (Utilities|GetObjectName (Variables|/Script/Engine.MaterialInstance|GetParent _asmaterial_instance_dynamic)) (.materialName (Utilities|Struct|BreakVrmBlendShapeMaterialList _array_element_3)))
                              (bind _returnvalue (Rendering|Material|GetVectorParameterValue (.AsMaterial%20Instance%20Constant (Utilities|Casting|CastToMaterialInstanceConstant (Variables|/Script/Engine.MaterialInstance|GetParent _asmaterial_instance_dynamic))) (Utilities|String|StringToName (.propertyName (Utilities|Struct|BreakVrmBlendShapeMaterialList _array_element_3))) :!class /Script/Engine.MaterialInstanceConstant))
                              (Rendering|Material|SetVectorParameterValue _asmaterial_instance_dynamic (Utilities|String|StringToName (.propertyName (Utilities|Struct|BreakVrmBlendShapeMaterialList _array_element_3))) (Math|Color|Lerp(LinearColor) _returnvalue (Math|Color|MakeColor (.R (Math|Color|BreakColor (.color (Utilities|Struct|BreakVrmBlendShapeMaterialList _array_element_3)))) (.G (Math|Color|BreakColor (.color (Utilities|Struct|BreakVrmBlendShapeMaterialList _array_element_3)))) (.B (Math|Color|BreakColor (.color (Utilities|Struct|BreakVrmBlendShapeMaterialList _array_element_3)))) (select (Variables|Default|GetbUseDefaultAlpha) (.A (Utilities|Struct|BreakLinearColor _returnvalue)) (.A (Math|Color|BreakColor (.color (Utilities|Struct|BreakVrmBlendShapeMaterialList _array_element_3)))))) (Math|Float|Max(Float) _array_element_2 (Utilities|Array|Get(acopy) (Variables|Default|Getparam_for_sequencer) _array_index))) :!class /Script/Engine.MaterialInstanceDynamic)
                              (Utilities|FlowControl|Sequence
                                (:then_0
                                  (if (not (Variables|Default|GetbBeginPlay))
                                    (Rendering|Material|SetVectorParameterValue (.AsMaterial%20Instance%20Dynamic (Utilities|Casting|CastToMaterialInstanceDynamic (Utilities|Array|Get(acopy) (Rendering|Material|GetMaterials (Variables|Default|GetSkeletalMesh%28Preview%29)) _array_index_2))) (Utilities|String|StringToName (.propertyName (Utilities|Struct|BreakVrmBlendShapeMaterialList _array_element_3))) (Math|Color|Lerp(LinearColor) _returnvalue (Math|Color|MakeColor (.R (Math|Color|BreakColor (.color (Utilities|Struct|BreakVrmBlendShapeMaterialList _array_element_3)))) (.G (Math|Color|BreakColor (.color (Utilities|Struct|BreakVrmBlendShapeMaterialList _array_element_3)))) (.B (Math|Color|BreakColor (.color (Utilities|Struct|BreakVrmBlendShapeMaterialList _array_element_3)))) (select (Variables|Default|GetbUseDefaultAlpha) (.A (Utilities|Struct|BreakLinearColor _returnvalue)) (.A (Math|Color|BreakColor (.color (Utilities|Struct|BreakVrmBlendShapeMaterialList _array_element_3)))))) (Math|Float|Max(Float) _array_element_2 (Utilities|Array|Get(acopy) (Variables|Default|Getparam_for_sequencer) _array_index))) :!class /Script/Engine.MaterialInstanceDynamic)))
                                (:then_1
                                  (goto _label Break)))))
                          (:CastFailed
                            (Development|PrintString (Utilities|String|Append "warning: not dynamic material  ->  " (Utilities|GetDisplayName _array_element_4) " 
use  TargetActor with MToonAttachActor"))))))))))
            (:then_1
              ;[1 1 1] MorphGroup
              (if (not (Variables|Default|GetbSkipMorphTarget))
                (bind _array_element_5 (Utilities|Array|ForEachLoopwithBreak (.BlendShape (Utilities|Struct|BreakVrmBlendShapeGroup (.Value (Utilities|Map|Find (Variables|develop|GetBlendShapeList_Group) (Utilities|Array|Get(acopy) _keys_2 _array_index))))))
                  (:LoopBody
                    (Components|SkeletalMesh|SetMorphTarget (Variables|/VRM4U/Util/Actor/Misc/sub/BP_VrmUtilComponent.BP_VrmUtilComponent_C|GetTargetMeshComponent (Variables|Default|GetBP_VrmUtilComponent)) (Utilities|String|StringToName (.morphTargetName (Utilities|Struct|BreakVrmBlendShape _array_element_5))) (* (Math|Float|Max(Float) _array_element_2 (Utilities|Array|Get(acopy) (Variables|Default|Getparam_for_sequencer) _array_index)) (/ (Math|Conversions|ToFloat(Integer) (.weight (Utilities|Struct|BreakVrmBlendShape _array_element_5))) 1e+02)) true)
                    (if (not (Variables|Default|GetbBeginPlay))
                      (Components|SkeletalMesh|SetMorphTarget (Variables|Default|GetSkeletalMesh%28Preview%29) (Utilities|String|StringToName (.morphTargetName (Utilities|Struct|BreakVrmBlendShape _array_element_5))) (* (Math|Float|Max(Float) _array_element_2 (Utilities|Array|Get(acopy) (Variables|Default|Getparam_for_sequencer) _array_index)) (/ (Math|Conversions|ToFloat(Integer) (.weight (Utilities|Struct|BreakVrmBlendShape _array_element_5))) 1e+02)) true)))))))))
      (:then_1
        (Utilities|Map|Add (Variables|develop|GetMorphList_param_tmp) (Utilities|Array|Get(acopy) _keys_2 _array_index) (Math|Float|Max(Float) _array_element_2 (Utilities|Array|Get(acopy) (Variables|Default|Getparam_for_sequencer) _array_index)))))))

(event EventBeginPlay
  (Utilities|FlowControl|Sequence
    (:then_0
      (bind _skeletalmesh_preview_ (Variables|Default|GetSkeletalMesh%28Preview%29)
        (:then
          (Rendering|SetVisibility _skeletalmesh_preview_ false true))
        (:else)))
    (:then_1
      (Variables|Default|SetbBeginPlay false))))

(event Collision|EventActorBeginOverlap
  (params (OtherActor :type Actor%20Object%20Reference)))

(event EventTick
  (params (DeltaSeconds :type Float%20%28single-precision%29)))

(fn ConstructionScript
  (CallFunction|Init false))