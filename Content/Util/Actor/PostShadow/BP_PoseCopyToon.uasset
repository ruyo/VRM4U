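; Pose-copy actor that applies post-process-style toon shading and shadows to a VRM or skeletal mesh character.
; On Init, the target mesh gets MI_BaseLight dynamic materials, while a translucent copy follows its pose via master pose with MI_PostToon.
; Both copy source material instance parameters and M_VrmNone slots, then receive shadow, highlight and per-material-index overrides.
; It also sets lighting channels, per-bone motion blur and a debug toggle hiding the toon layer.
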(event EventBeginPlay
  (|CallParentFunction) ; This node is disabled and will not be called.\nDrag off pins to build functionality.
)

(event Collision|EventActorBeginOverlap
  (params (OtherActor :type Actor%20Object%20Reference))
  (|CallParentFunction OtherActor) ; This node is disabled and will not be called.\nDrag off pins to build functionality.
)

(event EventTick
  (params (DeltaSeconds :type Float%20%28single-precision%29))
  (|CallParentFunction DeltaSeconds) ; This node is disabled and will not be called.\nDrag off pins to build functionality.
)

(event EventInit
  (params (dummy :type Boolean))
  (bind _materialno_normaltocam (Variables|Default|GetMaterialNo_NormalToCam))
  (bind _vrmposeablemesh_translucent (Variables|Default|GetVrmPoseableMesh_translucent))
  (bind _materialno_highlightcolor (Variables|Default|GetMaterialNo_HighLightColor))
  (bind _materialno_forceshadow (Variables|Default|GetMaterialNo_ForceShadow))
  (bind _lightchannel (Variables|Default|GetLightChannel))
  (bind _vrmposeablemesh_translucent_2 (Variables|Default|GetVrmPoseableMesh_translucent))
  (bind _skeletalmesh (Variables|Default|GetSkeletalMesh))
  (bind _skeletalmesh_2 (Variables|Default|GetSkeletalMesh))
  (|CallParentFunction false)
  (Utilities|FlowControl|Sequence
    (:then_0
      (Variables|Default|SetTargetMeshForLight (Variables|Default|GetVrmPoseableMesh))
      (Variables|/Script/Engine.SkinnedMeshComponent|GetSkeletalMesh _skeletalmesh
        (:then
          (Variables|Default|SetTargetMeshForLight _skeletalmesh))
        (:else)))
    (:then_1
      (Utilities|FlowControl|Sequence
        (:then_0
          (for (_ _array_index) (Rendering|Material|GetMaterials (Variables|Default|GetTargetMeshForLight))
            (bind _returnvalue (Rendering|Material|CreateDynamicMaterialInstance "/VRM4U/Util/Actor/PostShadow/MI_BaseLight.MI_BaseLight" "None" :!class /Script/Engine.KismetMaterialLibrary))
            (Rendering|Material|SetMaterial (Variables|Default|GetTargetMeshForLight) _array_index _returnvalue)))
        (:then_1
          (Class|SkinnedMeshComponent|SetSkeletalMesh _vrmposeablemesh_translucent (Variables|/Script/Engine.SkinnedMeshComponent|GetSkeletalMesh (Variables|Default|GetTargetMeshForLight)) true)
          (Class|SkinnedMeshComponent|SetMasterPoseComponent _vrmposeablemesh_translucent (Variables|Default|GetTargetMeshForLight) false)
          (for (_ _array_index_2) (Rendering|Material|GetMaterials _vrmposeablemesh_translucent_2)
            (bind _returnvalue_2 (Rendering|Material|CreateDynamicMaterialInstance "/VRM4U/Util/Actor/PostShadow/MI_PostToon.MI_PostToon" "None" :!class /Script/Engine.KismetMaterialLibrary))
            (Rendering|Material|SetMaterial _vrmposeablemesh_translucent_2 _array_index_2 _returnvalue_2)))
        (:then_2
          (bind _tmpcomponent (Variables|Default|GetTmpComponent)
            (:then
              (for (_array_element _array_index_3) (Rendering|Material|GetMaterials _tmpcomponent)
                (bind _returnvalue_3 (Rendering|Material|GetBaseMaterial _array_element))
                (if (or (== _array_element "/VRM4U/MaterialUtil/MToonUtil/M_VrmNone.M_VrmNone") (== _returnvalue_3 "/VRM4U/MaterialUtil/MToonUtil/M_VrmNone.M_VrmNone"))
                  (Rendering|Material|SetMaterial (Variables|Default|GetVrmPoseableMesh_translucent) _array_index_3 "/VRM4U/MaterialUtil/MToonUtil/M_VrmNone.M_VrmNone"))))
            (:else)))))
    (:then_2
      (Utilities|FlowControl|Sequence
        (:then_0
          (Utilities|FlowControl|Sequence
            (:then_0
              (Variables|Default|SetBaseMeshForMaterial (Variables|Default|GetTmpComponent))
              (Variables|/Script/Engine.SkinnedMeshComponent|GetSkeletalMesh _skeletalmesh_2
                (:then
                  (Variables|Default|SetBaseMeshForMaterial _skeletalmesh_2))
                (:else)))
            (:then_1
              (for (_array_element_2 _array_index_4) (Rendering|Material|GetMaterials (Variables|Default|GetBaseMeshForMaterial))
                (Variables|Default|SetNewVar_0 _array_element_2)
                (Utilities|Casting|CastToMaterialInstanceDynamic _array_element_2
                  (:then
                    (Variables|Default|SetNewVar_0 (.MaterialInterface (Utilities|Struct|BreakSkeletalMaterial (Utilities|Array|Get(acopy) (Variables|/Script/Engine.SkeletalMesh|GetMaterials (Variables|/Script/Engine.SkinnedMeshComponent|GetSkeletalMesh (Variables|Default|GetBaseMeshForMaterial))) _array_index_4)))))
                  (:CastFailed
                    _))
                (bind _asmaterial_instance_constant (Utilities|Casting|CastToMaterialInstanceConstant (Variables|Default|GetNewVar_0)))
                (Utilities|FlowControl|Sequence
                  (:then_0
                    (for _array_element_3 (Variables|/Script/Engine.MaterialInstance|GetTextureParameterValues _asmaterial_instance_constant)
                      (Rendering|Material|SetTextureParameterValue (.AsMaterial%20Instance%20Dynamic (Utilities|Casting|CastToMaterialInstanceDynamic (Utilities|Array|Get(acopy) (Rendering|Material|GetMaterials (Variables|Default|GetTargetMeshForLight)) _array_index_4))) (.Name (Utilities|Struct|BreakMaterialParameterInfo (.ParameterInfo (Utilities|Struct|BreakTextureParameterValue _array_element_3)))) (.ParameterValue (Utilities|Struct|BreakTextureParameterValue _array_element_3)))))
                  (:then_1
                    (for _array_element_4 (Variables|/Script/Engine.MaterialInstance|GetVectorParameterValues _asmaterial_instance_constant)
                      (Rendering|Material|SetVectorParameterValue (.AsMaterial%20Instance%20Dynamic (Utilities|Casting|CastToMaterialInstanceDynamic (Utilities|Array|Get(acopy) (Rendering|Material|GetMaterials (Variables|Default|GetTargetMeshForLight)) _array_index_4))) (.Name (Utilities|Struct|BreakMaterialParameterInfo (.ParameterInfo (Utilities|Struct|BreakVectorParameterValue _array_element_4)))) (.ParameterValue (Utilities|Struct|BreakVectorParameterValue _array_element_4)) :!class /Script/Engine.MaterialInstanceDynamic)))
                  (:then_2
                    (for _array_element_5 (Variables|/Script/Engine.MaterialInstance|GetScalarParameterValues _asmaterial_instance_constant)
                      (Rendering|Material|SetScalarParameterValue (.AsMaterial%20Instance%20Dynamic (Utilities|Casting|CastToMaterialInstanceDynamic (Utilities|Array|Get(acopy) (Rendering|Material|GetMaterials (Variables|Default|GetTargetMeshForLight)) _array_index_4))) (.Name (Utilities|Struct|BreakMaterialParameterInfo (.ParameterInfo (Utilities|Struct|BreakScalarParameterValue _array_element_5)))) (.ParameterValue (Utilities|Struct|BreakScalarParameterValue _array_element_5)) :!class /Script/Engine.MaterialInstanceDynamic)))
                  (:then_3
                    (Rendering|Material|SetScalarParameterValue (.AsMaterial%20Instance%20Dynamic (Utilities|Casting|CastToMaterialInstanceDynamic (Utilities|Array|Get(acopy) (Rendering|Material|GetMaterials (Variables|Default|GetTargetMeshForLight)) _array_index_4))) "DebugShadow" (Math|Float|SelectFloat 1.0 0.0 (Variables|Default|GetbDebugDrawShadow)) :!class /Script/Engine.MaterialInstanceDynamic)
                    (Rendering|Material|SetScalarParameterValue (.AsMaterial%20Instance%20Dynamic (Utilities|Casting|CastToMaterialInstanceDynamic (Utilities|Array|Get(acopy) (Rendering|Material|GetMaterials (Variables|Default|GetTargetMeshForLight)) _array_index_4))) "ShadowRange" (Variables|Default|GetShadowRange) :!class /Script/Engine.MaterialInstanceDynamic)
                    (Rendering|Material|SetScalarParameterValue (.AsMaterial%20Instance%20Dynamic (Utilities|Casting|CastToMaterialInstanceDynamic (Utilities|Array|Get(acopy) (Rendering|Material|GetMaterials (Variables|Default|GetVrmPoseableMesh_translucent)) _array_index_4))) "HighRange" (Variables|Default|GetHighLightRange) :!class /Script/Engine.MaterialInstanceDynamic)
                    (Rendering|Material|SetVectorParameterValue (.AsMaterial%20Instance%20Dynamic (Utilities|Casting|CastToMaterialInstanceDynamic (Utilities|Array|Get(acopy) (Rendering|Material|GetMaterials (Variables|Default|GetTargetMeshForLight)) _array_index_4))) "HighLightColor" (Variables|Default|GetHighLightColor) :!class /Script/Engine.MaterialInstanceDynamic)
                    (Rendering|Material|SetVectorParameterValue (.AsMaterial%20Instance%20Dynamic (Utilities|Casting|CastToMaterialInstanceDynamic (Utilities|Array|Get(acopy) (Rendering|Material|GetMaterials (Variables|Default|GetTargetMeshForLight)) _array_index_4))) "MRSA" (Variables|Default|GetMRSA) :!class /Script/Engine.MaterialInstanceDynamic)
                    (Rendering|Material|SetScalarParameterValue (.AsMaterial%20Instance%20Dynamic (Utilities|Casting|CastToMaterialInstanceDynamic (Utilities|Array|Get(acopy) (Rendering|Material|GetMaterials (Variables|Default|GetTargetMeshForLight)) _array_index_4))) "bUseDirectionalLightDot" (select (Variables|Default|GetbUseLightDirectionDotShadow) 1.0 0.0) :!class /Script/Engine.MaterialInstanceDynamic)))))))
        (:then_1
          (Utilities|FlowControl|Sequence
            (:then_0
              (bind _keys (Utilities|Map|Keys _materialno_normaltocam))
              (for _array_element_6 _keys
                (Rendering|Material|SetScalarParameterValue (.AsMaterial%20Instance%20Dynamic (Utilities|Casting|CastToMaterialInstanceDynamic (Utilities|Array|Get(acopy) (Rendering|Material|GetMaterials (Variables|Default|GetVrmPoseableMesh_translucent)) _array_element_6))) "NormalToCameraMat" (.Value (Utilities|Map|Find _materialno_normaltocam _array_element_6)) :!class /Script/Engine.MaterialInstanceDynamic)))
            (:then_1
              (bind _keys_2 (Utilities|Map|Keys _materialno_highlightcolor))
              (for _array_element_7 _keys_2
                (Rendering|Material|SetVectorParameterValue (.AsMaterial%20Instance%20Dynamic (Utilities|Casting|CastToMaterialInstanceDynamic (Utilities|Array|Get(acopy) (Rendering|Material|GetMaterials (Variables|Default|GetVrmPoseableMesh_translucent)) _array_element_7))) "HighLightColor" (.Value (Utilities|Map|Find _materialno_highlightcolor _array_element_7)) :!class /Script/Engine.MaterialInstanceDynamic)))
            (:then_2
              (bind _keys_3 (Utilities|Map|Keys _materialno_forceshadow))
              (for _array_element_8 _keys_3
                (Utilities|Map|Add _materialno_forceshadow _array_element_8 (Math|Integer|Clamp(Integer) (.Value (Utilities|Map|Find _materialno_forceshadow _array_element_8)) 0 2))
                (Rendering|Material|SetScalarParameterValue (.AsMaterial%20Instance%20Dynamic (Utilities|Casting|CastToMaterialInstanceDynamic (Utilities|Array|Get(acopy) (Rendering|Material|GetMaterials (Variables|Default|GetTargetMeshForLight)) _array_element_8))) "ForceShadow" (Utilities|Select :Index (Math|Integer|Clamp(Integer) (.Value (Utilities|Map|Find _materialno_forceshadow _array_element_8)) 0 2) :Option%200 -1.0 :Option%201 0.0 :Option%202 1.0) :!class /Script/Engine.MaterialInstanceDynamic)))))))
    (:then_4
      (Rendering|SetVisibility (Variables|Default|GetVrmPoseableMesh_translucent) (not (Variables|Default|GetbDebugDrawRaw)) false))
    (:then_5
      (Class|VrmBPFunctionLibrary|VRMSetLightingChannelPrim (Variables|Default|GetTargetMeshForLight) (Utilities|Array|Get(acopy) _lightchannel) (Utilities|Array|Get(acopy) _lightchannel 1) (Utilities|Array|Get(acopy) _lightchannel 2)))
    (:then_6
      (Class|VrmBPFunctionLibrary|VRMSetPerBoneMotionBlur (Variables|Default|GetVrmPoseableMesh_translucent) (Variables|Default|GetbUsePerBoneMotionBlur)))))

(fn ConstructionScript
  (|CallParentFunction))