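; Pose-copy actor for VRM characters that gives a duplicate poseable mesh post-shadow materials.
; On Init it copies the source's skeletal mesh and master pose component, and takes the render target from BP_PostShadowCapture if no shadow texture is set.
; With auto-generation on, it creates dynamic materials per slot from custom, override or default parents, copying MToon textures.
; When those materials already exist, Init only updates shadow and SSAO ranges.
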(event EventBeginPlay
  (|CallParentFunction) ; This node is disabled and will not be called.\nDrag off pins to build functionality.
)

(event Collision|EventActorBeginOverlap
  (params (OtherActor :type Actor%20Object%20Reference))
  (|CallParentFunction OtherActor) ; This node is disabled and will not be called.\nDrag off pins to build functionality.
)

(event EventTick
  (params (DeltaSeconds :type Float%20%28single-precision%29))
  (|CallParentFunction DeltaSeconds) ; This node is disabled and will not be called.\nDrag off pins to build functionality.
)

(event EventInit
  (params (dummy :type Boolean))
  (bind _overridebase (Variables|Default|GetOverrideBase))
  (|CallParentFunction false)
  (Utilities|FlowControl|Sequence
    (:then_0
      (Class|SkinnedMeshComponent|SetSkeletalMesh (Variables|Default|GetVrmPoseableMeshPostShadow) (Variables|/Script/Engine.SkinnedMeshComponent|GetSkeletalMesh (Variables|Default|GetVrmPoseableMesh)) true)
      (Class|SkinnedMeshComponent|SetMasterPoseComponent (Variables|Default|GetVrmPoseableMeshPostShadow) (Variables|/Script/Engine.SkinnedMeshComponent|GetMasterPoseComponent (Variables|Default|GetVrmPoseableMesh)) true))
    (:then_1
      (Utilities|FlowControl|Sequence
        (:then_1
          (Variables|Default|GetPostShadowTexture
            (:then)
            (:else
              (bind _outactors (Actor|GetAllActorsOfClass "/VRM4U/Util/Actor/PostShadow/old/BP_PostShadowCapture.BP_PostShadowCapture_C"))
              (if (> (Utilities|Array|Length _outactors) 0)
                (Variables|Default|SetPostShadowTexture (Variables|/VRM4U/Util/Actor/PostShadow/old/BP_PostShadowCapture.BP_PostShadowCapture_C|GetRenderTarget (Utilities|Array|Get(acopy) _outactors)))))))
        (:then_3
          (if (Variables|Default|GetbAutoGenerateMaterial)
            (if (> (Utilities|Array|Length (Variables|Default|GetMaterialList)) 0)
              (for _array_element (Variables|Default|GetMaterialList)
                (Rendering|Material|SetScalarParameterValue _array_element "PostShadow_Shadow_Range" (Variables|Default|GetShadowRange) :!class /Script/Engine.MaterialInstanceDynamic)
                (Rendering|Material|SetScalarParameterValue _array_element "PostShadow_SSAO_Range" (Variables|Default|GetSSAORange) :!class /Script/Engine.MaterialInstanceDynamic))
              (else
                (for (_array_element_2 _array_index) (Rendering|Material|GetMaterials (Variables|Default|GetVrmPoseableMesh))
                  (Utilities|FlowControl|Sequence
                    (:then_0
                      (bind _returnvalue (Rendering|Material|CreateDynamicMaterialInstance (select (.ReturnValue (Utilities|Map|Find (Variables|Default|GetMaterialCustom) _array_index)) (.Value (Utilities|Map|Find (Variables|Default|GetMaterialCustom) _array_index)) (select (Utilities|IsValid _overridebase) _overridebase "/VRM4U/Util/Actor/PostShadow/old/sub/MI_PostShadowParent.MI_PostShadowParent")) "None" :!class /Script/Engine.KismetMaterialLibrary))
                      (Rendering|Material|SetMaterial (Variables|Default|GetVrmPoseableMeshPostShadow) _array_index _returnvalue)
                      (Utilities|Array|Add (Variables|Default|GetMaterialList) _returnvalue))
                    (:then_1
                      (bind _asmaterial_instance (Utilities|Casting|CastToMaterialInstance _array_element_2))
                      (for _array_element_3 (Variables|/Script/Engine.MaterialInstance|GetTextureParameterValues _asmaterial_instance)
                        (Utilities|FlowControl|Sequence
                          (:then_0
                            (Utilities|FlowControl|Sequence
                              (:then_0
                                ;[1 1 1] Shadow Texture
                                (Rendering|Material|SetTextureParameterValue _returnvalue "PostShadowTexture" (Variables|Default|GetPostShadowTexture)))
                              (:then_1
                                ;[1 1 1] copy params
                                (Utilities|FlowControl|Sequence
                                  (:then_0
                                    (if (Utilities|Name|Equal(Name) (.Name (Utilities|Struct|BreakMaterialParameterInfo (.ParameterInfo (Utilities|Struct|BreakTextureParameterValue _array_element_3)))) "gltf_tex_diffuse")
                                      (Rendering|Material|SetTextureParameterValue _returnvalue (.Name (Utilities|Struct|BreakMaterialParameterInfo (.ParameterInfo (Utilities|Struct|BreakTextureParameterValue _array_element_3)))) (.AsTexture%202D (Utilities|Casting|CastToTexture2D (.ParameterValue (Utilities|Struct|BreakTextureParameterValue _array_element_3)))))
                                      (Rendering|Material|SetTextureParameterValue _returnvalue "mtoon_tex_ShadeTexture" (.AsTexture%202D (Utilities|Casting|CastToTexture2D (.ParameterValue (Utilities|Struct|BreakTextureParameterValue _array_element_3)))))))
                                  (:then_1
                                    (if (Utilities|Name|Equal(Name) (.Name (Utilities|Struct|BreakMaterialParameterInfo (.ParameterInfo (Utilities|Struct|BreakTextureParameterValue _array_element_3)))) "mtoon_tex_BumpMap")
                                      (Rendering|Material|SetTextureParameterValue _returnvalue (.Name (Utilities|Struct|BreakMaterialParameterInfo (.ParameterInfo (Utilities|Struct|BreakTextureParameterValue _array_element_3)))) (.AsTexture%202D (Utilities|Casting|CastToTexture2D (.ParameterValue (Utilities|Struct|BreakTextureParameterValue _array_element_3)))))))
                                  (:then_2
                                    (if (Utilities|Name|Equal(Name) (.Name (Utilities|Struct|BreakMaterialParameterInfo (.ParameterInfo (Utilities|Struct|BreakTextureParameterValue _array_element_3)))) "mtoon_tex_SphereAdd")
                                      (Rendering|Material|SetTextureParameterValue _returnvalue (.Name (Utilities|Struct|BreakMaterialParameterInfo (.ParameterInfo (Utilities|Struct|BreakTextureParameterValue _array_element_3)))) (.AsTexture%202D (Utilities|Casting|CastToTexture2D (.ParameterValue (Utilities|Struct|BreakTextureParameterValue _array_element_3))))))))))))))))))))))))

(fn ConstructionScript
  (|CallParentFunction))