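; Post-shadow capture actor that renders the player or editor camera's view into a render target, created on demand.
; Construction configures two SceneCaptures, filling show-only lists from TargetForRenderTarget (optional for the main capture).
; Tick and VrmCameraCheck camera-move events align the actor and both FOVs to the camera.
; It also speeds up exposure adaptation on UE 4.25+, optionally applies AO, and can show a debug cube.
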(event Custom|CustomEvent_0
  (params (dummy :type Boolean))
  (bind (_transform _fovdegree) (Class|VrmBPFunctionLibrary|VRMGetCameraTransform 0 false))
  (bind (_major _minor) (Class|VrmBPFunctionLibrary|VRMGetUEVersion))
  (bind _scenecapturecomponent2d (Variables|Default|GetSceneCaptureComponent2D))
  (bind _scenecapturecomponent2d1 (Variables|Default|GetSceneCaptureComponent2D1))
  (bind _scenecapturecomponent2d_2 (Variables|Default|GetSceneCaptureComponent2D))
  (bind _scenecapturecomponent2d_3 (Variables|Default|GetSceneCaptureComponent2D))
  (bind _vrmcameracheck (Variables|Default|GetVrmCameraCheck))
  (bind _targetforrendertarget (Variables|Default|GetTargetForRenderTarget))
  (bind _postprocesssettings (Variables|/Script/Engine.SceneCaptureComponent2D|GetPostProcessSettings _scenecapturecomponent2d))
  (Utilities|FlowControl|Sequence
    (:then_0
      (Utilities|FlowControl|Sequence
        (:then_0
          (Variables|Default|GetRenderTarget
            (:then)
            (:else
              (bind _returnvalue (Class|VrmBPFunctionLibrary|VRMCreateRenderTarget2D 2048 2048 "RTF_RGBA8" "(R=0.000000,G=0.000000,B=0.000000,A=1.000000)"))
              (Variables|Default|SetRenderTarget _returnvalue)
              (Variables|/Script/Engine.SceneCaptureComponent2D|SetTextureTarget (Variables|Default|GetSceneCaptureComponent2D) _returnvalue))))
        (:then_1
          (if (> (Utilities|Array|Length _targetforrendertarget) 0)
            (for _array_element _targetforrendertarget
              (Utilities|Array|AddUnique (Variables|/Script/Engine.SceneCaptureComponent|GetShowOnlyActors (Variables|Default|GetSceneCaptureComponent2D1)) _array_element)
              (Utilities|FlowControl|Sequence
                (:then_0
                  (if (Variables|Default|GetbUseActorList)
                    (Utilities|Array|AddUnique (Variables|/Script/Engine.SceneCaptureComponent|GetShowOnlyActors _scenecapturecomponent2d_2) _array_element)
                    (Variables|/Script/Engine.SceneCaptureComponent|SetPrimitiveRenderMode _scenecapturecomponent2d_2 "PRM_UseShowOnlyList")))))
            (else
              (bind _output_get (Variables|/Script/Engine.SceneCaptureComponent|SetbCaptureEveryFrame _scenecapturecomponent2d1 false))
              (Variables|/Script/Engine.SceneCaptureComponent|SetbCaptureOnMovement _scenecapturecomponent2d1 _output_get))))
        (:then_2
          (if (Variables|Default|GetbUseActorList)
            (Variables|/Script/Engine.SceneCaptureComponent|SetPrimitiveRenderMode _scenecapturecomponent2d_3 "PRM_UseShowOnlyList")
            (Utilities|Array|Add (Variables|/Script/Engine.SceneCaptureComponent|GetShowFlagSettings _scenecapturecomponent2d_3) (Utilities|Struct|MakeEngineShowFlagsSetting "AtmosphericFog"))))))
    (:then_1
      (EventDispatchers|BindEventtoOnCameraMove _vrmcameracheck (delegate Custom|CustomEvent_1))
      (Class|VrmCameraCheckComponent|SetCameraCheck _vrmcameracheck true)
      (Utilities|FlowControl|Sequence
        (:then_0
          (if (Variables|Default|GetbShowDebug)
            (bind _rendertarget (Variables|Default|GetRenderTarget)
              (:then
                (bind _returnvalue_2 (Rendering|Material|CreateDynamicMaterialInstance (Variables|Default|GetCube) 0 0 "None" :!class /Script/Engine.PrimitiveComponent))
                (Rendering|Material|SetTextureParameterValue _returnvalue_2 "Texture" _rendertarget))
              (:else))
            (else
              (bind _cube (Variables|Default|GetCube)
                (:then
                  (Components|DestroyComponent _cube))
                (:else)))))
        (:then_1
          (if (or (>= _major 5) (and (== _major 4) (>= _minor 25)))
            (bind _structout (Utilities|Struct|SetmembersinPostProcessSettings _postprocesssettings 1e+02 1e+02))
            (Utilities|Struct|SetmembersinPostProcessSettings _structout 1e+02 1e+02)))
        (:then_2
          (if (Variables|Default|GetbUseAO)
            (Utilities|Struct|SetmembersinPostProcessSettings _postprocesssettings (Variables|Default|GetAO_Intensity) (Variables|Default|GetAO_Radius))))))
    (:then_2
      (Utilities|FlowControl|Sequence
        (:then_0
          (Transformation|SetActorTransform self _transform)
          (Variables|/Script/Engine.SceneCaptureComponent2D|SetFOVAngle (Variables|Default|GetSceneCaptureComponent2D) _fovdegree)
          (Variables|/Script/Engine.SceneCaptureComponent2D|SetFOVAngle (Variables|Default|GetSceneCaptureComponent2D1) _fovdegree))
        (:then_1
          (Variables|Default|GetCube
            (:then
              (Transformation|SetWorldTransform (Variables|Default|GetCube) (Math|Transform|ComposeTransforms (Math|Transform|MakeTransform "330.000000,-100.000000, 0") _transform) false false))
            (:else)))))))

(event Custom|CustomEvent_1
  (bind (_transform _fovdegree) (Class|VrmBPFunctionLibrary|VRMGetCameraTransform 0 false))
  (Utilities|FlowControl|Sequence
    (:then_0
      (Transformation|SetActorTransform self _transform)
      (Variables|/Script/Engine.SceneCaptureComponent2D|SetFOVAngle (Variables|Default|GetSceneCaptureComponent2D) _fovdegree)
      (Variables|/Script/Engine.SceneCaptureComponent2D|SetFOVAngle (Variables|Default|GetSceneCaptureComponent2D1) _fovdegree))
    (:then_1
      (Variables|Default|GetCube
        (:then
          (Transformation|SetWorldTransform (Variables|Default|GetCube) (Math|Transform|ComposeTransforms (Math|Transform|MakeTransform "330.000000,-100.000000, 0") _transform) false false))
        (:else)))))

(event EventBeginPlay
  (bind (_major _minor) (Class|VrmBPFunctionLibrary|VRMGetUEVersion))
  (bind _scenecapturecomponent2d (Variables|Default|GetSceneCaptureComponent2D))
  (bind _vrmcameracheck (Variables|Default|GetVrmCameraCheck))
  (bind _postprocesssettings (Variables|/Script/Engine.SceneCaptureComponent2D|GetPostProcessSettings _scenecapturecomponent2d))
  (EventDispatchers|BindEventtoOnCameraMove _vrmcameracheck (delegate Custom|CustomEvent_1))
  (Class|VrmCameraCheckComponent|SetCameraCheck _vrmcameracheck true)
  (Utilities|FlowControl|Sequence
    (:then_0
      (if (Variables|Default|GetbShowDebug)
        (bind _rendertarget (Variables|Default|GetRenderTarget)
          (:then
            (bind _returnvalue (Rendering|Material|CreateDynamicMaterialInstance (Variables|Default|GetCube) 0 0 "None" :!class /Script/Engine.PrimitiveComponent))
            (Rendering|Material|SetTextureParameterValue _returnvalue "Texture" _rendertarget))
          (:else))
        (else
          (bind _cube (Variables|Default|GetCube)
            (:then
              (Components|DestroyComponent _cube))
            (:else)))))
    (:then_1
      (if (or (>= _major 5) (and (== _major 4) (>= _minor 25)))
        (bind _structout (Utilities|Struct|SetmembersinPostProcessSettings _postprocesssettings 1e+02 1e+02))
        (Utilities|Struct|SetmembersinPostProcessSettings _structout 1e+02 1e+02)))
    (:then_2
      (if (Variables|Default|GetbUseAO)
        (Utilities|Struct|SetmembersinPostProcessSettings _postprocesssettings (Variables|Default|GetAO_Intensity) (Variables|Default|GetAO_Radius))))))

(event Collision|EventActorBeginOverlap
  (params (OtherActor :type Actor%20Object%20Reference)))

(event EventTick
  (params (DeltaSeconds :type Float%20%28single-precision%29))
  (bind (_transform _fovdegree) (Class|VrmBPFunctionLibrary|VRMGetCameraTransform 0 false))
  (Transformation|SetActorTransform self _transform)
  (Variables|/Script/Engine.SceneCaptureComponent2D|SetFOVAngle (Variables|Default|GetSceneCaptureComponent2D) _fovdegree)
  (Variables|/Script/Engine.SceneCaptureComponent2D|SetFOVAngle (Variables|Default|GetSceneCaptureComponent2D1) _fovdegree))

(fn ConstructionScript
  (CallFunction|CustomEvent0 false))