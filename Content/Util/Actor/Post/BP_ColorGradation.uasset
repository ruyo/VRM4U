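; BP_ColorGradation is an actor that applies a color gradation post-process effect through a dynamic instance of MI_ColorGradation.
; BeginPlay and the Construction Script, via Apply, share one setup that disables the effect when ignored or on mobile without MobileHDR.
; Otherwise it registers the material as a blendable and feeds it contrast, inversion, blend and circle shape settings, plus indexed position and color parameters from arrays.
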(event Custom|Apply
  (params (dummy :type Boolean))
  (bind _postprocess (Variables|Default|GetPostProcess))
  (bind _returnvalue (Development|GetConsoleVariableIntValue "r.MobileHDR"))
  (if (or (and (.IsMobile (Class|VrmBPFunctionLibrary|VRMGetMobileMode)) (== _returnvalue 0)) (Variables|Default|GetbIgnore))
    (Variables|/Script/Engine.PostProcessComponent|SetbEnabled _postprocess false)
    (else
      (Variables|/Script/Engine.PostProcessComponent|SetbEnabled _postprocess true)
      (Variables|/Script/Engine.PostProcessComponent|SetPriority _postprocess (Variables|Default|GetPriority))
      (Utilities|FlowControl|Sequence
        (:then_0
          (bind _returnvalue_2 (Rendering|Material|CreateDynamicMaterialInstance "/VRM4U/Util/Actor/Post/sub/MI_ColorGradation.MI_ColorGradation" "None" :!class /Script/Engine.KismetMaterialLibrary))
          (Variables|Develop|SetNewVar_1 _returnvalue_2)
          (Utilities|Struct|SetmembersinPostProcessSettings (Variables|/Script/Engine.PostProcessComponent|GetSettings (Variables|Default|GetPostProcess)) (Utilities|Struct|MakeWeightedBlendables (Utilities|Array|MakeArray (Utilities|Struct|MakeWeightedBlendable 1.0 (Variables|Develop|GetNewVar_1))))))
        (:then_1
          (Rendering|Material|SetScalarParameterValue (Variables|Develop|GetNewVar_1) "Inv" (Math|Float|SelectFloat 1.0 0.0 (Variables|Default|GetbSubColor)) :!class /Script/Engine.MaterialInstanceDynamic)
          (Rendering|Material|SetScalarParameterValue (Variables|Develop|GetNewVar_1) "pow" (Variables|Default|GetCurveContrast) :!class /Script/Engine.MaterialInstanceDynamic)
          (Rendering|Material|SetScalarParameterValue (Variables|Develop|GetNewVar_1) "SizeOffset" (Variables|Default|GetSizeOffset) :!class /Script/Engine.MaterialInstanceDynamic))
        (:then_2
          (for (_array_element _array_index) (Variables|Default|Getposition)
            (Rendering|Material|SetVectorParameterValue (Variables|Develop|GetNewVar_1) (Utilities|String|StringToName (Utilities|String|Append "pos" (Utilities|String|ToString(Integer) (+ _array_index 1)))) (Utilities|Struct|MakeLinearColor (.X (Math|Vector|BreakVector _array_element)) (.Y (Math|Vector|BreakVector _array_element)) (.Z (Math|Vector|BreakVector _array_element)) 0.0) :!class /Script/Engine.MaterialInstanceDynamic)
            (Rendering|Material|SetVectorParameterValue (Variables|Develop|GetNewVar_1) (Utilities|String|StringToName (Utilities|String|Append "color" (Utilities|String|ToString(Integer) (+ _array_index 1)))) (select (Utilities|Array|Get(acopy) (Variables|Default|GetbIgnoreColor) _array_index) (Math|Color|MakeColor 0.0 0.0 0.0 0.0) (Utilities|Array|Get(acopy) (Variables|Default|Getcolor) _array_index)) :!class /Script/Engine.MaterialInstanceDynamic)
            (Rendering|Material|SetScalarParameterValue (Variables|Develop|GetNewVar_1) "BlendRate" (Variables|Default|GetBlendRate) :!class /Script/Engine.MaterialInstanceDynamic)
            (Rendering|Material|SetVectorParameterValue (Variables|Develop|GetNewVar_1) "CircleScale" (Variables|Default|GetCircleScaleXY) :!class /Script/Engine.MaterialInstanceDynamic)))))))

(event EventBeginPlay
  (bind _postprocess (Variables|Default|GetPostProcess))
  (bind _returnvalue (Development|GetConsoleVariableIntValue "r.MobileHDR"))
  (if (or (and (.IsMobile (Class|VrmBPFunctionLibrary|VRMGetMobileMode)) (== _returnvalue 0)) (Variables|Default|GetbIgnore))
    (Variables|/Script/Engine.PostProcessComponent|SetbEnabled _postprocess false)
    (else
      (Variables|/Script/Engine.PostProcessComponent|SetbEnabled _postprocess true)
      (Variables|/Script/Engine.PostProcessComponent|SetPriority _postprocess (Variables|Default|GetPriority))
      (Utilities|FlowControl|Sequence
        (:then_0
          (bind _returnvalue_2 (Rendering|Material|CreateDynamicMaterialInstance "/VRM4U/Util/Actor/Post/sub/MI_ColorGradation.MI_ColorGradation" "None" :!class /Script/Engine.KismetMaterialLibrary))
          (Variables|Develop|SetNewVar_1 _returnvalue_2)
          (Utilities|Struct|SetmembersinPostProcessSettings (Variables|/Script/Engine.PostProcessComponent|GetSettings (Variables|Default|GetPostProcess)) (Utilities|Struct|MakeWeightedBlendables (Utilities|Array|MakeArray (Utilities|Struct|MakeWeightedBlendable 1.0 (Variables|Develop|GetNewVar_1))))))
        (:then_1
          (Rendering|Material|SetScalarParameterValue (Variables|Develop|GetNewVar_1) "Inv" (Math|Float|SelectFloat 1.0 0.0 (Variables|Default|GetbSubColor)) :!class /Script/Engine.MaterialInstanceDynamic)
          (Rendering|Material|SetScalarParameterValue (Variables|Develop|GetNewVar_1) "pow" (Variables|Default|GetCurveContrast) :!class /Script/Engine.MaterialInstanceDynamic)
          (Rendering|Material|SetScalarParameterValue (Variables|Develop|GetNewVar_1) "SizeOffset" (Variables|Default|GetSizeOffset) :!class /Script/Engine.MaterialInstanceDynamic))
        (:then_2
          (for (_array_element _array_index) (Variables|Default|Getposition)
            (Rendering|Material|SetVectorParameterValue (Variables|Develop|GetNewVar_1) (Utilities|String|StringToName (Utilities|String|Append "pos" (Utilities|String|ToString(Integer) (+ _array_index 1)))) (Utilities|Struct|MakeLinearColor (.X (Math|Vector|BreakVector _array_element)) (.Y (Math|Vector|BreakVector _array_element)) (.Z (Math|Vector|BreakVector _array_element)) 0.0) :!class /Script/Engine.MaterialInstanceDynamic)
            (Rendering|Material|SetVectorParameterValue (Variables|Develop|GetNewVar_1) (Utilities|String|StringToName (Utilities|String|Append "color" (Utilities|String|ToString(Integer) (+ _array_index 1)))) (select (Utilities|Array|Get(acopy) (Variables|Default|GetbIgnoreColor) _array_index) (Math|Color|MakeColor 0.0 0.0 0.0 0.0) (Utilities|Array|Get(acopy) (Variables|Default|Getcolor) _array_index)) :!class /Script/Engine.MaterialInstanceDynamic)
            (Rendering|Material|SetScalarParameterValue (Variables|Develop|GetNewVar_1) "BlendRate" (Variables|Default|GetBlendRate) :!class /Script/Engine.MaterialInstanceDynamic)
            (Rendering|Material|SetVectorParameterValue (Variables|Develop|GetNewVar_1) "CircleScale" (Variables|Default|GetCircleScaleXY) :!class /Script/Engine.MaterialInstanceDynamic)))))))

(fn ConstructionScript
  (CallFunction|Apply false))