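; BP_PostCenterBlur is a post-effect actor that configures a center blur material, judging by its name and parameters.
; On Init it runs the parent Init, then copies its center, density, radius, rotation, scale and step variables into scalar parameters on MaterialDynamic.
; The values are pushed only in Init, as BeginPlay, overlap and Tick are disabled stubs and the construction script only calls the parent.
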(event EventBeginPlay
  (|CallParentFunction) ; This node is disabled and will not be called.\nDrag off pins to build functionality.
)

(event Collision|EventActorBeginOverlap
  (params (OtherActor :type Actor%20Object%20Reference))
  (|CallParentFunction OtherActor) ; This node is disabled and will not be called.\nDrag off pins to build functionality.
)

(event EventTick
  (params (DeltaSeconds :type Float%20%28single-precision%29))
  (|CallParentFunction DeltaSeconds) ; This node is disabled and will not be called.\nDrag off pins to build functionality.
)

(event EventInit
  (params (Dummy :type Boolean))
  (bind _materialdynamic (Variables|Default|GetMaterialDynamic))
  (|CallParentFunction false)
  (Rendering|Material|SetScalarParameterValue _materialdynamic "CenterX" (Variables|Default|GetCenterX) :!class /Script/Engine.MaterialInstanceDynamic)
  (Rendering|Material|SetScalarParameterValue _materialdynamic "CenterY" (Variables|Default|GetCenterY) :!class /Script/Engine.MaterialInstanceDynamic)
  (Rendering|Material|SetScalarParameterValue _materialdynamic "Density" (Variables|Default|GetDensity) :!class /Script/Engine.MaterialInstanceDynamic)
  (Rendering|Material|SetScalarParameterValue _materialdynamic "Radius" (Variables|Default|GetRadius) :!class /Script/Engine.MaterialInstanceDynamic)
  (Rendering|Material|SetScalarParameterValue _materialdynamic "Rotate" (Variables|Default|GetRotate) :!class /Script/Engine.MaterialInstanceDynamic)
  (Rendering|Material|SetScalarParameterValue _materialdynamic "ScaleX" (Variables|Default|GetScaleX) :!class /Script/Engine.MaterialInstanceDynamic)
  (Rendering|Material|SetScalarParameterValue _materialdynamic "ScaleY" (Variables|Default|GetScaleY) :!class /Script/Engine.MaterialInstanceDynamic)
  (Rendering|Material|SetScalarParameterValue _materialdynamic "Step" (Variables|Default|GetStep) :!class /Script/Engine.MaterialInstanceDynamic)
  (Rendering|Material|SetScalarParameterValue _materialdynamic "StepScale" (Variables|Default|GetStepScale) :!class /Script/Engine.MaterialInstanceDynamic))

(fn ConstructionScript
  (|CallParentFunction))