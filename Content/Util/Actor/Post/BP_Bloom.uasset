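; BP_Bloom is a post-process actor that applies a custom bloom effect through the M_PostBloom material.
; On BeginPlay, and from the construction script via Apply, it creates a dynamic material instance, feeds it the exposed bloom and debug settings, and registers it as a post-process blendable.
; It disables the PostProcess component when Ignore is set or on mobile with r.MobileHDR off, otherwise applying the configured priority.
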(event Custom|Apply
  (params (dummy :type Boolean))
  (bind _postprocess (Variables|Default|GetPostProcess))
  (bind _returnvalue (Development|GetConsoleVariableIntValue "r.MobileHDR"))
  (if (or (and (.IsMobile (Class|VrmBPFunctionLibrary|VRMGetMobileMode)) (== _returnvalue 0)) (Variables|Default|GetbIgnore))
    (Variables|/Script/Engine.PostProcessComponent|SetbEnabled _postprocess false)
    (else
      (Variables|/Script/Engine.PostProcessComponent|SetbEnabled _postprocess true)
      (Variables|/Script/Engine.PostProcessComponent|SetPriority _postprocess (Variables|Default|GetPriority))
      (Utilities|FlowControl|Sequence
        (:then_0
          (bind _returnvalue_2 (Rendering|Material|CreateDynamicMaterialInstance "/VRM4U/Util/Actor/Post/sub/M_PostBloom.M_PostBloom" "None" :!class /Script/Engine.KismetMaterialLibrary))
          (bind _output_get (Variables|Develop|SetPostMat _returnvalue_2))
          (Utilities|FlowControl|Sequence
            (:then_0
              (Rendering|Material|SetScalarParameterValue _output_get "DebugDraw" (select (Variables|Default|GetDebugDraw) 1.0 0.0) :!class /Script/Engine.MaterialInstanceDynamic))
            (:then_1
              (Rendering|Material|SetScalarParameterValue _output_get "Step" (Variables|Default|GetStep) :!class /Script/Engine.MaterialInstanceDynamic)
              (Rendering|Material|SetScalarParameterValue _output_get "Intensity" (Variables|Default|GetIntensity) :!class /Script/Engine.MaterialInstanceDynamic)
              (Rendering|Material|SetScalarParameterValue _output_get "Width" (Variables|Default|GetWidth) :!class /Script/Engine.MaterialInstanceDynamic))
            (:then_2
              (Rendering|Material|SetVectorParameterValue _output_get "BaseScaleAndOffset_XY" (Utilities|Struct|MakeLinearColor (Variables|Default|GetThreshold_Scale) (Variables|Default|GetThreshold_Offset) (Variables|Default|GetPower) (Variables|Default|GetBloomLimit)) :!class /Script/Engine.MaterialInstanceDynamic))))
        (:then_3
          (Utilities|Struct|SetmembersinPostProcessSettings (Variables|/Script/Engine.PostProcessComponent|GetSettings (Variables|Default|GetPostProcess)) (Utilities|Struct|MakeWeightedBlendables (Utilities|Array|MakeArray (Utilities|Struct|MakeWeightedBlendable 1.0 (Variables|Develop|GetPostMat))))))))))

(event EventBeginPlay
  (bind _postprocess (Variables|Default|GetPostProcess))
  (bind _returnvalue (Development|GetConsoleVariableIntValue "r.MobileHDR"))
  (if (or (and (.IsMobile (Class|VrmBPFunctionLibrary|VRMGetMobileMode)) (== _returnvalue 0)) (Variables|Default|GetbIgnore))
    (Variables|/Script/Engine.PostProcessComponent|SetbEnabled _postprocess false)
    (else
      (Variables|/Script/Engine.PostProcessComponent|SetbEnabled _postprocess true)
      (Variables|/Script/Engine.PostProcessComponent|SetPriority _postprocess (Variables|Default|GetPriority))
      (Utilities|FlowControl|Sequence
        (:then_0
          (bind _returnvalue_2 (Rendering|Material|CreateDynamicMaterialInstance "/VRM4U/Util/Actor/Post/sub/M_PostBloom.M_PostBloom" "None" :!class /Script/Engine.KismetMaterialLibrary))
          (bind _output_get (Variables|Develop|SetPostMat _returnvalue_2))
          (Utilities|FlowControl|Sequence
            (:then_0
              (Rendering|Material|SetScalarParameterValue _output_get "DebugDraw" (select (Variables|Default|GetDebugDraw) 1.0 0.0) :!class /Script/Engine.MaterialInstanceDynamic))
            (:then_1
              (Rendering|Material|SetScalarParameterValue _output_get "Step" (Variables|Default|GetStep) :!class /Script/Engine.MaterialInstanceDynamic)
              (Rendering|Material|SetScalarParameterValue _output_get "Intensity" (Variables|Default|GetIntensity) :!class /Script/Engine.MaterialInstanceDynamic)
              (Rendering|Material|SetScalarParameterValue _output_get "Width" (Variables|Default|GetWidth) :!class /Script/Engine.MaterialInstanceDynamic))
            (:then_2
              (Rendering|Material|SetVectorParameterValue _output_get "BaseScaleAndOffset_XY" (Utilities|Struct|MakeLinearColor (Variables|Default|GetThreshold_Scale) (Variables|Default|GetThreshold_Offset) (Variables|Default|GetPower) (Variables|Default|GetBloomLimit)) :!class /Script/Engine.MaterialInstanceDynamic))))
        (:then_3
          (Utilities|Struct|SetmembersinPostProcessSettings (Variables|/Script/Engine.PostProcessComponent|GetSettings (Variables|Default|GetPostProcess)) (Utilities|Struct|MakeWeightedBlendables (Utilities|Array|MakeArray (Utilities|Struct|MakeWeightedBlendable 1.0 (Variables|Develop|GetPostMat))))))))))

(fn ConstructionScript
  (CallFunction|Apply false))