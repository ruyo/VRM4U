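; BP_DiffusionFilter is a post-effect actor that configures a diffusion filter material.
; Its Init event runs the parent Init, then loops over paired name and value arrays to push its variables into the dynamic material as scalar parameters.
; The parameters cover base intensity and saturation, sampling shape and count, cross and stencil toggles, and base color, bloom and overall blend scales.
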(event EventBeginPlay)

(event Collision|EventActorBeginOverlap
  (params (OtherActor :type Actor%20Object%20Reference)))

(event EventTick
  (params (DeltaSeconds :type Float%20%28single-precision%29)))

(event EventInit
  (params (Dummy :type Boolean))
  (|CallParentFunction false)
  (for (_array_element _array_index) (Utilities|Array|MakeArray (Variables|Default|GetBaseIntensityScale) (Variables|Default|GetBaseSaturatePower) (Variables|Default|GetSampleWeightPow) (Variables|Default|GetSampleWidth) (Variables|Default|GetSampleIntensity) (Variables|Default|GetSampleAdd) (Variables|Default|GetSampleMultiply) (Variables|Default|GetSamplePow) (Variables|Default|GetSampleCount%28optimize%29) (Math|Conversions|ToFloat(Boolean) (Variables|Default|GetbCross)) (Math|Conversions|ToFloat(Byte) (Variables|Default|GetStencil)) (Variables|Default|GetBlendScale_BaseColor) (Variables|Default|GetBlendScale_Bloom) (Variables|Default|GetBlendScale_All))
    (Rendering|Material|SetScalarParameterValue (Variables|Default|GetMaterialDynamic) (Utilities|Array|Get(acopy) (Utilities|Array|MakeArray "BaseIntensityScale" "BaseSaturatePower" "SampleWeightPow" "SampleWidth" "SampleIntensity" "SampleAdd" "SampleMultiply" "SamplePow" "SampleCount" "bCross" "SampleStencil" "BlendScale_BaseColor" "BlendScale_Bloom" "BlendScale_All") _array_index) _array_element :!class /Script/Engine.MaterialInstanceDynamic)))

(fn ConstructionScript)