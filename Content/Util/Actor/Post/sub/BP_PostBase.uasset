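; BP_PostBase is a base actor for post-process effects, wrapping a PostProcess component around a material.
; The construction script calls Init, which enables the component unless Ignore is set.
; When Material is valid, Init stores a dynamic instance of it in MaterialDynamic and assigns it as a full-weight blendable in the component's settings.
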(event Custom|Init
  (params (Dummy :type Boolean))
  (Variables|/Script/Engine.PostProcessComponent|SetbEnabled (Variables|Default|GetPostProcess) (not (Variables|Default|GetbIgnore)))
  (bind _material (Variables|Default|GetMaterial)
    (:then
      (bind _returnvalue (Rendering|Material|CreateDynamicMaterialInstance _material "None" "None" :!class /Script/Engine.KismetMaterialLibrary))
      (Variables|Default|SetMaterialDynamic _returnvalue)
      (Utilities|Struct|SetmembersinPostProcessSettings (Variables|/Script/Engine.PostProcessComponent|GetSettings (Variables|Default|GetPostProcess)) (Utilities|Struct|MakeWeightedBlendables (Utilities|Array|MakeArray (Utilities|Struct|MakeWeightedBlendable 1.0 _returnvalue)))))
    (:else)))

(event EventBeginPlay)

(event Collision|EventActorBeginOverlap
  (params (OtherActor :type Actor%20Object%20Reference)))

(event EventTick
  (params (DeltaSeconds :type Float%20%28single-precision%29)))

(fn ConstructionScript
  (CallFunction|Init false))